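; BP_DungeonPart is a dungeon piece with a floor, an optional ceiling and a minimap mesh.
; Its construction script assigns the meshes, offsets the map mesh, toggles the ceiling and optionally yaws the floor by a random listed angle.
; Secret parts hide their map mesh until a BP_DungeonPawn overlaps the Box.
; The secret minimap material is assigned to the variable only after the map's material is applied.
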(event OnComponentBeginOverlap(Box)
  (params (OverlappedComponent :type Primitive%20Component%20Object%20Reference) (OtherActor :type Actor%20Object%20Reference) (OtherComp :type Primitive%20Component%20Object%20Reference) (OtherBodyIndex :type Integer) (bFromSweep :type Boolean) (SweepResult :type Hit%20Result%20Structure%20%28by%20ref%29))
  (Utilities|Casting|CastToBP_DungeonPawn OtherActor)
  (Rendering|SetVisibility (Variables|Default|GetMap) true false))

(fn ConstructionScript
  (bind _zceiling (Variables|Default|GetZCeiling))
  (bind _map (Variables|Default|GetMap))
  (bind _map_2 (Variables|Default|GetMap))
  (Components|StaticMesh|SetStaticMesh (Variables|Default|GetFloor) (Variables|Meshes|GetFloorMesh))
  (Components|StaticMesh|SetStaticMesh (Variables|Default|GetZCeiling) (Variables|Meshes|GetCeilingMesh))
  (Utilities|FlowControl|Sequence
    (:then_0
      ;[1 0.6172 0.159] Map Setup
      (Transformation|AddLocalOffset _map_2 (Math|Vector|MakeVector 0.0 0.0 (Variables|Default|GetMapHeightOffset)) false false)
      (Rendering|Material|SetMaterial _map_2 0 (Variables|Default|GetMap%20Material))
      (if (Variables|Switches|GetbIsSecret)
        (Rendering|SetVisibility _map false false)
        (Variables|Default|SetMap%20Material "/Game/Materials/Interface/MI_Minimap_Secret.MI_Minimap_Secret")
        (else
          (Rendering|SetVisibility _map true false))))
    (:then_1
      ;[0.000304 0.6584 0.1413] Ceiling
      (if (Variables|Switches|GetbAddCeiling)
        (Rendering|SetVisibility _zceiling true false)
        (Transformation|AddLocalOffset (Variables|Default|GetZCeiling) (Math|Vector|MakeVector 0.0 0.0 0.0) false false)
        (else
          (Rendering|SetVisibility _zceiling false false))))
    (:then_2
      (if (Variables|Switches|GetbRandomRotation)
        (Transformation|AddRelativeRotation (Variables|Default|GetFloor) (Math|Rotator|MakeRotator 0.0 0.0 (.OutItem (Utilities|Array|Random (Variables|Default|GetRendomRotations)))) false false)))))