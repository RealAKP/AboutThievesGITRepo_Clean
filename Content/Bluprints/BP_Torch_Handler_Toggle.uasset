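; Interactable wall or prop torch that toggles lit and unlit based on its interact state, powering linked actors when turned on.
; Lighting activates fire and audio and plays a timeline that flickers the point light's intensity and position; extinguishing reverses this.
; BeginPlay, instant state updates and the construction script's PreviewState apply the matching look.
; Cursor hover toggles a material highlight, and each flicker update prints a debug string.
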(event Custom|EventFlickeringSTOP
  (bind _pointlight (Variables|Default|GetPointLight))
  (Rendering|SetVisibility (Variables|Default|GetPointLight) false false)
  (Components|Activation|Deactivate (Variables|Default|GetFire))
  (Audio|Components|Audio|SetVolumeMultiplier (Variables|Default|GetAudio) 0.0 :!class /Script/Engine.AudioComponent)
  (bind _intensity (Timeline|Flickering Stop)
    (:Update
      (Rendering|Components|Light|SetIntensity _pointlight (Math|Float|Lerp (Variables|Default|GetMinINT) (Variables|Default|GetMaxINT) _intensity))
      (Transformation|SetRelativeLocation _pointlight (Math|Conversions|ToVector(Float) (* _intensity 15.0)) false false)
      (Transformation|AddRelativeLocation _pointlight "40.000000,0.000000,120.000000" false false)
      (Development|PrintString (Utilities|GetObjectName self) true true "(R=0.000000,G=0.660000,B=1.000000,A=1.000000)" 0.0))))

(event Custom|EventFlickering
  (bind _pointlight (Variables|Default|GetPointLight))
  (Rendering|SetVisibility (Variables|Default|GetPointLight) true false)
  (Components|Activation|Activate (Variables|Default|GetFire) true)
  (Audio|Components|Audio|SetVolumeMultiplier (Variables|Default|GetAudio) 1.0 :!class /Script/Engine.AudioComponent)
  (bind _intensity (Timeline|Flickering PlayFromStart)
    (:Update
      (Rendering|Components|Light|SetIntensity _pointlight (Math|Float|Lerp (Variables|Default|GetMinINT) (Variables|Default|GetMaxINT) _intensity))
      (Transformation|SetRelativeLocation _pointlight (Math|Conversions|ToVector(Float) (* _intensity 15.0)) false false)
      (Transformation|AddRelativeLocation _pointlight "40.000000,0.000000,120.000000" false false)
      (Development|PrintString (Utilities|GetObjectName self) true true "(R=0.000000,G=0.660000,B=1.000000,A=1.000000)" 0.0))))

(event MouseInput|EventActorBeginCursorOver
  (Rendering|Material|SetScalarParameterValueonMaterials (Variables|Default|GetSM_FireTorch_SX_001) "Highlight" 1.0))

(event MouseInput|EventActorEndCursorOver
  (Rendering|Material|SetScalarParameterValueonMaterials (Variables|Default|GetSM_FireTorch_SX_001) "Highlight" 0.0))

(event EventUpdateStateInstantly
  (params (DesiredState :type EInteractState%20Enum :default "NewEnumerator0"))
  (switch Utilities|FlowControl|Switch|SwitchonEInteractState DesiredState
    (:NewEnumerator0
      (CallFunction|EventFlickeringSTOP))
    (:NewEnumerator2
      (CallFunction|EventFlickering))))

(event EventActivate
  (params (bTurnOn :type Boolean) (TriggeringActor :type Actor%20Object%20Reference))
  (Audio|PlaySoundatLocation "/Game/Audio/Items/A_Torch_Attack_01_Cue.A_Torch_Attack_01_Cue" (Transformation|GetWorldLocation (Variables|Default|GetAudio)) "0, 0, 0" 1.0 1.0 0.0 "/Game/DCT/Sound/ATT_Dungeon.ATT_Dungeon" 0 0 0)
  (Variables|Default|SetInteractState (Variables|Default|GetDesiredState))
  (if bTurnOn
    (CallFunction|PowerActors (Variables|Default|GetInteractState))
    (CallFunction|EventFlickering)
    (else
      (CallFunction|EventFlickeringSTOP))))

(event EventBeginPlay
  (|CallParentFunction)
  (bind _output_get (Variables|Default|SetInteractState (Variables|Default|GetDesiredState)))
  (switch Utilities|FlowControl|Switch|SwitchonEInteractState _output_get
    (:NewEnumerator0
      (CallFunction|EventFlickeringSTOP))
    (:NewEnumerator2
      (CallFunction|EventFlickering))))

(fn ConstructionScript
  (|CallParentFunction)
  (switch Utilities|FlowControl|Switch|SwitchonEInteractState (Variables|Default|GetPreviewState)
    (:NewEnumerator0
      (CallFunction|EventFlickeringSTOP))
    (:NewEnumerator2
      (CallFunction|EventFlickering))))