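; BP_Breakable_Boxes_Destroyed is the broken state of a wooden box, made up of ten separate fragment mesh components.
; On BeginPlay it waits three seconds, then turns off physics simulation on every fragment so the debris stops moving.
; It has no other logic, and its construction script is empty.
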(event EventBeginPlay
  (Utilities|FlowControl|Delay 3.0)
  (Physics|SetSimulatePhysics (Variables|Default|GetSM_Wooden_box_fragment4) false))

(fn ConstructionScript)