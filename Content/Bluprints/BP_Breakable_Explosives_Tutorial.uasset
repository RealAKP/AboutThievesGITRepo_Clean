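; Tutorial explosive prop that occupies and blocks a dungeon grid tile until it is destroyed by damage.
; Damage lowers health and shows floating numbers; at zero it spawns break effects, a destroyed version and a short-lived explosion damage trigger.
; It then reopens its tile and replaces any open character dialog with a typewritten line attributed to a random living party member.
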(event EventBeginPlay
  (Utilities|FlowControl|Delay 0.0)
  (bind _gridindex (Default|FindNearbyValidTile (.DungeonManager (CallFunction|GetDungeonManager)) (Transformation|GetActorLocation)))
  (Variables|Default|SetGridIndex _gridindex)
  (Default|BlockTile (.DungeonManager (CallFunction|GetDungeonManager)) (Variables|Default|GetGridIndex))
  (Default|AddObjecttoGrid (.DungeonManager (CallFunction|GetDungeonManager)) self (Variables|Default|GetGridIndex)))

(event EventTakeDamage
  (params (Damage :type Float%20%28double-precision%29))
  (bind _returnvalue (Transformation|GetActorTransform))
  (bind _returnvalue_2 (Transformation|GetActorLocation))
  (Variables|Default|SetHealth (- (Variables|Default|GetHealth) Damage))
  (bind _returnvalue_3 (Game|SpawnActorfromClass "/Game/DCT/Blueprints/Core/BP_FloatingText.BP_FloatingText_C" (Math|Transform|MakeTransform (+ (Transformation|GetActorLocation) "0,0.000000,150.000000") "0, 0, 0" "1.000000,1.000000,1.000000") "AlwaysSpawn" "OverrideRootScale" 0 (Utilities|Text|ToText(Float) Damage "HalfToEven") 0))
  (Default|SetColor _returnvalue_3 "(R=1.000000,G=0.008023,B=0.009721,A=1.000000)")
  (if (< (Variables|Default|GetHealth) 1.0)
    (Default|RemoveObjectfromGrid (.DungeonManager (CallFunction|GetDungeonManager)) self (Variables|Default|GetGridIndex))
    (Niagara|SpawnSystematLocation (Variables|Default|GetBreakSystem) _returnvalue_2)
    (Game|SpawnActorfromClass "/Game/Bluprints/BP_Breakable_Explosives_Destroyed.BP_Breakable_Explosives_Destroyed_C" _returnvalue "Undefined" "OverrideRootScale" 0 0)
    (Audio|PlaySoundatLocation "/Game/Audio/Chaos/A_Explosion_Cue.A_Explosion_Cue" _returnvalue_2 "0, 0, 0" 1.0 1.0 0.0 0 0 0 0)
    (bind _returnvalue_4 (Game|SpawnActorfromClass "/Game/Bluprints/BP_Trigger_Damage_Explosion.BP_Trigger_Damage_Explosion_C" _returnvalue "Undefined" "OverrideRootScale" 0 0))
    (Utilities|FlowControl|Delay 0.2)
    (Actor|DestroyActor _returnvalue_4)
    (Utilities|FlowControl|Sequence
      (:then_0
        (Actor|DestroyActor)
        (Default|ReopenTile (.DungeonManager (CallFunction|GetDungeonManager)) (Variables|Default|GetGridIndex)))
      (:then_1
        (bind _foundwidgets (Widget|GetAllWidgetsOfClass "/Game/DCT/UserInterface/WBP_Character_Dialog.WBP_Character_Dialog_C" false))
        (Widget|RemovefromParent _foundwidgets)
        (bind _returnvalue_5 (UserInterface|CreateWidget "/Game/DCT/UserInterface/WBP_Character_Dialog.WBP_Character_Dialog_C" (Game|GetPlayerController 0) 0))
        (Variables|/Game/DCT/UserInterface/WBP_Character_Dialog.WBP_Character_Dialog_C|SetDialog%20Text _returnvalue_5 (Variables|Default|GetDialog%20Text))
        (bind (_bfoundlivingcharacters _livingplayercharacters) (Default|GetLivingPlayerCharacters (.DungeonState (CallFunction|GetDungeonGameState))))
        (if _bfoundlivingcharacters
          (bind _output_get (Variables|Default|SetRNG (Math|Random|RandomIntegerinRange 0 (Utilities|Array|LastIndex _livingplayercharacters))))
          (Variables|/Game/DCT/UserInterface/WBP_Character_Dialog.WBP_Character_Dialog_C|SetCharacter%20Name _returnvalue_5 (Utilities|Text|ToText(Name) (Variables|/Game/DCT/Blueprints/Core/BP_PlayerCharacter.BP_PlayerCharacter_C|GetName (Utilities|Array|Get(acopy) _livingplayercharacters _output_get))))
          (Variables|/Game/DCT/UserInterface/WBP_Character_Dialog.WBP_Character_Dialog_C|SetDialog%20Portrait _returnvalue_5 (Utilities|Struct|MakeSlateBrush "(SpecifiedColor=(R=1.000000,G=1.000000,B=1.000000,A=1.000000),ColorUseRule=UseColor_Specified)" "Image" "NoTile" "NoMirror" "(X=96.000000,Y=96.000000)" "(Left=0.000000,Top=0.000000,Right=0.000000,Bottom=0.000000)" (Variables|/Game/DCT/Blueprints/Core/BP_PlayerCharacter.BP_PlayerCharacter_C|GetPortrait (Utilities|Array|Get(acopy) _livingplayercharacters _output_get)) "(CornerRadii=(X=0.000000,Y=0.000000,Z=0.000000,W=0.000000),Color=(SpecifiedColor=(R=0.000000,G=0.000000,B=0.000000,A=0.000000),ColorUseRule=UseColor_Specified),Width=0.000000,RoundingType=HalfHeightRadius,bUseBrushTransparency=False)"))
          (UserInterface|Viewport|AddtoViewport _returnvalue_5 -1)
          (Default|InitiateTypewrite _returnvalue_5)
          (Actor|DestroyActor))))))

(fn ConstructionScript)

(fn GetWeight
  (return 1.0))

(fn AttemptInteract
  (params (TriggeringActor :type Actor%20Object%20Reference))
  (return false))

(fn GetDodgeChance
  (return -0.5))