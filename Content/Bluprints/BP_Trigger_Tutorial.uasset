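; BP_Trigger_Tutorial is a one-shot trigger actor that shows a tutorial message on screen.
; It fires on BeginPlay when AutoActivate is set, or when a BP_DungeonPawn overlaps it.
; Behind a DoOnce, it removes existing WBP_Tutorial_RichText widgets, adds a new one carrying its Tutorial data, then destroys itself.
; Save and player step-end events only forward to the parent class.
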(event Collision|EventActorBeginOverlap
  (params (OtherActor :type Actor%20Object%20Reference))
  (|CallParentFunction OtherActor)
  (Utilities|Casting|CastToBP_DungeonPawn OtherActor)
  (Utilities|FlowControl|DoOnce false
    (:Completed
      (bind _foundwidgets (Widget|GetAllWidgetsOfClass "/Game/DCT/UserInterface/Tutorials/WBP_Tutorial_RichText.WBP_Tutorial_RichText_C" false))
      (Widget|RemovefromParent _foundwidgets)
      (bind _returnvalue (UserInterface|CreateWidget "/Game/DCT/UserInterface/Tutorials/WBP_Tutorial_RichText.WBP_Tutorial_RichText_C"))
      (Variables|/Game/DCT/UserInterface/Tutorials/WBP_Tutorial_RichText.WBP_Tutorial_RichText_C|SetTutorial _returnvalue (Variables|Default|GetTutorial))
      (UserInterface|Viewport|AddtoViewport _returnvalue -2)
      (Actor|DestroyActor))))

(event EventCallonPlayerStepEnd
  (params (DungeonPawn :type BP%20Dungeon%20Pawn%20Object%20Reference))
  (|CallParentFunction DungeonPawn))

(event EventSaveActor
  (params (DungeonInstance :type BP%20GI%20Dungeon%20Object%20Reference))
  (|CallParentFunction DungeonInstance))

(event EventBeginPlay
  (|CallParentFunction)
  (if (Variables|Default|GetAutoActivate)
    (Utilities|FlowControl|DoOnce false
      (:Completed
        (bind _foundwidgets (Widget|GetAllWidgetsOfClass "/Game/DCT/UserInterface/Tutorials/WBP_Tutorial_RichText.WBP_Tutorial_RichText_C" false))
        (Widget|RemovefromParent _foundwidgets)
        (bind _returnvalue (UserInterface|CreateWidget "/Game/DCT/UserInterface/Tutorials/WBP_Tutorial_RichText.WBP_Tutorial_RichText_C"))
        (Variables|/Game/DCT/UserInterface/Tutorials/WBP_Tutorial_RichText.WBP_Tutorial_RichText_C|SetTutorial _returnvalue (Variables|Default|GetTutorial))
        (UserInterface|Viewport|AddtoViewport _returnvalue -2)
        (Actor|DestroyActor)))))

(fn ConstructionScript
  (|CallParentFunction))