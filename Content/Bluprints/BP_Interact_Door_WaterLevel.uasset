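; Interactable door Blueprint, named for the water level, that opens once when activated.
; Activate calls MoveDoor at 100 and then destroys the Box component.
; MoveDoor sets the Pivot's relative Z to PercentOpen times 200 in one step with no interpolation, so activation jumps it to 20,000 units.
; The construction script only calls its parent, and GetAttachSlot is an empty stub.
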(event EventActivate
  (params (bTurnOn :type Boolean) (TriggeringActor :type Actor%20Object%20Reference))
  (CallFunction|MoveDoor 1e+02)
  (Components|DestroyComponent (Variables|Default|GetBox)))

(fn ConstructionScript
  (|CallParentFunction))

(fn MoveDoor
  (params (PercentOpen :type Float%20%28double-precision%29))
  (Transformation|SetRelativeLocation (Variables|Default|GetPivot) (Math|Vector|MakeVector 0.0 0.0 (* PercentOpen 2e+02)) false false))

(fn GetAttachSlot
  (return 0))