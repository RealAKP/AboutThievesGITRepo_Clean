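; Freeze spell trigger that applies a temporary frost effect to the first overlapping BP_Monster, ignoring the immune red Szlamek.
; On hit it destroys its overlap area, then after a short delay adds a fixed offset to the monster's MoveSpeed and applies a dynamic frost overlay material.
; The CoolOff timeline drives overlay opacity, then restores the data-defined speed and destroys the trigger.
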(event Collision|EventActorBeginOverlap
  (params (OtherActor :type Actor%20Object%20Reference))
  ;[1 0.5036 0] Immune Monster
  (Utilities|Casting|CastToBP_Monster_Szlamek_Red OtherActor
    (:CastFailed
      (bind _asbp_monster (Utilities|Casting|CastToBP_Monster OtherActor))
      (Components|DestroyComponent (Variables|Default|GetOverlapArea))
      (Utilities|FlowControl|DoOnce false
        (:Completed
          (bind _output_get (Variables|Default|SetOriginal%20Speed (.movespeed (.Data (Default|GetMonsterData _asbp_monster)))))
          (Development|PrintString (Utilities|String|ToString(Float) _output_get))
          (Utilities|FlowControl|Delay 0.1)
          (bind _output_get_2 (Variables|/Game/DCT/Blueprints/Monsters/BP_Monster.BP_Monster_C|SetMoveSpeed _asbp_monster (+ (Variables|Default|GetOriginal%20Speed) 2.0)))
          (Development|PrintString (Utilities|String|ToString(Float) _output_get_2))
          (bind _returnvalue (Rendering|Material|CreateDynamicMaterialInstance "/Game/Materials/Overlays/M_Overlay_Frost.M_Overlay_Frost" "None" "None" :!class /Script/Engine.KismetMaterialLibrary))
          (bind _output_get_3 (Variables|Default|SetOverlayMaterial _returnvalue))
          (Rendering|Material|SetOverlayMaterial (Variables|/Game/DCT/Blueprints/Monsters/BP_Monster.BP_Monster_C|GetSkeletalMesh _asbp_monster) _output_get_3 :!class /Script/Engine.MeshComponent)
          (bind _linearfloat (Timeline|CoolOff Play)
            (:Update
              (Rendering|Material|SetScalarParameterValue (Variables|Default|GetOverlayMaterial) "Opacity" _linearfloat :!class /Script/Engine.MaterialInstanceDynamic))
            (:Finished
              (bind _output_get_4 (Variables|/Game/DCT/Blueprints/Monsters/BP_Monster.BP_Monster_C|SetMoveSpeed _asbp_monster (Variables|Default|GetOriginal%20Speed)))
              (Development|PrintString (Utilities|String|ToString(Float) _output_get_4))
              (Actor|DestroyActor))))))))

(fn ConstructionScript
  (|CallParentFunction))