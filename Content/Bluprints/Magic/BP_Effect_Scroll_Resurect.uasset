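; Scroll effect that resurrects the dungeon party when used.
; On use it runs the parent effect, then loops over all player characters in the dungeon state, reviving each and restoring a small capped amount of health.
; Each iteration also plays a healing sound and spawns a Niagara burst at the first player pawn's location.
; Its description prepends a duration stat icon and seconds to the parent's text.
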(event EventUseEffect
  (params (ActivatingPlayerCharacter :type BP%20Player%20Character%20Object%20Reference) (ResidingSlot :type WBP%20Slot%20Object%20Reference) (ItemType :type Data%20Table%20Row%20Handle%20Structure))
  (|CallParentFunction ActivatingPlayerCharacter ResidingSlot ItemType)
  (for _array_element (Variables|/Game/DCT/Blueprints/Core/BP_Dungeon_State.BP_Dungeon_State_C|GetPlayerCharacters (.DungeonState (CallFunction|GetDungeonGameState)))
    (Default|RevivePlayerCharacter _array_element)
    (Default|ModifyStatCapped _array_element "(TagName=\"Stat.Health\")" 1e+01)
    (Audio|PlaySound2D "/Game/Audio/Magic___Spell_Sounds_PRO/General/wav/Healing_10.Healing_10" 1.0 1.0 0.0 0 0)
    (Niagara|SpawnSystematLocation "/Game/Particles/Magic/NS_PH_ShieldofFaith_End.NS_PH_ShieldofFaith_End" (Transformation|GetActorLocation (Game|Player|GetPlayerPawn 0)))))

(fn ConstructionScript
  (|CallParentFunction))

(fn GetEffectDescription
  (params (ItemType :type Data%20Table%20Row%20Handle%20Structure))
  (bind _statdescription (|CallParentFunction ItemType))
  (return (Utilities|String|Append "<img id=\"StatTime\"/>" (Utilities|String|ToString(Integer) (Variables|Default|GetDuration)) " s" "" _statdescription)))