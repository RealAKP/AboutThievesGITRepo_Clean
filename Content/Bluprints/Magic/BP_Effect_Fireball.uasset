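; Fireball magic item effect that spawns the item's projectile class when used.
; UseEffect runs the parent logic, then, if the class is valid, spawns it at player pawn 0's transform raised by a height offset, passing the item and pawn as source.
; It uses player 0 instead of the activating character.
; GetEffectDescription returns the duration with a time icon, leaving stat-list and cooldown text logic unreachable.
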(event EventUseEffect
  (params (ActivatingPlayerCharacter :type BP%20Player%20Character%20Object%20Reference) (ResidingSlot :type WBP%20Slot%20Object%20Reference) (ItemType :type Data%20Table%20Row%20Handle%20Structure))
  (bind _returnvalue (Game|Player|GetPlayerPawn 0))
  (bind _returnvalue_2 (Transformation|GetActorTransform _returnvalue))
  (|CallParentFunction ActivatingPlayerCharacter ResidingSlot ItemType)
  (if (Utilities|IsValidClass (Utilities|Struct|BreakFItem (CallFunction|GetItemData)))
    (Game|SpawnActorfromClass (Utilities|Struct|BreakFItem (CallFunction|GetItemData)) (Math|Transform|MakeTransform (+ (.location _returnvalue_2) (Math|Vector|MakeVector 0.0 0.0 (Variables|Default|GetProjectileSpawnHeight))) (.rotation _returnvalue_2) (.scale _returnvalue_2)) "Undefined" "SelectDefaultAtRuntime" 0 7e+02 0.0 (Variables|Default|GetItemType) _returnvalue 0)))

(fn ConstructionScript
  (|CallParentFunction))

(fn GetEffectDescription
  (params (ItemType :type Data%20Table%20Row%20Handle%20Structure))
  (|CallParentFunction ItemType)
  (return (Utilities|String|Append "<img id=\"StatTime\"/>" (Utilities|String|ToString(Integer) (Variables|Default|GetDuration)) " s")))