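; Magic Missile power effect that spawns the item's projectile from the player pawn when used.
; UseEffect runs the parent logic, then, if the item data has a valid projectile class, spawns it at a height offset, passing the item and player as source.
; FindValidTarget separately asks the dungeon manager for monsters on one adjacent grid tile.
; The description prepends a magic damage icon and value or range to the parent's text.
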(event EventUseEffect
  (params (ActivatingPlayerCharacter :type BP%20Player%20Character%20Object%20Reference) (ResidingSlot :type WBP%20Slot%20Object%20Reference) (ItemType :type Data%20Table%20Row%20Handle%20Structure))
  (bind _returnvalue (Game|Player|GetPlayerPawn 0))
  (bind _returnvalue_2 (Transformation|GetActorTransform _returnvalue))
  (|CallParentFunction ActivatingPlayerCharacter ResidingSlot ItemType)
  (if (Utilities|IsValidClass (Utilities|Struct|BreakFItem (CallFunction|GetItemData)))
    (Game|SpawnActorfromClass (Utilities|Struct|BreakFItem (CallFunction|GetItemData)) (Math|Transform|MakeTransform (+ (.location _returnvalue_2) (Math|Vector|MakeVector 0.0 0.0 (Variables|Default|GetProjectileSpawnHeight))) (.rotation _returnvalue_2) (.scale _returnvalue_2)) "Undefined" 0 7e+02 0.0 (Variables|Default|GetItemType) _returnvalue 0)))

(fn ConstructionScript
  (|CallParentFunction))

(fn FindValidTarget
  (bind _returnvalue (Actor|GetActorOfClass "/Game/DCT/Blueprints/Core/BP_DungeonManager.BP_DungeonManager_C"))
  (bind _adjacentgridindex (Default|GetAdjacentTilefromLocation _returnvalue (Game|Player|GetPlayerPawn 0) "NewEnumerator0"))
  (bind (_bobjectfound _objectrefs) (Default|FindObjectsOfClassonGrid _returnvalue _adjacentgridindex "/Game/DCT/Blueprints/Monsters/BP_Monster.BP_Monster_C"))
  (return _bobjectfound _objectrefs))

(fn GetEffectDescription
  (params (ItemType :type Data%20Table%20Row%20Handle%20Structure))
  (bind _itemdata (CallFunction|GetItemData))
  (bind _effectstats (Utilities|Struct|BreakFItem _itemdata))
  (bind (_mindamage _maxdamage) (CallFunction|GetDamageRange _effectstats))
  (bind _returnvalue (Utilities|String|ToString(Integer) _maxdamage))
  (bind _statdescription (|CallParentFunction ItemType))
  (return (Utilities|String|Append (select (== _mindamage _maxdamage) (Utilities|String|Append "<img id=\"StatMDamage\"/>" _returnvalue) (Utilities|String|Append "<img id=\"StatMDamage\"/>" (Utilities|String|ToString(Integer) _mindamage) " - " _returnvalue)) _statdescription)))