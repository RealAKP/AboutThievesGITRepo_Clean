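; BP_Effect_Power_SlowTime is a magic power effect that temporarily slows global time when used.
; UseEffect calls the parent, drops global time dilation, spawns a 2D clock sound and plays a timeline that drives that sound's pitch.
; When the timeline finishes, it restores normal time, silences and destroys the clock sound, then plays a dispel cue.
; The construction script and effect description only defer to the parent.
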(event EventUseEffect
  (params (ActivatingPlayerCharacter :type BP%20Player%20Character%20Object%20Reference) (ResidingSlot :type WBP%20Slot%20Object%20Reference) (ItemType :type Data%20Table%20Row%20Handle%20Structure))
  (|CallParentFunction ActivatingPlayerCharacter ResidingSlot ItemType)
  (Utilities|Time|SetGlobalTimeDilation 0.3)
  (bind _returnvalue (Audio|SpawnSound2D "/Game/Audio/Magic/S_Clock_Cue.S_Clock_Cue" 1.0 1.0 0.0 0 false false))
  (bind _pitch (Timeline|Timeline Play)
    (:Update
      (Audio|Components|Audio|SetPitchMultiplier _returnvalue _pitch))
    (:Finished
      (Utilities|Time|SetGlobalTimeDilation 1.0)
      (Audio|Components|Audio|AdjustVolume _returnvalue 0.0 0.0 "Linear" :!class /Script/Engine.AudioComponent)
      (Components|DestroyComponent _returnvalue)
      (Audio|SpawnSound2D "/Game/Audio/Magic/S_Clock_Dispell_Cue.S_Clock_Dispell_Cue" 1.0 1.0 0.0 0))))

(fn ConstructionScript
  (|CallParentFunction))

(fn GetEffectDescription
  (params (ItemType :type Data%20Table%20Row%20Handle%20Structure))
  (bind _statdescription (|CallParentFunction ItemType))
  (return _statdescription))