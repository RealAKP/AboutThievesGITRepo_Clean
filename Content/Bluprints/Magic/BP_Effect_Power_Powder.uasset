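; Powder magic item effect that temporarily blinds monsters on a dungeon tile adjacent to the player.
; UseEffect plays Niagara and sound effects, then Strike gets that tile's monsters from BP_DungeonManager through FindValidTarget.
; Strike drops their Dodge and Accuracy and shows BLINDED text, then restores base stats after a Delay inside the target loop.
; With no valid target, Miss shows MISS text instead.
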(event Custom|Strike
  (bind _returnvalue (Game|Player|GetPlayerPawn 0))
  (bind _returnvalue_2 (Transformation|GetActorForwardVector _returnvalue))
  (bind _returnvalue_3 (Transformation|GetActorLocation _returnvalue))
  (bind _returnvalue_4 (* _returnvalue_2 1.5e+02))
  (bind _returnvalue_5 (+ _returnvalue_3 _returnvalue_4))
  (bind (_bsuccess _targets) (CallFunction|FindValidTarget))
  (if _bsuccess
    (for _array_element _targets
      (bind _asbp_monster (Utilities|Casting|CastToBP_Monster _array_element))
      (Default|ModifyMonsterStat _asbp_monster "(TagName=\"Stat.Dodge\")" 0.0 "NewEnumerator2")
      (Default|ModifyMonsterStat _asbp_monster "(TagName=\"Stat.Accuracy\")" 0.1 "NewEnumerator2")
      (Development|PrintString "Monster Blinded")
      (Utilities|FlowControl|Sequence
        (:then_0
          (Game|SpawnActorfromClass "/Game/DCT/Blueprints/Core/BP_FloatingText.BP_FloatingText_C" (Math|Transform|MakeTransform (+ _returnvalue_5 "0, 0,100.000000") (Math|Rotator|FindLookatRotation _returnvalue_5 _returnvalue_3) "0.800000,0.800000,0.800000") "AlwaysSpawn" "OverrideRootScale" 0 "BLINDED" 0))
        (:then_1
          (Utilities|FlowControl|Delay 5.0)
          (Default|ModifyMonsterStat _asbp_monster "(TagName=\"Stat.Dodge\")" (.Value (Utilities|Map|Find (.BaseStats (Default|GetMonsterBaseStats _asbp_monster)) "(TagName=\"Stat.Dodge\")")) "NewEnumerator2")
          (Default|ModifyMonsterStat _asbp_monster "(TagName=\"Stat.Accuracy\")" (.Value (Utilities|Map|Find (.BaseStats (Default|GetMonsterBaseStats _asbp_monster)) "(TagName=\"Stat.Accuracy\")")) "NewEnumerator2"))))
    (else
      (CallFunction|Miss))))

(event Custom|Miss
  (bind _returnvalue (Game|Player|GetPlayerPawn 0))
  (bind _returnvalue_2 (Transformation|GetActorForwardVector _returnvalue))
  (bind _returnvalue_3 (Transformation|GetActorLocation _returnvalue))
  (bind _returnvalue_4 (* _returnvalue_2 1.5e+02))
  (bind _returnvalue_5 (+ _returnvalue_3 _returnvalue_4))
  (Game|SpawnActorfromClass "/Game/DCT/Blueprints/Core/BP_FloatingText.BP_FloatingText_C" (Math|Transform|MakeTransform (+ _returnvalue_5 "0, 0,100.000000") (Math|Rotator|FindLookatRotation _returnvalue_5 _returnvalue_3) "0.800000,0.800000,0.800000") "AlwaysSpawn" "OverrideRootScale" 0 "MISS" 0))

(event EventUseEffect
  (params (ActivatingPlayerCharacter :type BP%20Player%20Character%20Object%20Reference) (ResidingSlot :type WBP%20Slot%20Object%20Reference) (ItemType :type Data%20Table%20Row%20Handle%20Structure))
  (bind _returnvalue (Game|Player|GetPlayerPawn 0))
  (bind _returnvalue_2 (Transformation|GetActorLocation _returnvalue))
  (|CallParentFunction ActivatingPlayerCharacter ResidingSlot ItemType)
  (bind _adjacenttilelocation (Default|GetAdjacentTilefromLocation (.DungeonManager (CallFunction|GetDungeonManager)) _returnvalue "NewEnumerator0"))
  (Niagara|SpawnSystematLocation "/Game/Particles/Magic/NS_Powder.NS_Powder" _adjacenttilelocation "0, 0, 0" "1.000000,1.000000,1.000000" false)
  (Niagara|SpawnSystematLocation "/Game/Particles/Magic/NS_Powder_Muzzle.NS_Powder_Muzzle" _returnvalue_2 (Transformation|GetActorRotation _returnvalue) "1.000000,1.000000,1.000000" false)
  (Audio|PlaySoundatLocation "/Game/Audio/Magic/A_Magic_Light_End_Cue.A_Magic_Light_End_Cue" _returnvalue_2 "0, 0, 0" 1.0 1.0 0.0 0 0 0 0)
  (CallFunction|Strike))

(fn ConstructionScript
  (|CallParentFunction))

(fn GetEffectDescription
  (params (ItemType :type Data%20Table%20Row%20Handle%20Structure))
  (bind _statdescription (|CallParentFunction ItemType))
  (return (Utilities|String|Append _statdescription "")))

(fn FindValidTarget
  (bind _localtargets (LocalVariables|GetLocalTargets))
  (bind _returnvalue (Actor|GetActorOfClass "/Game/DCT/Blueprints/Core/BP_DungeonManager.BP_DungeonManager_C"))
  (bind _adjacentgridindex (Default|GetAdjacentTilefromLocation _returnvalue (Game|Player|GetPlayerPawn 0) "NewEnumerator0"))
  (bind (_bobjectfound _objectrefs) (Default|GetAllObjectsonTile _returnvalue _adjacentgridindex))
  (if _bobjectfound
    (for _array_element _objectrefs
      (bind _asbp_monster (Utilities|Casting|CastToBP_Monster _array_element))
      (Utilities|Array|Add (LocalVariables|GetLocalTargets) _asbp_monster))
    (return (> (Utilities|Array|Length _localtargets) 0) _localtargets)
    (else
      (return false 0))))