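; BP_Effect_Power_Smoke is a magic power effect that creates a temporary smoke effect at the player's location.
; On use it runs the parent logic, then spawns the P_SmokeAndMirrors particle system and adds a child actor component at player pawn 0's position.
; After a Duration delay it destroys both components.
; It always uses player pawn 0 rather than the activating character, and its effect description defers to the parent.
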(event EventUseEffect
  (params (ActivatingPlayerCharacter :type BP%20Player%20Character%20Object%20Reference) (ResidingSlot :type WBP%20Slot%20Object%20Reference) (ItemType :type Data%20Table%20Row%20Handle%20Structure))
  (bind _returnvalue (Game|Player|GetPlayerPawn 0))
  (|CallParentFunction ActivatingPlayerCharacter ResidingSlot ItemType)
  (bind _returnvalue_2 (Niagara|SpawnSystematLocation "/Game/Particles/Magic/P_SmokeAndMirrors.P_SmokeAndMirrors" (Transformation|GetActorLocation _returnvalue) "0, 0, 0" "1.000000,1.000000,1.000000" false))
  (bind _returnvalue_3 (AddComponent|AddChildActorComponent false (Transformation|GetActorTransform _returnvalue)))
  (Utilities|FlowControl|Delay (Variables|Default|GetDuration))
  (Components|DestroyComponent _returnvalue_3))

(fn ConstructionScript
  (|CallParentFunction))

(fn GetEffectDescription
  (params (ItemType :type Data%20Table%20Row%20Handle%20Structure))
  (bind _statdescription (|CallParentFunction ItemType))
  (return _statdescription))