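; Trigger actor that grants a temporary Dodge bonus to the living party while the dungeon pawn is inside it.
; Begin overlap sets an in-radius flag and applies a small Dodge modifier to every living player character from the dungeon state.
; End overlap clears the flag and applies the same modifier with another manipulation mode, apparently to undo it.
; The actor's own damage and stat functions are empty stubs.
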(event Collision|EventActorBeginOverlap
  (params (OtherActor :type Actor%20Object%20Reference))
  (Utilities|Casting|CastToBP_DungeonPawn OtherActor)
  (Variables|Default|SetIs%20In%20Radius true)
  (bind _livingplayercharacters (Default|GetLivingPlayerCharacters (.DungeonState (CallFunction|GetDungeonGameState))))
  (for _array_element _livingplayercharacters
    (Default|ModifyStat _array_element 0.1 "(TagName=\"Stat.Dodge\")" false "NewEnumerator0" false false)))

(event Collision|EventActorEndOverlap
  (params (OtherActor :type Actor%20Object%20Reference))
  (Utilities|Casting|CastToBP_DungeonPawn OtherActor)
  (Variables|Default|SetIs%20In%20Radius false)
  (bind _livingplayercharacters (Default|GetLivingPlayerCharacters (.DungeonState (CallFunction|GetDungeonGameState))))
  (for _array_element _livingplayercharacters
    (Default|ModifyStat _array_element 0.1 "(TagName=\"Stat.Dodge\")" false "NewEnumerator1" false false)))

(fn ConstructionScript)

(fn TakeDamage
  (params (Damage :type Float%20%28double-precision%29)))

(fn GetStatValue
  (params (Stat :type Gameplay%20Tag%20Structure) (bBaseStat :type Boolean))
  (return 0.0))

(fn ModifyStat
  (params (Modifier :type Float%20%28double-precision%29) (Stat :type Gameplay%20Tag%20Structure) (bChangeBaseStat :type Boolean) (Manipulation :type EManipulate%20Enum :default "NewEnumerator0") (bUpdateDerivedStats :type Boolean) (bCanBeNegative :type Boolean))
  (return false 0.0))