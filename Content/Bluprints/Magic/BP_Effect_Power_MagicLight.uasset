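; Magic Light power effect that gives the player a temporary light hovering overhead.
; On use it adds a child actor component with a cast sound, then destroys it after the duration with an end Niagara effect and sound.
; Tick moves the light to a fixed height above the player pawn.
; An Activated flag and DoOnce block recasting while active, showing a warning and playing a fail sound instead.
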(event Custom|DeactivateLight
  (bind _returnvalue (Game|Player|GetPlayerPawn 0))
  (bind _returnvalue_2 (Transformation|GetActorLocation _returnvalue))
  (bind (_x _y _z) (Math|Vector|BreakVector _returnvalue_2))
  (Components|DestroyComponent (Variables|Default|GetMagicLight))
  (Niagara|SpawnSystematLocation "/Game/Particles/Magic/NS_PH_Light_End.NS_PH_Light_End" (Math|Vector|MakeVector _x _y (+ _z 5e+01)))
  (Audio|PlaySoundatLocation "/Game/Audio/Magic/A_Magic_Light_End_Cue.A_Magic_Light_End_Cue" _returnvalue_2 "0, 0, 0" 1.0 1.0 0.0 0 0 0 0)
  (Variables|Default|SetActivated false))

(event Custom|ActivateLight
  (bind _returnvalue (AddComponent|AddChildActorComponent false))
  (Variables|Default|SetMagicLight _returnvalue)
  (Variables|Default|SetActivated true))

(event EventUseEffect
  (params (ActivatingPlayerCharacter :type BP%20Player%20Character%20Object%20Reference) (ResidingSlot :type WBP%20Slot%20Object%20Reference) (ItemType :type Data%20Table%20Row%20Handle%20Structure))
  (bind _returnvalue (Game|Player|GetPlayerPawn 0))
  (bind _returnvalue_2 (Transformation|GetActorLocation _returnvalue))
  (|CallParentFunction ActivatingPlayerCharacter ResidingSlot ItemType)
  (if (Variables|Default|GetActivated)
    (Class|BPIPlayerController|DisplayWarning(Message) (Game|GetPlayerController 0) "This spell cannot be cast")
    (Audio|PlaySoundatLocation "/Game/Audio/Magic___Spell_Sounds_PRO/General/cue/Spell_Fail_08_Cue.Spell_Fail_08_Cue" _returnvalue_2 "0, 0, 0" 1.0 1.0 0.0 0 0 0 0)
    (else
      (Utilities|FlowControl|Sequence
        (:then_0
          (Utilities|FlowControl|DoOnce false :!label _label
            (:Completed
              (CallFunction|Activatelight)
              (Audio|PlaySoundatLocation "/Game/Audio/Magic/A_Magic_Light_Cast.A_Magic_Light_Cast" _returnvalue_2 "0, 0, 0" 1.0 1.0 0.0 0 0 0 0))))
        (:then_1
          (Utilities|FlowControl|Delay (Math|Conversions|ToFloat(Integer) (Variables|Default|GetDuration)))
          (CallFunction|DeactivateLight)
          (goto _label Reset))))))

(event EventTick
  (params (DeltaSeconds :type Float%20%28single-precision%29))
  (bind _returnvalue (Game|Player|GetPlayerPawn 0))
  (bind _magiclight (Variables|Default|GetMagicLight))
  (bind _returnvalue_2 (Transformation|GetActorLocation _returnvalue))
  (bind (_x _y _z) (Math|Vector|BreakVector _returnvalue_2))
  (if (Utilities|IsValid _magiclight)
    (Transformation|SetWorldLocation _magiclight (Math|Vector|MakeVector _x _y (+ _z 2e+02)) false false)))

(fn ConstructionScript
  (|CallParentFunction))

(fn GetEffectDescription
  (params (ItemType :type Data%20Table%20Row%20Handle%20Structure))
  (bind _statdescription (|CallParentFunction ItemType))
  (return _statdescription))