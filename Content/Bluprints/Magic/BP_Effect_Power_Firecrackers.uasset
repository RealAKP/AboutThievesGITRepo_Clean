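; Firecrackers power effect that sets off a volley of five explosions on the dungeon tile adjacent to the player.
; On use, a Sequence fires one burst immediately and four after random sub-second delays, each with scattered Niagara FX, a sound and its own Strike.
; Each Strike re-queries that tile through the dungeon manager, deals random damage to monsters found, or spawns floating "MISS" text.
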(event Custom|Miss
  (bind _returnvalue (Game|Player|GetPlayerPawn 0))
  (bind _returnvalue_2 (Transformation|GetActorForwardVector _returnvalue))
  (bind _returnvalue_3 (Transformation|GetActorLocation _returnvalue))
  (bind _returnvalue_4 (* _returnvalue_2 1.5e+02))
  (bind _returnvalue_5 (+ _returnvalue_3 _returnvalue_4))
  (Game|SpawnActorfromClass "/Game/DCT/Blueprints/Core/BP_FloatingText.BP_FloatingText_C" (Math|Transform|MakeTransform (+ _returnvalue_5 "0, 0,100.000000") (Math|Rotator|FindLookatRotation _returnvalue_5 _returnvalue_3) "0.800000,0.800000,0.800000") "AlwaysSpawn" 0 "MISS" 0))

(event Custom|Hit
  (params (Target :type Actor%20Object%20Reference) (Damage :type Float%20%28double-precision%29))
  (Class|BPIAttackTarget|TakeDamage(Message) Target Damage))

(event Custom|Strike
  (bind (_bsuccess _targets) (CallFunction|FindValidTarget))
  (if _bsuccess
    (for _array_element _targets
      (CallFunction|Hit _array_element (Math|Conversions|ToFloat(Integer) (Math|Random|RandomIntegerinRange 6 18))))
    (else
      (CallFunction|Miss))))

(event EventUseEffect
  (params (ActivatingPlayerCharacter :type BP%20Player%20Character%20Object%20Reference) (ResidingSlot :type WBP%20Slot%20Object%20Reference) (ItemType :type Data%20Table%20Row%20Handle%20Structure))
  (bind _returnvalue (Math|Random|RandomFloatinRange 0.0 4e+01))
  (bind _returnvalue_2 (Math|Random|RandomFloatinRange 1e+01 1e+02))
  (bind _returnvalue_3 (Math|Random|RandomFloatinRange 0.0 5e+01))
  (bind _returnvalue_4 (Math|Random|RandomFloatinRange 1e+01 6e+01))
  (bind _returnvalue_5 (Game|Player|GetPlayerPawn 0))
  (bind _returnvalue_6 (Math|Random|RandomFloatinRange 1e+01 1e+02))
  (bind _returnvalue_7 (Transformation|GetActorLocation _returnvalue_5))
  (|CallParentFunction ActivatingPlayerCharacter ResidingSlot ItemType)
  (bind _adjacenttilelocation (Default|GetAdjacentTilefromLocation (.DungeonManager (CallFunction|GetDungeonManager)) _returnvalue_5 "NewEnumerator0"))
  (Utilities|FlowControl|Sequence
    (:then_0
      (Niagara|SpawnSystematLocation "/Game/Particles/Magic/NS_Fireckracker.NS_Fireckracker" (+ _adjacenttilelocation (Math|Vector|MakeVector _returnvalue _returnvalue 0.0)))
      (Audio|PlaySoundatLocation "/Game/Audio/Magic/S_Firecracker_Cue.S_Firecracker_Cue" _returnvalue_7 "0, 0, 0" 1.0 1.0 0.0 0 0 0 0)
      (CallFunction|Strike))
    (:then_1
      (Utilities|FlowControl|Delay (Math|Random|RandomFloatinRange 0.0 1.0))
      (Niagara|SpawnSystematLocation "/Game/Particles/Magic/NS_Fireckracker.NS_Fireckracker" (+ _adjacenttilelocation (Math|Vector|MakeVector _returnvalue_3 _returnvalue_3 0.0)))
      (Audio|PlaySoundatLocation "/Game/Audio/Magic/S_Firecracker_Cue.S_Firecracker_Cue" _returnvalue_7 "0, 0, 0" 1.0 1.0 0.0 0 0 0 0)
      (CallFunction|Strike))
    (:then_2
      (Utilities|FlowControl|Delay (Math|Random|RandomFloatinRange 0.1 1.0))
      (Niagara|SpawnSystematLocation "/Game/Particles/Magic/NS_Fireckracker.NS_Fireckracker" (+ _adjacenttilelocation (Math|Vector|MakeVector _returnvalue_4 _returnvalue_4 0.0)))
      (Audio|PlaySoundatLocation "/Game/Audio/Magic/S_Firecracker_Cue.S_Firecracker_Cue" _returnvalue_7 "0, 0, 0" 1.0 1.0 0.0 0 0 0 0)
      (CallFunction|Strike))
    (:then_3
      (Utilities|FlowControl|Delay (Math|Random|RandomFloatinRange 0.3 1.0))
      (Niagara|SpawnSystematLocation "/Game/Particles/Magic/NS_Fireckracker.NS_Fireckracker" (+ _adjacenttilelocation (Math|Vector|MakeVector _returnvalue_6 _returnvalue_6 0.0)))
      (Audio|PlaySoundatLocation "/Game/Audio/Magic/S_Firecracker_Cue.S_Firecracker_Cue" _returnvalue_7 "0, 0, 0" 1.0 1.0 0.0 0 0 0 0)
      (CallFunction|Strike))
    (:then_4
      (Utilities|FlowControl|Delay (Math|Random|RandomFloatinRange 0.3 1.0))
      (Niagara|SpawnSystematLocation "/Game/Particles/Magic/NS_Fireckracker.NS_Fireckracker" (+ _adjacenttilelocation (Math|Vector|MakeVector _returnvalue_2 _returnvalue_2 0.0)))
      (Audio|PlaySoundatLocation "/Game/Audio/Magic/S_Firecracker_Cue.S_Firecracker_Cue" _returnvalue_7 "0, 0, 0" 1.0 1.0 0.0 0 0 0 0)
      (CallFunction|Strike))))

(fn ConstructionScript
  (|CallParentFunction))

(fn GetEffectDescription
  (params (ItemType :type Data%20Table%20Row%20Handle%20Structure))
  (bind _statdescription (|CallParentFunction ItemType))
  (return (Utilities|String|Append _statdescription "")))

(fn FindValidTarget
  (bind _localtargets (LocalVariables|GetLocalTargets))
  (bind _returnvalue (Actor|GetActorOfClass "/Game/DCT/Blueprints/Core/BP_DungeonManager.BP_DungeonManager_C"))
  (bind _adjacentgridindex (Default|GetAdjacentTilefromLocation _returnvalue (Game|Player|GetPlayerPawn 0) "NewEnumerator0"))
  (bind (_bobjectfound _objectrefs) (Default|GetAllObjectsonTile _returnvalue _adjacentgridindex))
  (if _bobjectfound
    (for _array_element _objectrefs
      (bind _asbp_monster (Utilities|Casting|CastToBP_Monster _array_element))
      (Utilities|Array|Add (LocalVariables|GetLocalTargets) _asbp_monster))
    (return (> (Utilities|Array|Length _localtargets) 0) _localtargets)
    (else
      (return false 0))))