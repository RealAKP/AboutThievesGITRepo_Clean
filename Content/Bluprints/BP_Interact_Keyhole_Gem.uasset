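; Interactable gem keyhole that powers linked actors once, reversible via ReversedPower, when used with the matching key item held on the cursor.
; The interaction check compares the mouse-follow widget's item row to RequiredKey, whose data-table mesh material also colors the lock at construction.
; Unlocking plays a sound and shows a key mesh, rotated by a timeline, then hidden.
; Cursor hover toggles a material Highlight parameter.
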(event MouseInput|EventActorBeginCursorOver
  (Rendering|Material|SetScalarParameterValueonMaterials (Variables|Default|GetLockMesh) "Highlight" 1.0))

(event MouseInput|EventActorEndCursorOver
  (Rendering|Material|SetScalarParameterValueonMaterials (Variables|Default|GetLockMesh) "Highlight" 0.0))

(event EventInteract
  (params (TriggeringActor :type Actor%20Object%20Reference))
  (bind _sm_item_sewers_key (Variables|Default|GetSM_Item_Sewers_Key))
  (Utilities|FlowControl|DoOnce false
    (:Completed
      (CallFunction|PowerActors (select (Variables|Default|GetbReversedPower) "NewEnumerator0" "NewEnumerator2"))
      (Audio|PlaySoundatLocation "/Game/Audio/Items/A_Lock_Opening_Short_Cue.A_Lock_Opening_Short_Cue" (Transformation|GetActorLocation) "0, 0, 0" 1.0 1.0 0.0 "/Game/DCT/Sound/ATT_Dungeon.ATT_Dungeon" 0 0 0)
      (Rendering|SetVisibility _sm_item_sewers_key true false)
      (bind _key_rotation (Timeline|Timeline_0 Play)
        (:Update
          (Transformation|AddRelativeRotation _sm_item_sewers_key (Math|Rotator|MakeRotator (* _key_rotation 1e+01) 0.0 0.0) false false))
        (:Finished
          (Utilities|FlowControl|Delay 0.2)
          (Rendering|SetVisibility _sm_item_sewers_key false false))))))

(fn ConstructionScript
  (bind _requiredkey (Variables|Default|GetRequiredKey))
  (|CallParentFunction)
  (bind _returnvalue (Utilities|GetDataTableRow (.datatable _requiredkey) (.rowname _requiredkey))
    (:then
      (Rendering|Material|SetMaterial (Variables|Default|GetLockMesh) 1 (Rendering|Material|GetMaterial (Utilities|Struct|BreakFItem _returnvalue) 0)))))

(fn CheckifAllowedInteract
  (params (TriggeringActor :type Object%20Object%20Reference))
  (bind _ballowed (|CallParentFunction TriggeringActor))
  (if (and _ballowed (Utilities|IsValid (Variables|/Game/DCT/Blueprints/Core/BP_PC_Dungeon.BP_PC_Dungeon_C|GetMouseFollowWidget (.DungeonPlayerController (CallFunction|GetDungeonPlayerController)))))
    (return (Utilities|Name|Equal(Name) (.rowname (Variables|Default|GetRequiredKey)) (.rowname (Variables|/Game/DCT/UserInterface/WBP_Item.WBP_Item_C|GetItemType (Variables|/Game/DCT/Blueprints/Core/BP_PC_Dungeon.BP_PC_Dungeon_C|GetMouseFollowWidget (.DungeonPlayerController (CallFunction|GetDungeonPlayerController)))))))
    (else
      (return false))))