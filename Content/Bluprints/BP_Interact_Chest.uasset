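; Interactable dungeon chest that opens once when powered and highlights its lid under the cursor.
; Power plays a lock sound and runs a timeline that rotates the lid open, then marks the chest as PostInteract.
; It also tells a triggering BP_DungeonPawn to Peak at the chest using the PeakArrow transform.
; UpdateStateInstantly sets the open flag from a desired state and resets the timeline time.
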(event MouseInput|EventActorBeginCursorOver
  (Rendering|Material|SetScalarParameterValueonMaterials (Variables|Default|GetChestLid) "Highlight" 1.0))

(event EventPower
  (params (TriggeringActor :type Actor%20Object%20Reference) (DesiredState :type EInteractState%20Enum :default "NewEnumerator0"))
  (Variables|Default|SetDesiredState "NewEnumerator2")
  (Utilities|FlowControl|Sequence
    (:then_0
      (if (not (Variables|Default|GetbOpen))
        (Utilities|FlowControl|DoOnce false
          (:Completed
            (Audio|PlaySoundatLocation "/Game/DCT/Sound/A_Lock.A_Lock" (Transformation|GetActorLocation) "0, 0, 0" 1.0 1.0 0.0 "/Game/DCT/Sound/ATT_Dungeon.ATT_Dungeon" 0 0 0)
            (bind _open (Timeline|TL_Open PlayFromStart)
              (:Update
                (Transformation|SetRelativeRotation (Variables|Default|GetChestLid) (Math|Rotator|MakeRotator (* _open -1.1e+02) 0.0 0.0) false false))
              (:Finished
                (Variables|Default|SetInteractState "NewEnumerator2")
                (Variables|Default|SetbOpen true)))))))
    (:then_1
      (bind _triggeringactor (Variables|Default|GetTriggeringActor)
        (:then
          (bind _asbp_dungeon_pawn (Utilities|Casting|CastToBP_DungeonPawn _triggeringactor))
          (Default|Peak _asbp_dungeon_pawn (Transformation|GetWorldTransform (Variables|Default|GetPeakArrow)) self)
          (if (Variables|Default|GetbOpen)
            (Variables|Default|SetInteractState "NewEnumerator2")))
        (:else)))))

(event MouseInput|EventActorEndCursorOver
  (Rendering|Material|SetScalarParameterValueonMaterials (Variables|Default|GetChestLid) "Highlight" 0.0))

(event EventUpdateStateInstantly
  (params (DesiredState :type EInteractState%20Enum :default "NewEnumerator0"))
  (Variables|Default|SetbOpen (Utilities|Select :Index DesiredState :NewEnumerator0 false :NewEnumerator2 true))
  (bind _open (Timeline|TL_Open SetNewTime)
    (:Update
      (Transformation|SetRelativeRotation (Variables|Default|GetChestLid) (Math|Rotator|MakeRotator (* _open -1.1e+02) 0.0 0.0) false false))
    (:Finished
      (Variables|Default|SetInteractState "NewEnumerator2")
      (Variables|Default|SetbOpen true))))

(fn ConstructionScript
  (|CallParentFunction))