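; BP_Lamp_Toggle is a child lamp Blueprint that switches its flame and glow on and off with the flicker state.
; EventFlickering shows the SMFLAMENEW flame and PointLightGlow, then calls the parent event.
; EventFlickeringSTOP hides both components, then calls the parent event.
; The construction script only calls the parent, so any flicker behavior itself lies outside this Blueprint.
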(event Custom|EventFlickeringSTOP
  (Rendering|SetVisibility (Variables|Default|GetPointLight_Glow) false false)
  (|CallParentFunction))

(event Custom|EventFlickering
  (Rendering|SetVisibility (Variables|Default|GetSM_FLAME_NEW) true false)
  (|CallParentFunction))

(fn ConstructionScript
  (|CallParentFunction))