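; Trigger actor that recovers lost items by teleporting them back to the player, despite the "AnyActor" name.
; On begin overlap it prints a debug "Zgubione" (lost) message, then continues only if the actor casts to BP_Item.
; It prints the item's name and teleports it to just above player pawn 0.
; The damage and stat functions are empty stubs.
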(event Collision|EventActorBeginOverlap
  (params (OtherActor :type Actor%20Object%20Reference))
  (bind _returnvalue (Game|Player|GetPlayerPawn 0))
  (bind _returnvalue_2 (Transformation|GetActorLocation _returnvalue))
  (if (Collision|IsOverlappingActor OtherActor :!class /Script/Engine.Actor)
    (Development|PrintString "Zgubione" true false)
    (bind _asbp_item (Utilities|Casting|CastToBP_Item OtherActor))
    (Development|PrintString (Utilities|String|ToString(Name) (Default|GetItemName _asbp_item)) true false)
    (Transformation|SetActorLocation OtherActor (Math|Vector|MakeVector (.x _returnvalue_2) (.y _returnvalue_2) (+ (.z _returnvalue_2) 8e+01)) false true)))

(fn ConstructionScript)

(fn TakeDamage
  (params (Damage :type Float%20%28double-precision%29)))

(fn GetStatValue
  (params (Stat :type Gameplay%20Tag%20Structure) (bBaseStat :type Boolean))
  (return 0.0))

(fn ModifyStat
  (params (Modifier :type Float%20%28double-precision%29) (Stat :type Gameplay%20Tag%20Structure) (bChangeBaseStat :type Boolean) (Manipulation :type EManipulate%20Enum :default "NewEnumerator0") (bUpdateDerivedStats :type Boolean) (bCanBeNegative :type Boolean))
  (return false 0.0))