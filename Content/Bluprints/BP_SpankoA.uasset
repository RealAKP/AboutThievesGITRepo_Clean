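; BP_SpankoA is a sleep point in a dungeon crawler that highlights on cursor hover and rests the party when its Power event fires.
; It refuses with a warning during cooldown or when the monster sight check, evaluated only for the loop's last monster, finds a living watcher.
; Resting restores living characters' health and mana, saves the game, and briefly shows WBP_Spanko with input disabled before a timed cooldown.
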(event MouseInput|EventActorBeginCursorOver
  (Rendering|Material|SetScalarParameterValueonMaterials (Variables|Default|GetStaticMesh) "Highlight" 1.0))

(event MouseInput|EventActorEndCursorOver
  (Rendering|Material|SetScalarParameterValueonMaterials (Variables|Default|GetStaticMesh) "Highlight" 0.0))

(event EventPower
  (params (TriggeringActor :type Actor%20Object%20Reference) (DesiredState :type EInteractState%20Enum :default "NewEnumerator0"))
  (bind _returnvalue (Game|Player|GetPlayerPawn 0))
  ;[0.2969 0.09269 0] Timer Check
  (if (Variables|Default|GetWaitEnded)
    (Development|PrintString "SLEEP TRIGGERED")
    ;[0 0.3073 0.09852] Nearby Monsters Check
    (bind _outactors (Actor|GetAllActorsOfClass "/Game/DCT/Blueprints/Monsters/BP_Monster.BP_Monster_C"))
    (for _array_element _outactors
      (bind _bactorfound (Default|LookforActor _array_element (.DungeonPawn (CallFunction|GetDungeonPawn)) false "TraceTypeQuery1")))
    (if _bactorfound
      (if (Variables|/Game/DCT/Blueprints/Monsters/BP_Monster.BP_Monster_C|GetbDead _array_element)
        (Development|PrintString "DED NO PROBLEM!")
        (Variables|Default|SetWaitEnded false :!label _label)
        (Input|DisableInput _returnvalue 0)
        (Utilities|Casting|CastToBP_DungeonPawn _returnvalue)
        (bind _livingplayercharacters (Default|GetLivingPlayerCharacters (.DungeonState (CallFunction|GetDungeonGameState))))
        (for _array_element_2 _livingplayercharacters
          (Default|ModifyStatCapped _array_element_2 "(TagName=\"Stat.Health\")" 3e+02)
          (Default|ModifyStatCapped _array_element_2 "(TagName=\"Stat.Mana\")" 1e+03))
        (Default|SaveAll (.DungeonInstance (CallFunction|GetDungeonGameInstance)) true)
        (bind _returnvalue_2 (UserInterface|CreateWidget "/Game/DCT/UserInterface/WBP_Spanko.WBP_Spanko_C"))
        (UserInterface|Viewport|AddtoViewport _returnvalue_2 0)
        (Utilities|FlowControl|Delay 5.0)
        (Widget|RemovefromParent _returnvalue_2)
        (Input|EnableInput _returnvalue 0)
        (Utilities|FlowControl|Delay 6e+01)
        (Variables|Default|SetWaitEnded true)
        (else
          (Class|BPIPlayerController|DisplayWarning(Message) (Game|GetPlayerController 0) (Variables|Default|GetMessage%20Monsters))))
      (else
        (Development|PrintString "NO MONSTERS")
        (goto _label)))
    (else
      (Class|BPIPlayerController|DisplayWarning(Message) (Game|GetPlayerController 0) (Variables|Default|GetMessage%20Delay)))))

(fn ConstructionScript
  (|CallParentFunction))