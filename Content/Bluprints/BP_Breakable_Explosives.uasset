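; BP_Breakable_Explosives is a destructible explosive prop that occupies a tile on the dungeon grid.
; On BeginPlay it finds a nearby valid tile through the DungeonManager, blocks it and registers itself there.
; Damage lowers Health and spawns red floating text; at depletion it unregisters, spawns effects, a destroyed version and a short-lived explosion damage trigger, then destroys itself and reopens the tile.
; It rejects interaction and returns a negative dodge chance.
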(event EventBeginPlay
  (|CallParentFunction)
  (Utilities|FlowControl|Delay 0.0)
  (bind _gridindex (Default|FindNearbyValidTile (.DungeonManager (CallFunction|GetDungeonManager)) (Transformation|GetActorLocation)))
  (Variables|Default|SetGridIndex _gridindex)
  (Default|BlockTile (.DungeonManager (CallFunction|GetDungeonManager)) (Variables|Default|GetGridIndex))
  (Default|AddObjecttoGrid (.DungeonManager (CallFunction|GetDungeonManager)) self (Variables|Default|GetGridIndex)))

(event EventTakeDamage
  (params (Damage :type Float%20%28double-precision%29))
  (bind _returnvalue (Transformation|GetActorTransform))
  (bind _returnvalue_2 (Transformation|GetActorLocation))
  (Variables|Default|SetHealth (- (Variables|Default|GetHealth) Damage))
  (bind _returnvalue_3 (Game|SpawnActorfromClass "/Game/DCT/Blueprints/Core/BP_FloatingText.BP_FloatingText_C" (Math|Transform|MakeTransform (+ (Transformation|GetActorLocation) "0,0.000000,150.000000") "0, 0, 0" "1.000000,1.000000,1.000000") "AlwaysSpawn" "OverrideRootScale" 0 (Utilities|Text|ToText(Float) Damage "HalfToEven") 0))
  (Default|SetColor _returnvalue_3 "(R=1.000000,G=0.008023,B=0.009721,A=1.000000)")
  (if (< (Variables|Default|GetHealth) 1.0)
    (Default|RemoveObjectfromGrid (.DungeonManager (CallFunction|GetDungeonManager)) self (Variables|Default|GetGridIndex))
    (Niagara|SpawnSystematLocation (Variables|Default|GetBreakSystem) _returnvalue_2)
    (Game|SpawnActorfromClass "/Game/Bluprints/BP_Breakable_Explosives_Destroyed.BP_Breakable_Explosives_Destroyed_C" _returnvalue "Undefined" "OverrideRootScale" 0 0)
    (Audio|PlaySoundatLocation "/Game/Audio/Chaos/A_Explosion_Cue.A_Explosion_Cue" _returnvalue_2 "0, 0, 0" 1.0 1.0 0.0 0 0 0 0)
    (bind _returnvalue_4 (Game|SpawnActorfromClass "/Game/Bluprints/BP_Trigger_Damage_Explosion.BP_Trigger_Damage_Explosion_C" _returnvalue "Undefined" "OverrideRootScale" 0 0))
    (Utilities|FlowControl|Delay 0.2)
    (Actor|DestroyActor _returnvalue_4)
    (Actor|DestroyActor)
    (Default|ReopenTile (.DungeonManager (CallFunction|GetDungeonManager)) (Variables|Default|GetGridIndex))))

(fn ConstructionScript)

(fn GetWeight
  (return 1.0))

(fn AttemptInteract
  (params (TriggeringActor :type Actor%20Object%20Reference))
  (return false))

(fn GetDodgeChance
  (return -0.5))