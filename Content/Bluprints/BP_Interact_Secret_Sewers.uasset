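; Interactable secret sewer door that slides vertically between pre- and post-interact states in the dungeon.
; Activation drives a timeline that moves the door, with start, chain and closing sounds.
; The blocking box's collision follows the desired state, and instant state updates skip the animation.
; Dungeon tiles nearby refresh when movement starts and ends, after which monsters are forced to look for the player.
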(event EventUpdateStateInstantly
  (params (DesiredState :type EInteractState%20Enum :default "NewEnumerator0"))
  (Variables|Default|SetDesiredState DesiredState)
  (Utilities|FlowControl|Sequence
    (:then_0
      (bind _open (Timeline|TL_Open SetNewTime)
        (:Update
          (CallFunction|MoveDoor _open))
        (:Finished
          (Utilities|FlowControl|Sequence
            (:then_0
              (Collision|SetCollisionEnabled (Variables|Default|GetWallBlockingBox) (Utilities|Select :Index (Variables|Default|GetDesiredState) :NewEnumerator0 "QueryOnly" :NewEnumerator2 "NoCollision") :!label _label))
            (:then_1
              (Audio|PlaySoundatLocation "/Game/Audio/Doors/A_Doors_Closed_Cue.A_Doors_Closed_Cue" (Transformation|GetActorLocation) "0, 0, 0" 1.0 1.0 0.0 "/Game/DCT/Sound/ATT_Dungeon.ATT_Dungeon" 0 0 0)
              (Components|Activation|SetActive (Variables|Default|GetA_Doors_Chain_Cue) false false)
              (Default|UpdateTilesinRange (.DungeonManager (CallFunction|GetDungeonManager)) 2 0 (Transformation|GetActorLocation) false)
              (Variables|Default|SetInteractState (Variables|Default|GetDesiredState))
              (CallFunction|ForceMonstersLookforPlayer))))))
    (:then_1
      (goto _label))))

(event EventUpdateDesiredState
  (params (NewState :type EInteractState%20Enum :default "NewEnumerator0"))
  (|CallParentFunction NewState))

(event EventBeginPlay
  (|CallParentFunction)
  (Collision|SetCollisionEnabled (Variables|Default|GetWallBlockingBox) (Utilities|Select :Index (Variables|Default|GetDesiredState) :NewEnumerator0 "QueryOnly" :NewEnumerator2 "NoCollision")))

(event EventActivate
  (params (bTurnOn :type Boolean) (TriggeringActor :type Actor%20Object%20Reference))
  (bind _a_doors_chain_cue (Variables|Default|GetA_Doors_Chain_Cue))
  (Collision|SetCollisionEnabled (Variables|Default|GetWallBlockingBox) "QueryAndPhysics")
  (Default|UpdateTilesinRange (.DungeonManager (CallFunction|GetDungeonManager)) 2 0 (Transformation|GetActorLocation) false)
  (if (Audio|Components|Audio|IsPlaying (Variables|Default|GetTL_Open))
    _
    (else
      (Audio|PlaySoundatLocation "/Game/Audio/Doors/A_Doors_Start_Cue.A_Doors_Start_Cue" (Transformation|GetActorLocation) "0, 0, 0" 1.0 1.0 0.0 "/Game/DCT/Sound/ATT_Dungeon.ATT_Dungeon" 0 0 0)))
  (switch Utilities|FlowControl|Switch|SwitchonEInteractState (Variables|Default|GetDesiredState)
    (:NewEnumerator0
      (Components|Activation|SetActive _a_doors_chain_cue true true)
      (bind _open (Timeline|TL_Open Reverse)
        (:Update
          (CallFunction|MoveDoor _open))
        (:Finished
          (Utilities|FlowControl|Sequence
            (:then_0
              (Collision|SetCollisionEnabled (Variables|Default|GetWallBlockingBox) (Utilities|Select :Index (Variables|Default|GetDesiredState) :NewEnumerator0 "QueryOnly" :NewEnumerator2 "NoCollision")))
            (:then_1
              (Audio|PlaySoundatLocation "/Game/Audio/Doors/A_Doors_Closed_Cue.A_Doors_Closed_Cue" (Transformation|GetActorLocation) "0, 0, 0" 1.0 1.0 0.0 "/Game/DCT/Sound/ATT_Dungeon.ATT_Dungeon" 0 0 0)
              (Components|Activation|SetActive (Variables|Default|GetA_Doors_Chain_Cue) false false)
              (Default|UpdateTilesinRange (.DungeonManager (CallFunction|GetDungeonManager)) 2 0 (Transformation|GetActorLocation) false)
              (Variables|Default|SetInteractState (Variables|Default|GetDesiredState))
              (CallFunction|ForceMonstersLookforPlayer))))))
    (:NewEnumerator2
      (Components|Activation|SetActive _a_doors_chain_cue true true)
      (Timeline|TL_Open Play))))

(fn ConstructionScript
  (|CallParentFunction)
  (Collision|SetCollisionEnabled (Variables|Default|GetWallBlockingBox) (Utilities|Select :Index (Variables|Default|GetDesiredState) :NewEnumerator0 "QueryOnly" :NewEnumerator2 "NoCollision")))

(fn MoveDoor
  (params (PercentOpen :type Float%20%28double-precision%29))
  (Transformation|SetRelativeLocation (Variables|Default|GetDoor) (Math|Vector|MakeVector 0.0 0.0 (* PercentOpen 2e+02)) false false))

(fn GetAttachSlot
  (return (Variables|Default|GetAttachSlot)))