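; Interactable sliding door that runs a one-time scripted cutscene when activated.
; Activation disables player input, then timed delays sequence banging and unlock sounds, the GryzomirSEQ level sequence and two typewriter character dialog widgets before input returns.
; Cursor hover toggles a material highlight on the door.
; The construction script sets blocking-box collision from the interact state, and MoveDoor maps open percentage to vertical door offset.
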(event MouseInput|EventActorBeginCursorOver
  (Rendering|Material|SetScalarParameterValueonMaterials (Variables|Default|GetDoor) "Highlight" 1.0))

(event MouseInput|EventActorEndCursorOver
  (Rendering|Material|SetScalarParameterValueonMaterials (Variables|Default|GetDoor) "Highlight" 0.0))

(event EventActivate
  (params (bTurnOn :type Boolean) (TriggeringActor :type Actor%20Object%20Reference))
  (bind _door (Variables|Default|GetDoor))
  (bind _returnvalue (Transformation|GetWorldLocation _door))
  (Utilities|FlowControl|DoOnce false
    (:Completed
      (Variables|Default|SetDesiredState "NewEnumerator0")
      (Input|DisableInput (Game|Player|GetPlayerPawn 0) (Game|GetPlayerController 0))
      ;[1 1 1] Pukanie do drzwi
      (Audio|PlaySoundatLocation "/Game/Audio/Doors/A_Doors_Banging_Cue.A_Doors_Banging_Cue" _returnvalue "0, 0, 0" 1.2 1.0 0.0 "/Game/Audio/SA_Buttons_Levers.SA_Buttons_Levers" 0 0 0)
      (Utilities|FlowControl|Delay 1.5)
      ;[1 1 1] Klucz
      (Audio|PlaySoundatLocation "/Game/Audio/Items/A_Lock_Opening_Cue.A_Lock_Opening_Cue" _returnvalue "0, 0, 0" 0.5 1.0 0.0 "/Game/Audio/SA_Buttons_Levers.SA_Buttons_Levers" 0 0 0)
      (Utilities|FlowControl|Delay 4.0)
      (bind _returnvalue_2 (Sequencer|Player|CreateLevelSequencePlayer (Variables|Default|GetGryzomir_SEQ)))
      (Sequencer|Player|Play _returnvalue_2 :!class /Script/MovieScene.MovieSceneSequencePlayer)
      (Utilities|FlowControl|Delay 2.0)
      (bind _returnvalue_3 (UserInterface|CreateWidget "/Game/DCT/UserInterface/WBP_Character_Dialog.WBP_Character_Dialog_C" (Game|GetPlayerController 0) 0))
      (Variables|/Game/DCT/UserInterface/WBP_Character_Dialog.WBP_Character_Dialog_C|SetX%20Visibility _returnvalue_3 "Hidden")
      (Variables|/Game/DCT/UserInterface/WBP_Character_Dialog.WBP_Character_Dialog_C|SetDialog%20Text _returnvalue_3 (Variables|Default|GetDialog%20Text))
      (Variables|/Game/DCT/UserInterface/WBP_Character_Dialog.WBP_Character_Dialog_C|SetCharacter%20Name _returnvalue_3 (Variables|Default|GetCharacter%20Name))
      (UserInterface|Viewport|AddtoViewport _returnvalue_3 -1)
      (Default|InitiateTypewrite _returnvalue_3)
      (Class|Image|SetBrush (Variables|/Game/DCT/UserInterface/WBP_Character_Dialog.WBP_Character_Dialog_C|GetPortrait _returnvalue_3) (Utilities|Struct|MakeSlateBrush "(SpecifiedColor=(R=1.000000,G=1.000000,B=1.000000,A=1.000000),ColorUseRule=UseColor_Specified)" "Image" "NoTile" "NoMirror" "(X=96.000000,Y=96.000000)" "(Left=0.000000,Top=0.000000,Right=0.000000,Bottom=0.000000)" "/Game/Textures/Interface/Portraits/S_P_Gryzomir.S_P_Gryzomir" "(CornerRadii=(X=0.000000,Y=0.000000,Z=0.000000,W=0.000000),Color=(SpecifiedColor=(R=0.000000,G=0.000000,B=0.000000,A=0.000000),ColorUseRule=UseColor_Specified),Width=0.000000,RoundingType=HalfHeightRadius,bUseBrushTransparency=False)"))
      (Utilities|FlowControl|Delay 15.0)
      (Widget|RemovefromParent _returnvalue_3)
      (bind _returnvalue_4 (UserInterface|CreateWidget "/Game/DCT/UserInterface/WBP_Character_Dialog.WBP_Character_Dialog_C" (Game|GetPlayerController 0) 0))
      (Variables|/Game/DCT/UserInterface/WBP_Character_Dialog.WBP_Character_Dialog_C|SetX%20Visibility _returnvalue_4 "Hidden")
      (Variables|/Game/DCT/UserInterface/WBP_Character_Dialog.WBP_Character_Dialog_C|SetDialog%20Text _returnvalue_4 (Variables|Default|GetDialog%20Text%202))
      (Variables|/Game/DCT/UserInterface/WBP_Character_Dialog.WBP_Character_Dialog_C|SetCharacter%20Name _returnvalue_4 (Variables|Default|GetCharacter%20Name))
      (Class|Image|SetBrush (Variables|/Game/DCT/UserInterface/WBP_Character_Dialog.WBP_Character_Dialog_C|GetPortrait _returnvalue_4) (Utilities|Struct|MakeSlateBrush "(SpecifiedColor=(R=1.000000,G=1.000000,B=1.000000,A=1.000000),ColorUseRule=UseColor_Specified)" "Image" "NoTile" "NoMirror" "(X=96.000000,Y=96.000000)" "(Left=0.000000,Top=0.000000,Right=0.000000,Bottom=0.000000)" "/Game/Textures/Interface/Portraits/S_P_Gryzomir.S_P_Gryzomir" "(CornerRadii=(X=0.000000,Y=0.000000,Z=0.000000,W=0.000000),Color=(SpecifiedColor=(R=0.000000,G=0.000000,B=0.000000,A=0.000000),ColorUseRule=UseColor_Specified),Width=0.000000,RoundingType=HalfHeightRadius,bUseBrushTransparency=False)"))
      (UserInterface|Viewport|AddtoViewport _returnvalue_4 -1)
      (Default|InitiateTypewrite _returnvalue_4)
      (Utilities|FlowControl|Delay 1e+01)
      (Input|EnableInput (Game|Player|GetPlayerPawn 0) (Game|GetPlayerController 0)))))

(fn ConstructionScript
  (|CallParentFunction)
  (Collision|SetCollisionEnabled (Variables|Default|GetWallBlockingBox) (Utilities|Select :Index (Variables|Default|GetDesiredState) :NewEnumerator0 "QueryOnly" :NewEnumerator2 "NoCollision")))

(fn MoveDoor
  (params (PercentOpen :type Float%20%28double-precision%29))
  (Transformation|SetRelativeLocation (Variables|Default|GetDoor) (Math|Vector|MakeVector 0.0 0.0 (* PercentOpen 2e+02)) false false))

(fn GetAttachSlot
  (return (Variables|Default|GetAttachSlot)))