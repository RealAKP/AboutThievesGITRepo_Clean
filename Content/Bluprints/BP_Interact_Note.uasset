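; BP_Interact_Note is an interactable note actor that shows its text on screen.
; Its Power event sets DesiredState, then creates a WBP_Note widget for the first player controller, passes it NoteText and adds it to the viewport.
; Cursor hover toggles a Highlight scalar parameter on the SMNote mesh's materials.
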(event MouseInput|EventActorBeginCursorOver
  (Rendering|Material|SetScalarParameterValueonMaterials (Variables|Default|GetSM_Note) "Highlight" 1.0))

(event EventPower
  (params (TriggeringActor :type Actor%20Object%20Reference) (DesiredState :type EInteractState%20Enum :default "NewEnumerator0"))
  (Variables|Default|SetDesiredState "NewEnumerator2")
  (bind _returnvalue (UserInterface|CreateWidget "/Game/DCT/UserInterface/WBP_Note.WBP_Note_C" (Game|GetPlayerController 0)))
  (Variables|/Game/DCT/UserInterface/WBP_Note.WBP_Note_C|SetNote%20Text _returnvalue (Variables|Default|GetNote%20Text))
  (UserInterface|Viewport|AddtoViewport _returnvalue 0))

(event MouseInput|EventActorEndCursorOver
  (Rendering|Material|SetScalarParameterValueonMaterials (Variables|Default|GetSM_Note) "Highlight" 0.0))

(fn ConstructionScript)