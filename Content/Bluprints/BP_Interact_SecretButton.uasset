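; BP_Interact_SecretButton is an interactable stone-sounding button that powers other actors when pressed.
; Activate, ignored while the press timeline plays, plays a sound and runs the timeline to slide the button mesh along its local Y axis.
; When the timeline finishes, it calls PowerActors.
; Cursor hover toggles a Highlight material parameter on the button.
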(event MouseInput|EventActorBeginCursorOver
  (Rendering|Material|SetScalarParameterValueonMaterials (Variables|Default|GetButton) "Highlight" 1.0))

(event EventActivate
  (params (bTurnOn :type Boolean) (TriggeringActor :type Actor%20Object%20Reference))
  (bind _button (Variables|Default|GetButton))
  (bind _relativelocation (Variables|/Script/Engine.SceneComponent|GetRelativeLocation _button))
  (if (not (Audio|Components|Audio|IsPlaying (Variables|Default|GetTL_Press)))
    (Audio|PlaySoundatLocation "/Game/Audio/Items/A_Stone_Button_Cue.A_Stone_Button_Cue" (Transformation|GetActorLocation) "0, 0, 0" 1.0 1.0 0.0 "/Game/DCT/Sound/ATT_Dungeon.ATT_Dungeon" 0 0 0)
    (bind _press (Timeline|TL_Press PlayFromStart)
      (:Update
        (Transformation|SetRelativeLocation _button (Math|Vector|MakeVector (.x _relativelocation) (* _press -1.0) (.z _relativelocation)) false false))
      (:Finished
        (CallFunction|PowerActors "NewEnumerator2")))))

(event MouseInput|EventActorEndCursorOver
  (Rendering|Material|SetScalarParameterValueonMaterials (Variables|Default|GetButton) "Highlight" 0.0))

(fn ConstructionScript)