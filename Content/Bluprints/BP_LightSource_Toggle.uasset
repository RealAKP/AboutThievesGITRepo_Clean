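; Interactable lamp that toggles a flickering point light between Pre Interact (off) and Post Interact (on) states, with a cursor-hover material highlight.
; Activation plays a power sound and applies the desired state, while instant updates switch silently and the construction script applies a preview state.
; A Flickering timeline drives intensity between min and max, optionally also shifting the light's position.
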(event Custom|EventFlickeringSTOP
  (bind _pointlight (Variables|Default|GetPointLight))
  (Rendering|SetVisibility (Variables|Default|GetPointLight) false false)
  (bind _intensity (Timeline|Flickering Stop)
    (:Update
      (Rendering|Components|Light|SetIntensity _pointlight (Math|Float|Lerp (Variables|Default|GetMinINT) (Variables|Default|GetMaxINT) _intensity))
      (if (Variables|Default|GetbModifyFlickerLocation)
        (Transformation|SetRelativeLocation _pointlight (Math|Conversions|ToVector(Float) (* _intensity (Variables|Default|GetFlickerLocationModifier))) false false)
        (Transformation|AddRelativeLocation _pointlight (Variables|Default|GetFlickerDeltaLocation) false false)))))

(event Custom|EventFlickering
  (bind _pointlight (Variables|Default|GetPointLight))
  (Rendering|SetVisibility (Variables|Default|GetPointLight) true false)
  (bind _intensity (Timeline|Flickering Play)
    (:Update
      (Rendering|Components|Light|SetIntensity _pointlight (Math|Float|Lerp (Variables|Default|GetMinINT) (Variables|Default|GetMaxINT) _intensity))
      (if (Variables|Default|GetbModifyFlickerLocation)
        (Transformation|SetRelativeLocation _pointlight (Math|Conversions|ToVector(Float) (* _intensity (Variables|Default|GetFlickerLocationModifier))) false false)
        (Transformation|AddRelativeLocation _pointlight (Variables|Default|GetFlickerDeltaLocation) false false)))))

(event MouseInput|EventActorBeginCursorOver
  (Rendering|Material|SetScalarParameterValueonMaterials (Variables|Default|GetSM_Lamp) "Highlight" 1.0))

(event EventBeginPlay
  (|CallParentFunction)
  (CallFunction|UpdateDesiredState (Variables|Default|GetDesiredState)))

(event MouseInput|EventActorEndCursorOver
  (Rendering|Material|SetScalarParameterValueonMaterials (Variables|Default|GetSM_Lamp) "Highlight" 0.0))

(event EventActivate
  (params (bTurnOn :type Boolean) (TriggeringActor :type Actor%20Object%20Reference))
  (Audio|PlaySoundatLocation (Variables|Default|GetPowerSound) (Transformation|GetActorLocation) "0, 0, 0" 1.0 1.0 0.0 "/Game/DCT/Sound/ATT_Dungeon.ATT_Dungeon" 0 0 0)
  (bind _output_get (Variables|Default|SetInteractState (Variables|Default|GetDesiredState)))
  (switch Utilities|FlowControl|Switch|SwitchonEInteractState _output_get
    (:NewEnumerator0
      (CallFunction|EventFlickeringSTOP))
    (:NewEnumerator2
      (CallFunction|EventFlickering))))

(event EventUpdateStateInstantly
  (params (DesiredState :type EInteractState%20Enum :default "NewEnumerator0"))
  (switch Utilities|FlowControl|Switch|SwitchonEInteractState DesiredState
    (:NewEnumerator0
      (CallFunction|EventFlickeringSTOP))
    (:NewEnumerator2
      (CallFunction|EventFlickering))))

(fn ConstructionScript
  (|CallParentFunction)
  (switch Utilities|FlowControl|Switch|SwitchonEInteractState (Variables|Default|GetPreviewState)
    (:NewEnumerator0
      (CallFunction|EventFlickeringSTOP))
    (:NewEnumerator2
      (CallFunction|EventFlickering))))