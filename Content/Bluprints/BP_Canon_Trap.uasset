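; BP_Canon_Trap is a cannon trap that fires when activated.
; Its Activate event waits for a configurable delay, sets InteractState from DesiredState, then proceeds only if TurnOn is true.
; It then powers other actors with that state, spawns an actor with a preset velocity at the Arrow component's transform, and plays a cannon shot sound there.
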(event EventActivate
  (params (bTurnOn :type Boolean) (TriggeringActor :type Actor%20Object%20Reference))
  (bind _arrow (Variables|Default|GetArrow))
  (Utilities|FlowControl|Delay (Variables|Default|GetDelay))
  (bind _output_get (Variables|Default|SetInteractState (Variables|Default|GetDesiredState)))
  (if bTurnOn
    (CallFunction|PowerActors _output_get)
    (Game|SpawnActorfromClass :Class "/Game/Bluprints/Magic/Projectiles/BP_Projectile_Fireball.BP_Projectile_Fireball_C" :SpawnTransform (Transformation|GetWorldTransform _arrow) :CollisionHandlingOverride "AlwaysSpawn" :TransformScaleMethod "SelectDefaultAtRuntime" :Velocity 5e+02 :SourceActor 0 :Instigator 0)
    (Audio|PlaySoundatLocation "/Game/Audio/Items/A_CanonShot_Cue.A_CanonShot_Cue" (Transformation|GetWorldLocation _arrow) "0, 0, 0" 1.0 1.0 0.0 0 0 0 0)))

(fn ConstructionScript)