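; BP_Rope_Spline is a construction-script Blueprint that builds a rope or wire from spline mesh components along a spline.
; SplineMeshVar selects the layout: one segment per pair of spline points using their tangents, or segments at fixed Spacing along the length with direction scaled by TangentScale.
; Both variants apply WireSize as a uniform start and end cross-section scale to each segment.
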(fn ConstructionScript
  (bind _spline (Variables|Default|GetSpline))
  (bind _spline_2 (Variables|Default|GetSpline))
  (bind _wire_size (Variables|Default|GetWire%20Size))
  (bind _spacing (Variables|Default|GetSpacing))
  (bind _tangent_scale (Variables|Default|GetTangent%20Scale))
  (Variables|Default|SetConponent%201 0)
  (switch int (Variables|Default|GetSpline%20Mesh%20Var)
    (:Default
      ;[1 1 1] SplinePoints
      (for _index (range 0 (- (Spline|GetNumberOfSplinePoints (Variables|Default|GetSpline)) 2)) :!label _label
        (Variables|Default|SetPoints _index)
        ;[1 1 1] Get Position Variant 1
        (bind _returnvalue (AddComponent|AddSplineMeshComponent false))
        (Variables|Default|SetConponent%201 _returnvalue)
        (SplineMesh|SetStartandEnd (Variables|Default|GetConponent%201) (.Location (Spline|GetLocationandTangentatSplinePoint _spline (Variables|Default|GetPoints) "Local")) (.Tangent (Spline|GetLocationandTangentatSplinePoint _spline (Variables|Default|GetPoints) "Local")) (.Location (Spline|GetLocationandTangentatSplinePoint _spline (+ (Variables|Default|GetPoints) 1) "Local")) (.Tangent (Spline|GetLocationandTangentatSplinePoint _spline (+ (Variables|Default|GetPoints) 1) "Local")) true :!class /Script/Engine.SplineMeshComponent)
        ;[1 1 1] Wire Scale
        (SplineMesh|SetStartScale (Variables|Default|GetConponent%201) (Math|Vector2D|MakeVector2D _wire_size _wire_size) true :!class /Script/Engine.SplineMeshComponent)
        (SplineMesh|SetEndScale (Variables|Default|GetConponent%201) (Math|Vector2D|MakeVector2D _wire_size _wire_size) true :!class /Script/Engine.SplineMeshComponent)))
    (:0
      (goto _label))
    (:1
      ;[1 1 1] Get Position Variant 2
      (for _index_2 (range 0 (.ReturnValue (Math|Float|Division(WholeandRemainder) (Spline|GetSplineLength _spline_2) _spacing)))
        (bind _returnvalue_2 (AddComponent|AddSplineMeshComponent false))
        (Variables|Default|SetConponent%201 _returnvalue_2)
        (SplineMesh|SetStartandEnd (Variables|Default|GetConponent%201) (Spline|GetLocationatDistanceAlongSpline _spline_2 (* _index_2 _spacing) "Local") (* (Spline|GetDirectionatDistanceAlongSpline _spline_2 (* _index_2 _spacing) "Local") _tangent_scale) (Spline|GetLocationatDistanceAlongSpline _spline_2 (+ (* _index_2 _spacing) _spacing) "Local") (* (Spline|GetDirectionatDistanceAlongSpline _spline_2 (+ (* _index_2 _spacing) _spacing) "Local") _tangent_scale) true :!class /Script/Engine.SplineMeshComponent)
        (SplineMesh|SetStartScale (Variables|Default|GetConponent%201) (Math|Vector2D|MakeVector2D _wire_size _wire_size) true :!class /Script/Engine.SplineMeshComponent)
        (SplineMesh|SetEndScale (Variables|Default|GetConponent%201) (Math|Vector2D|MakeVector2D _wire_size _wire_size) true :!class /Script/Engine.SplineMeshComponent)))))