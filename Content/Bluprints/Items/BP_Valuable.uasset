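; BP_Valuable is a pickup item that grants dungeon experience when interacted with.
; Interact plays the item's use sound, rewards XP through the game state's DungeonState, spawns orange floating XP text and a Niagara effect, then destroys the actor.
; The XP amount reuses the Cooldown field of the item data, which the construction script also writes to the XPdebug text.
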(event EventInteract
  (params (TriggeringActor :type Actor%20Object%20Reference))
  (bind _itemdata (CallFunction|GetItemData))
  (Audio|PlaySoundatLocation (.usesound _itemdata) (Transformation|GetWorldLocation (Variables|Default|GetItemMesh)) "0, 0, 0" 1.5 1.0 0.0 "/Game/Audio/SA_Buttons_Levers.SA_Buttons_Levers" 0 0 0)
  (Default|RewardExperience (.DungeonState (CallFunction|GetDungeonGameState)) (.cooldown _itemdata))
  (bind _returnvalue (Game|SpawnActorfromClass "/Game/DCT/Blueprints/Core/BP_FloatingText.BP_FloatingText_C" (Math|Transform|MakeTransform (+ (Transformation|GetActorLocation) "0,0.000000,40.000000") "0, 0, 0" "1.000000,1.000000,1.000000") "AlwaysSpawn" "OverrideRootScale" 0 (Utilities|Text|ToText(String) (Utilities|String|Append (Utilities|String|ToString(Integer) (Math|Float|Truncate (.cooldown _itemdata))) " XP")) 0))
  (Default|SetColor _returnvalue "(R=1.000000,G=0.617207,B=0.158961,A=1.000000)")
  (Niagara|SpawnSystematLocation "/Game/Particles/Magic/NS_PH_Valuable.NS_PH_Valuable" (Transformation|GetActorLocation))
  (Actor|DestroyActor))

(fn ConstructionScript
  (|CallParentFunction)
  (Rendering|Components|TextRender|SetText (Variables|Default|GetXPdebug) (Utilities|Text|ToText(Float) (.cooldown (CallFunction|GetItemData)) "HalfToEven")))