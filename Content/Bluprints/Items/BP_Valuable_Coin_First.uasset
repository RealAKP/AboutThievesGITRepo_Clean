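; BP_Valuable_Coin_First is a valuable coin item that shows a party dialog line when interacted with.
; After the parent interaction, it removes existing character dialog widgets and picks a random living player character from the dungeon state.
; If one is found, a new WBP_Character_Dialog displays the item's DialogText with that character's name and dynamic-material portrait, revealed by typewriter effect.
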(event EventInteract
  (params (TriggeringActor :type Actor%20Object%20Reference))
  (|CallParentFunction TriggeringActor)
  (bind _foundwidgets (Widget|GetAllWidgetsOfClass "/Game/DCT/UserInterface/WBP_Character_Dialog.WBP_Character_Dialog_C" false))
  (Widget|RemovefromParent _foundwidgets)
  (bind _returnvalue (UserInterface|CreateWidget "/Game/DCT/UserInterface/WBP_Character_Dialog.WBP_Character_Dialog_C" 0 0))
  (Variables|/Game/DCT/UserInterface/WBP_Character_Dialog.WBP_Character_Dialog_C|SetDialog%20Text _returnvalue (Variables|Default|GetDialog%20Text))
  (bind (_bfoundlivingcharacters _livingplayercharacters) (Default|GetLivingPlayerCharacters (.DungeonState (CallFunction|GetDungeonGameState))))
  (if _bfoundlivingcharacters
    (bind _output_get (Variables|Default|SetRNG (Math|Random|RandomIntegerinRange 0 (Utilities|Array|LastIndex _livingplayercharacters))))
    (Variables|/Game/DCT/UserInterface/WBP_Character_Dialog.WBP_Character_Dialog_C|SetCharacter%20Name _returnvalue (Utilities|Text|ToText(Name) (Variables|/Game/DCT/Blueprints/Core/BP_PlayerCharacter.BP_PlayerCharacter_C|GetName (Utilities|Array|Get(acopy) _livingplayercharacters _output_get))))
    (bind _returnvalue_2 (Rendering|Material|CreateDynamicMaterialInstance (Variables|/Game/DCT/Blueprints/Core/BP_PlayerCharacter.BP_PlayerCharacter_C|GetPortrait (Utilities|Array|Get(acopy) _livingplayercharacters _output_get)) "None" "None" :!class /Script/Engine.KismetMaterialLibrary))
    (bind _output_get_2 (Variables|Default|SetPortraitMID _returnvalue_2))
    (Class|Image|SetBrush (Variables|/Game/DCT/UserInterface/WBP_Character_Dialog.WBP_Character_Dialog_C|GetPortrait _returnvalue) (Utilities|Struct|MakeSlateBrush "(SpecifiedColor=(R=1.000000,G=1.000000,B=1.000000,A=1.000000),ColorUseRule=UseColor_Specified)" "Image" "NoTile" "NoMirror" "(X=32.000000,Y=32.000000)" "(Left=0.000000,Top=0.000000,Right=0.000000,Bottom=0.000000)" _output_get_2 "(CornerRadii=(X=0.000000,Y=0.000000,Z=0.000000,W=0.000000),Color=(SpecifiedColor=(R=0.000000,G=0.000000,B=0.000000,A=0.000000),ColorUseRule=UseColor_Specified),Width=0.000000,RoundingType=HalfHeightRadius,bUseBrushTransparency=False)"))
    (Variables|/Game/DCT/UserInterface/WBP_Character_Dialog.WBP_Character_Dialog_C|SetDialog%20Portrait%20Mat _returnvalue (Variables|/Game/DCT/Blueprints/Core/BP_PlayerCharacter.BP_PlayerCharacter_C|GetPortrait (Utilities|Array|Get(acopy) _livingplayercharacters _output_get)))
    (UserInterface|Viewport|AddtoViewport _returnvalue -1)
    (Default|InitiateTypewrite _returnvalue)))

(fn ConstructionScript
  (|CallParentFunction))