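; Short-lived explosion damage trigger that applies separate damage amounts to the player party and to monsters, then destroys itself shortly after spawning.
; When the dungeon pawn overlaps its volume, every living player character from the dungeon state receives the player damage message.
; Any other overlapping actor receives the monster damage message directly.
; Its own damage and stat functions are empty stubs.
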(event OnComponentBeginOverlap(Overlap_All)
  (params (OverlappedComponent :type Primitive%20Component%20Object%20Reference) (OtherActor :type Actor%20Object%20Reference) (OtherComp :type Primitive%20Component%20Object%20Reference) (OtherBodyIndex :type Integer) (bFromSweep :type Boolean) (SweepResult :type Hit%20Result%20Structure%20%28by%20ref%29))
  (Utilities|Casting|CastToBP_DungeonPawn OtherActor
    (:then
      (bind _livingplayercharacters (Default|GetLivingPlayerCharacters (.DungeonState (CallFunction|GetDungeonGameState))))
      (for _array_element _livingplayercharacters
        (Class|BPIAttackTarget|TakeDamage(Message) _array_element (Variables|Default|GetDamage%20Player))))
    (:CastFailed
      (Class|BPIAttackTarget|TakeDamage(Message) OtherActor (Variables|Default|GetDamage%20Monsters)))))

(event EventBeginPlay
  ;[0.3532 1 0.839] Time on scene
  (Utilities|FlowControl|Delay 0.1)
  (Actor|DestroyActor))

(fn ConstructionScript)

(fn TakeDamage
  (params (Damage :type Float%20%28double-precision%29)))

(fn GetStatValue
  (params (Stat :type Gameplay%20Tag%20Structure) (bBaseStat :type Boolean))
  (return 0.0))

(fn ModifyStat
  (params (Modifier :type Float%20%28double-precision%29) (Stat :type Gameplay%20Tag%20Structure) (bChangeBaseStat :type Boolean) (Manipulation :type EManipulate%20Enum :default "NewEnumerator0") (bUpdateDerivedStats :type Boolean) (bCanBeNegative :type Boolean))
  (return false 0.0))