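; Interactable wall valve that turns its lever when activated and powers other actors once the turn finishes.
; A timeline drives lever yaw and turning-sound volume; on finish it plays an end cue, silences the turning sound, commits the desired interact state and passes it to PowerActors.
; Deactivation reverses the timeline, instant state updates set its time, and cursor hover toggles a material highlight on the lever.
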(event MouseInput|EventActorBeginCursorOver
  (Rendering|Material|SetScalarParameterValueonMaterials (Variables|Default|GetLever) "Highlight" 1.0))

(event MouseInput|EventActorEndCursorOver
  (Rendering|Material|SetScalarParameterValueonMaterials (Variables|Default|GetLever) "Highlight" 0.0))

(event EventUpdateStateInstantly
  (params (DesiredState :type EInteractState%20Enum :default "NewEnumerator0"))
  (bind (_direction _volume _rotation) (Timeline|Timeline SetNewTime)
    (:Update
      (Transformation|SetRelativeRotation (Variables|Default|GetLever) (Math|Rotator|MakeRotator 0.0 0.0 (* _rotation 1e+02)) false false)
      (Audio|Components|Audio|SetVolumeMultiplier (stale EventActivate _returnvalue) _volume :!class /Script/Engine.AudioComponent))
    (:Finished
      (Audio|PlaySoundatLocation "/Game/Audio/Items/S_Valve_End_Cue.S_Valve_End_Cue" (Transformation|GetActorLocation) "0, 0, 0" 1.0 1.0 0.0 "/Game/DCT/Sound/ATT_Dungeon.ATT_Dungeon" 0 0 0)
      (Audio|Components|Audio|SetVolumeMultiplier (stale EventActivate _returnvalue) 0.0 :!class /Script/Engine.AudioComponent)
      (bind _output_get (Variables|Default|SetInteractState (Variables|Default|GetDesiredState)))
      (CallFunction|PowerActors _output_get))))

(event EventActivate
  (params (bTurnOn :type Boolean) (TriggeringActor :type Actor%20Object%20Reference))
  (if bTurnOn
    (bind _returnvalue (Audio|SpawnSoundatLocation (Variables|Default|GetSound) (Transformation|GetActorLocation) "0, 0, 0" 0.0 1.0 0.0 0 0))
    (bind (_direction _volume _rotation) (Timeline|Timeline Play)
      (:Update
        (Transformation|SetRelativeRotation (Variables|Default|GetLever) (Math|Rotator|MakeRotator 0.0 0.0 (* _rotation 1e+02)) false false)
        (Audio|Components|Audio|SetVolumeMultiplier _returnvalue _volume :!class /Script/Engine.AudioComponent))
      (:Finished
        (Audio|PlaySoundatLocation "/Game/Audio/Items/S_Valve_End_Cue.S_Valve_End_Cue" (Transformation|GetActorLocation) "0, 0, 0" 1.0 1.0 0.0 "/Game/DCT/Sound/ATT_Dungeon.ATT_Dungeon" 0 0 0)
        (Audio|Components|Audio|SetVolumeMultiplier _returnvalue 0.0 :!class /Script/Engine.AudioComponent)
        (bind _output_get (Variables|Default|SetInteractState (Variables|Default|GetDesiredState)))
        (CallFunction|PowerActors _output_get)))
    (else
      (Timeline|Timeline Reverse))))

(fn ConstructionScript)