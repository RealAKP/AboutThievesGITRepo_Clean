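; BP_Trigger_Damage_Continuos is a trigger that deals repeated damage to the dungeon party or monsters while they overlap it.
; A BP_DungeonPawn overlap damages every living player character from the DungeonState, while a BP_Monster takes damage itself.
; Both branches send TakeDamageMessage, then loop through a one-second Delay while the shared IsInRadius flag is set.
; End overlap of either type clears that flag.
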(event Collision|EventActorBeginOverlap
  (params (OtherActor :type Actor%20Object%20Reference))
  (Utilities|FlowControl|Sequence
    (:then_0
      (Utilities|Casting|CastToBP_DungeonPawn OtherActor)
      (Variables|Default|SetIs%20In%20Radius true)
      (bind _livingplayercharacters (Default|GetLivingPlayerCharacters (.DungeonState (CallFunction|GetDungeonGameState)) :!label _label))
      (for _array_element _livingplayercharacters
        (Class|BPIAttackTarget|TakeDamage(Message) _array_element (Variables|Default|GetDamage))
        (Utilities|FlowControl|Delay 1.0)
        (if (Variables|Default|GetIs%20In%20Radius)
          (goto _label))))
    (:then_1
      (bind _asbp_monster (Utilities|Casting|CastToBP_Monster OtherActor))
      (Variables|Default|SetIs%20In%20Radius true)
      (Class|BPIAttackTarget|TakeDamage(Message) _asbp_monster (Variables|Default|GetDamage) :!label _label_2)
      (Utilities|FlowControl|Delay 1.0)
      (if (Variables|Default|GetIs%20In%20Radius)
        (goto _label_2)))))

(event Collision|EventActorEndOverlap
  (params (OtherActor :type Actor%20Object%20Reference))
  (Utilities|FlowControl|Sequence
    (:then_0
      (Utilities|Casting|CastToBP_DungeonPawn OtherActor)
      (Variables|Default|SetIs%20In%20Radius false))
    (:then_1
      (Utilities|Casting|CastToBP_Monster OtherActor)
      (Variables|Default|SetIs%20In%20Radius false))))

(fn ConstructionScript)

(fn TakeDamage
  (params (Damage :type Float%20%28double-precision%29)))

(fn GetStatValue
  (params (Stat :type Gameplay%20Tag%20Structure) (bBaseStat :type Boolean))
  (return 0.0))

(fn ModifyStat
  (params (Modifier :type Float%20%28double-precision%29) (Stat :type Gameplay%20Tag%20Structure) (bChangeBaseStat :type Boolean) (Manipulation :type EManipulate%20Enum :default "NewEnumerator0") (bUpdateDerivedStats :type Boolean) (bCanBeNegative :type Boolean))
  (return false 0.0))