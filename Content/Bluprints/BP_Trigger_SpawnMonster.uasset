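; BP_Trigger_SpawnMonster is a one-shot trigger actor that spawns a BP_Monster on its first overlap.
; The monster spawns at a configured Location, with its type taken from the MonsterName row in DT_Monsters.
; After a short delay it destroys itself, first making every BP_Monster search for the player if Alarm is set.
; The construction script places a billboard above the spawn point, and CheckForWizardsAndRogues always returns false.
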(event Collision|EventActorBeginOverlap
  (params (OtherActor :type Actor%20Object%20Reference))
  (|CallParentFunction OtherActor)
  (Utilities|FlowControl|DoOnce false
    (:Completed
      (bind _returnvalue (Game|SpawnActorfromClass "/Game/DCT/Blueprints/Monsters/BP_Monster.BP_Monster_C" (Math|Transform|MakeTransform (Variables|Default|GetLocation)) "Undefined" "OverrideRootScale" 0 (Utilities|Struct|MakeDataTableRowHandle "/Game/DCT/Data/DT_Monsters.DT_Monsters" (Variables|Default|GetMonsterName)) 0 0))
      (Development|PrintString (Utilities|String|Append "Spawned" (Utilities|GetDisplayName _returnvalue)))
      (Utilities|FlowControl|Delay 0.2)
      (if (Variables|Default|GetAlarm!)
        (bind _outactors (Actor|GetAllActorsOfClass "/Game/DCT/Blueprints/Monsters/BP_Monster.BP_Monster_C"))
        (Default|SearchforPlayer _outactors)
        (Actor|DestroyActor)
        (else
          (Actor|DestroyActor))))))

(event EventCallonPlayerStepEnd
  (params (DungeonPawn :type BP%20Dungeon%20Pawn%20Object%20Reference))
  (|CallParentFunction DungeonPawn))

(event EventSaveActor
  (params (DungeonInstance :type BP%20GI%20Dungeon%20Object%20Reference))
  (|CallParentFunction DungeonInstance))

(event EventBeginPlay
  (|CallParentFunction))

(fn ConstructionScript
  (bind _location (Variables|Default|GetLocation))
  (bind (_x _y _z) (Math|Vector|BreakVector _location))
  (|CallParentFunction)
  (Transformation|SetWorldLocation (Variables|Default|GetBillboard_Spawn) (Math|Vector|MakeVector _x _y (+ _z 45.0)) false false))

(fn CheckforWizardsandRogues
  (return false))