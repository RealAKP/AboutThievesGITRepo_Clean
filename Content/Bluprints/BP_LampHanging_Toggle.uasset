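; BP_LampHanging_Toggle is a hanging lamp that extends a parent power and flicker Blueprint.
; Power calls SwingLamp, then the parent handler.
; Flicker start and stop show and hide the point light glow and flame mesh before calling their parent events.
; SwingLamp is empty; the timeline that would rock the lamp mesh on roll is disconnected, so the lamp never swings.
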(event Custom|EventFlickeringSTOP
  (Rendering|SetVisibility (Variables|Default|GetSM_FLAME_NEW) false false)
  (|CallParentFunction))

(event Custom|EventFlickering
  (Rendering|SetVisibility (Variables|Default|GetPointLight_Glow) true false)
  (|CallParentFunction))

(event Custom|SwingLamp)

(event EventPower
  (params (TriggeringActor :type Actor%20Object%20Reference) (DesiredState :type EInteractState%20Enum :default "NewEnumerator0"))
  (CallFunction|SwingLamp)
  (|CallParentFunction TriggeringActor DesiredState))

(fn ConstructionScript
  (|CallParentFunction))