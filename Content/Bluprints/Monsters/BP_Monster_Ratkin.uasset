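; Ratkin monster Blueprint that extends its parent's death handling in KillMonster.
; The weapon drops as a physics object and is destroyed after a delay; an unconnected branch would spawn a kitchen knife item.
; The body ragdolls after a random delay and is soon put to sleep.
; Meanwhile it disables capsule collision, leaves the monster grid, spawns a ghost effect and starts a destroy-when-unrendered loop.
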(event EventKillMonster
  (bind _weapon (Variables|Default|GetWeapon))
  (|CallParentFunction)
  (Utilities|FlowControl|Sequence
    (:then_0
      ;[0.03151 0.07973 0.3542] Weapon
      (Collision|SetCollisionProfileName _weapon "PhysicsActor" true :!class /Script/Engine.PrimitiveComponent)
      (Physics|SetSimulatePhysics _weapon true)
      (Utilities|FlowControl|Delay 1e+01)
      (Components|DestroyComponent _weapon))
    (:then_1
      (Collision|SetCollisionProfileName (Variables|Default|GetSkeletalMesh) "DeadBody" false :!class /Script/Engine.PrimitiveComponent)
      (Utilities|FlowControl|Delay (Math|Random|RandomFloatinRange 0.5 1.5))
      (Class|SkeletalMeshComponent|SetAllBodiesSimulatePhysics (Variables|Default|GetSkeletalMesh) true)
      (Utilities|FlowControl|Sequence
        (:then_0
          (Utilities|FlowControl|Delay 1.0)
          (Class|PrimitiveComponent|PutRigidBodytoSleep (Variables|Default|GetSkeletalMesh) "None"))
        (:then_1
          (Collision|SetCollisionEnabled (Variables|Default|GetCapsule) "NoCollision")
          (CallFunction|RemoveMonsterfromGrid)
          (Utilities|FlowControl|Delay 1.0)
          (Niagara|SpawnSystematLocation "/Game/Particles/Magic/NS_Ghost.NS_Ghost" (Transformation|GetActorLocation))
          (CallFunction|StartDestroyifUnrenderedLoop))))))

(fn ConstructionScript
  (|CallParentFunction))