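; Ghost ratkin monster, a child Blueprint that customizes what happens when the monster is killed.
; KillMonster runs the parent logic, switches the mesh to the DeadBody collision profile, disables capsule collision and removes the monster from the grid.
; After a short delay it spawns the NS_Ghost Niagara effect at the actor's location, then starts the inherited loop that destroys it if unrendered.
; An unconnected frost bolt hit effect spawn never runs.
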(event EventKillMonster
  (|CallParentFunction)
  (Collision|SetCollisionProfileName (Variables|Default|GetSkeletalMesh) "DeadBody" false :!class /Script/Engine.PrimitiveComponent)
  (Collision|SetCollisionEnabled (Variables|Default|GetCapsule) "NoCollision")
  (CallFunction|RemoveMonsterfromGrid)
  (Utilities|FlowControl|Delay 1.0)
  (Niagara|SpawnSystematLocation "/Game/Particles/Magic/NS_Ghost.NS_Ghost" (Transformation|GetActorLocation))
  (CallFunction|StartDestroyifUnrenderedLoop))

(fn ConstructionScript
  (|CallParentFunction))