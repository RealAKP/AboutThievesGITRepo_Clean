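; Red slime monster, a child Blueprint that customizes the death sequence to end in a damaging explosion.
; On KillMonster it calls the parent, then a timeline inflates the skeletal mesh while driving emissive power on a dynamic material.
; When the timeline finishes, it spawns a burst effect, three low-tier valuable loot drops, an explosion sound and a damage trigger, then destroys itself.
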(event EventBeginPlay
  (|CallParentFunction))

(event EventKillMonster
  (bind _returnvalue (Math|Random|RandomRotator false))
  (bind _returnvalue_2 (Transformation|GetActorLocation))
  (bind _returnvalue_3 (+ _returnvalue_2 "0,0,100.000000"))
  (bind _returnvalue_4 (Math|Transform|MakeTransform _returnvalue_3 _returnvalue))
  (|CallParentFunction)
  (bind _returnvalue_5 (Rendering|Material|CreateDynamicMaterialInstance (Variables|Default|GetSkeletalMesh) 0 "/Game/Materials/Monsters/MI_Monster_Slime_Red.MI_Monster_Slime_Red" "None" :!class /Script/Engine.PrimitiveComponent))
  (bind (_direction _newtrack_0 _newtrack_1) (Timeline|Inflate Play)
    (:Update
      (Transformation|SetRelativeScale3D (Variables|Default|GetSkeletalMesh) (Math|Conversions|ToVector(Float) _newtrack_0))
      (Rendering|Material|SetScalarParameterValue _returnvalue_5 "Emissive Power" _newtrack_1 :!class /Script/Engine.MaterialInstanceDynamic))
    (:Finished
      (Niagara|SpawnSystematLocation "/Game/Particles/Magic/NS_SlimeBurst_Die_RED.NS_SlimeBurst_Die_RED" _returnvalue_2)
      (Game|SpawnActorfromClass "/Game/Bluprints/Items/BP_Random_Loot_Valuables_Low.BP_Random_Loot_Valuables_Low_C" _returnvalue_4 "AlwaysSpawn" "OverrideRootScale" 0 0)
      (Game|SpawnActorfromClass "/Game/Bluprints/Items/BP_Random_Loot_Valuables_Low.BP_Random_Loot_Valuables_Low_C" _returnvalue_4 "AlwaysSpawn" "OverrideRootScale" 0 0)
      (Game|SpawnActorfromClass "/Game/Bluprints/Items/BP_Random_Loot_Valuables_Low.BP_Random_Loot_Valuables_Low_C" _returnvalue_4 "AlwaysSpawn" "OverrideRootScale" 0 0)
      (Audio|PlaySoundatLocation "/Game/Audio/Chaos/A_Explosion_Cue.A_Explosion_Cue" _returnvalue_2 "0, 0, 0" 1.0 1.0 0.0 0 0 0 0)
      (Game|SpawnActorfromClass "/Game/Bluprints/Magic/BP_Trigger_Damage_Explosion.BP_Trigger_Damage_Explosion_C" (Transformation|GetActorTransform) "AlwaysSpawn" "OverrideRootScale" 0 0)
      (Actor|DestroyActor))))

(fn ConstructionScript
  (|CallParentFunction))