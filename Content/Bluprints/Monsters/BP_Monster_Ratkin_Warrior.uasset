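; Ratkin Warrior monster that adds breakable armor and a physical death sequence to its parent's behavior.
; Hits play a metal sound until health falls to half, when a one-time break modifies the Armor stat and swaps the cuirass for physics fragments that dissolve through dynamic materials.
; Death drops the weapon as a temporary physics prop, ragdolls the body, removes it from the grid, starts an unrendered-cleanup loop and spawns a ghost effect.
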(event EventTakeDamage
  (params (Damage :type Float%20%28double-precision%29))
  (bind _sm_iron_cuirass_broken (Variables|Default|GetSM_Iron_Cuirass_Broken))
  (bind _capsule (Variables|Default|GetCapsule))
  (bind _returnvalue (Transformation|GetWorldLocation _capsule))
  ;[1 0.3292 0.07708] Armor Desintegrate
  (|CallParentFunction Damage)
  (if (> (.Value (CallFunction|GetMonsterStatValue "(TagName=\"Stat.Health\")")) (/ (CallFunction|GetHealthValue (.BaseStats (CallFunction|GetMonsterBaseStats))) 2.0))
    (Audio|PlaySoundatLocation "/Game/Audio/Chaos/A_Metal_Hit_Cue.A_Metal_Hit_Cue" (Transformation|GetActorLocation) "0, 0, 0" 1.0 1.0 0.0 0 0 0 0)
    (else
      (Utilities|FlowControl|DoOnce false
        (:Completed
          (CallFunction|ModifyMonsterStat "(TagName=\"Stat.Armor\")" 0.0 "NewEnumerator1")
          (Audio|PlaySoundatLocation "/Game/Audio/Chaos/A_Armor_Destroy_Cue.A_Armor_Destroy_Cue" _returnvalue "0, 0, 0" 1.0 1.0 0.0 0 0 0 0)
          (Niagara|SpawnSystematLocation "/Game/Particles/Debris/NS_Destroy_Armor.NS_Destroy_Armor" _returnvalue)
          (Components|DestroyComponent (Variables|Default|GetArmor))
          (Rendering|SetVisibility _sm_iron_cuirass_broken true false)
          (Physics|SetSimulatePhysics _sm_iron_cuirass_broken true)
          (Utilities|FlowControl|Delay 3.0)
          (Physics|SetSimulatePhysics (Variables|Default|GetSM_Iron_Cuirass_Broken) false)
          (bind _returnvalue_2 (Rendering|Material|CreateDynamicMaterialInstance (Variables|Default|GetSM_Iron_Cuirass_Broken) 0 "/Game/Materials/Items/Armour/MI_Amour_Steel_Dissolve.MI_Amour_Steel_Dissolve" "None" :!class /Script/Engine.PrimitiveComponent))
          (bind _returnvalue_3 (Rendering|Material|CreateDynamicMaterialInstance (Variables|Default|GetSM_Iron_Cuirass_Broken1) 0 "/Game/Materials/Items/Armour/MI_Amour_Steel_Dissolve.MI_Amour_Steel_Dissolve" "None" :!class /Script/Engine.PrimitiveComponent))
          (bind _returnvalue_4 (Rendering|Material|CreateDynamicMaterialInstance (Variables|Default|GetSM_Iron_Cuirass_Broken_Part02) 0 "/Game/Materials/Items/Armour/MI_Amour_Steel_Dissolve.MI_Amour_Steel_Dissolve" "None" :!class /Script/Engine.PrimitiveComponent))
          (bind _returnvalue_5 (Rendering|Material|CreateDynamicMaterialInstance (Variables|Default|GetSM_Iron_Cuirass_Broken_Part01) 0 "/Game/Materials/Items/Armour/MI_Amour_Steel_Dissolve.MI_Amour_Steel_Dissolve" "None" :!class /Script/Engine.PrimitiveComponent))
          (bind _dissolveprogress (Timeline|Dissolve Play)
            (:Update
              (Rendering|Material|SetScalarParameterValue _returnvalue_2 "Dissolve" _dissolveprogress :!class /Script/Engine.MaterialInstanceDynamic))
            (:Finished
              (Components|DestroyComponent (Variables|Default|GetSM_Iron_Cuirass_Broken)))))))))

(event EventKillMonster
  (bind _weapon (Variables|Default|GetWeapon))
  (|CallParentFunction)
  (Utilities|FlowControl|Sequence
    (:then_0
      ;[0.03151 0.07973 0.3542] Weapon
      (Collision|SetCollisionProfileName _weapon "PhysicsActor" true :!class /Script/Engine.PrimitiveComponent)
      (Physics|SetSimulatePhysics _weapon true)
      (Utilities|FlowControl|Delay 1e+01)
      (Components|DestroyComponent _weapon))
    (:then_1
      (Collision|SetCollisionProfileName (Variables|Default|GetSkeletalMesh) "DeadBody" true :!class /Script/Engine.PrimitiveComponent)
      (Utilities|FlowControl|Delay (Math|Random|RandomFloatinRange 0.5 1.5))
      (Class|SkeletalMeshComponent|SetAllBodiesSimulatePhysics (Variables|Default|GetSkeletalMesh) true)
      (Utilities|FlowControl|Sequence
        (:then_0
          (Utilities|FlowControl|Delay 1.0)
          (Class|PrimitiveComponent|PutRigidBodytoSleep (Variables|Default|GetSkeletalMesh) "None"))
        (:then_1
          (CallFunction|StartDestroyifUnrenderedLoop)
          (Collision|SetCollisionEnabled (Variables|Default|GetCapsule) "NoCollision")
          (CallFunction|RemoveMonsterfromGrid)
          (Utilities|FlowControl|Delay 1.0)
          (Niagara|SpawnSystematLocation "/Game/Particles/Magic/NS_Ghost.NS_Ghost" (Transformation|GetActorLocation)))))))

(fn ConstructionScript
  (|CallParentFunction))