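; Ratkin boss monster for the grid-based dungeon, extending a parent monster with slime bursts and a smash attack.
; BeginPlay runs an endless randomly timed loop that spawns burst effects, sound and a damage trigger at the boss.
; Attacks spawn a smash trigger on an adjacent tile, strike the player if standing there, then resume movement unless rotating.
; Death disables collision, clears the grid, bursts slime and starts destroy-if-unrendered cleanup.
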(event EventAttemptAttack
  ;[0 0 0] Attempt attack
  (Utilities|FlowControl|Sequence
    (:then_0
      (bind _returnvalue (Actor|GetActorOfClass "/Game/DCT/Blueprints/Core/BP_DungeonManager.BP_DungeonManager_C"))
      (bind (_bfoundvalidtile _btileisunoccupied _adjacenttilelocation _adjacentgridindex) (Default|GetAdjacentTilefromLocation _returnvalue self "NewEnumerator0"))
      (bind _returnvalue_2 (Game|SpawnActorfromClass "/Game/Bluprints/Magic/BP_Trigger_Damage_BossSmash.BP_Trigger_Damage_BossSmash_C" (Math|Conversions|ToTransform(Vector) _adjacenttilelocation) "AlwaysSpawn" "MultiplyWithRoot" 0 0))
      (Actor|SetOwner _returnvalue_2 self)
      (bind _asbp_dungeon_pawn (Utilities|Casting|CastToBP_DungeonPawn (Game|Player|GetPlayerPawn 0)))
      (if (== (Variables|/Game/DCT/Blueprints/Core/BP_DungeonPawn.BP_DungeonPawn_C|GetGridIndex _asbp_dungeon_pawn) _adjacentgridindex)
        (CallFunction|StrikePlayer)))
    (:then_1
      (Utilities|FlowControl|Delay 1.0)
      (if (not (Variables|Default|GetbRotating))
        (CallFunction|UpdateMove true)))))

(event EventBeginPlay
  (bind _capsule (Variables|Default|GetCapsule))
  (bind _returnvalue (Transformation|GetWorldLocation _capsule))
  (|CallParentFunction)
  (Utilities|FlowControl|Delay (Math|Random|RandomFloatinRange 3.0 1e+01) :!label _label)
  (Niagara|SpawnSystematLocation "/Game/Particles/Magic/NS_SlimeBurst_RatkinBoss.NS_SlimeBurst_RatkinBoss" _returnvalue)
  (Game|SpawnActorfromClass "/Game/Bluprints/Magic/BP_Trigger_Damage_SlimeBurst.BP_Trigger_Damage_SlimeBurst_C" (Math|Conversions|ToTransform(Vector) _returnvalue) "AlwaysSpawn" "MultiplyWithRoot" 0 0)
  (Audio|SpawnSoundatLocation "/Game/Audio/Monsters/RatkinBoss/A_RatkinBoss_SlimeBurst.A_RatkinBoss_SlimeBurst" _returnvalue "0, 0, 0" 1.0 1.0 0.0 0 0)
  (goto _label))

(event EventKillMonster
  (|CallParentFunction)
  (Collision|SetCollisionProfileName (Variables|Default|GetSkeletalMesh) "DeadBody" false :!class /Script/Engine.PrimitiveComponent)
  (Collision|SetCollisionEnabled (Variables|Default|GetCapsule) "NoCollision")
  (CallFunction|RemoveMonsterfromGrid)
  (Utilities|FlowControl|Delay 1.0)
  (Niagara|SpawnSystematLocation "/Game/Particles/Magic/NS_SlimeBurst_Die.NS_SlimeBurst_Die" (Transformation|GetWorldLocation (Variables|Default|GetCapsule)))
  (CallFunction|StartDestroyifUnrenderedLoop))

(fn ConstructionScript
  (|CallParentFunction))