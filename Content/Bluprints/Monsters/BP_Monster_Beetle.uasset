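; Beetle monster Blueprint that extends a parent monster class with its own death effect.
; On KillMonster it runs the parent logic, spawns a Niagara slime burst and a slime decal at its location, then destroys the actor immediately.
; BeginPlay and construction only call the parent.
; Disconnected leftover nodes hold an unused ragdoll-then-sleep death with grid removal and deferred destruction when unrendered.
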(event EventBeginPlay
  (|CallParentFunction))

(event EventKillMonster
  (bind _returnvalue (Transformation|GetActorLocation))
  (|CallParentFunction)
  (Niagara|SpawnSystematLocation "/Game/Particles/Magic/NS_SlimeBurst_Die.NS_SlimeBurst_Die" _returnvalue)
  (Rendering|Decal|SpawnDecalatLocation "/Game/Materials/Decals/MI_Slime_Decal.MI_Slime_Decal" "4.000000,128.000000,128.000000" _returnvalue "-90.000000,0.000000,0.000000" 0.0)
  (Actor|DestroyActor))

(fn ConstructionScript
  (|CallParentFunction))