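; Plant monster Blueprint that turns toward the player and attacks on sight, extending a parent monster class.
; Its move step, when the anim instance is not busy, rotates to the player pawn and checks visibility, then sends a delay-gated attack message or schedules a retry.
; Death runs the parent logic, switches the mesh to a dead-body collision profile, briefly enables physics simulation, then puts the body to sleep.
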(event EventMovePath
  (params (Path :type Array%20of%20Vectors))
  ;[0 0 0] Decide move, turn or attack
  (bind _isbusy (Class|BPIAnimation|IsBusy(Message) (Components|SkeletalMesh|GetAnimInstance (Variables|Default|GetSkeletalMesh))))
  (if (not _isbusy)
    (CallFunction|RotateMonsterTowardsLocation (Transformation|GetActorLocation (Game|Player|GetPlayerPawn 0)))
    (bind _bactorfound (CallFunction|LookforActor (Game|Player|GetPlayerPawn 0) false "TraceTypeQuery2"))
    (if _bactorfound
      (Utilities|DelayGate (Variables|Default|GetAttackDelay)
        (:Open
          (Class|BPIAnimation|AttackPlayer(Message) (Components|SkeletalMesh|GetAnimInstance (Variables|Default|GetSkeletalMesh)))))
      (else
        (CallFunction|DelayandRetryMoveUpdate)))))

(event EventKillMonster
  (|CallParentFunction)
  (Collision|SetCollisionProfileName (Variables|Default|GetSkeletalMesh) "DeadBody" true :!class /Script/Engine.PrimitiveComponent)
  (Utilities|FlowControl|Delay 0.1)
  (Class|SkeletalMeshComponent|SetAllBodiesSimulatePhysics (Variables|Default|GetSkeletalMesh) true)
  (Utilities|FlowControl|Delay 0.1)
  (Class|PrimitiveComponent|PutRigidBodytoSleep (Variables|Default|GetSkeletalMesh) "None"))

(fn ConstructionScript
  (|CallParentFunction))