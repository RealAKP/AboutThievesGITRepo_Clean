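; Worm monster Blueprint that handles the worm's death, bursting into a sliced corpse and food drops.
; On KillMonster it runs the parent logic, then swaps the main mesh for a sliced skeletal mesh.
; Next-tick delays stagger enabling physics on that mesh and launching it with a mostly upward impulse.
; Arrow components mark where the death Niagara effect and three BP_Food_WormRound item pickups spawn.
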(event EventKillMonster
  (bind _skm_worm_sliced_01 (Variables|Default|GetSKM_Worm_Sliced_01))
  (bind _arrow3 (Variables|Default|GetArrow3))
  (bind _arrow1 (Variables|Default|GetArrow1))
  (bind _arrow2 (Variables|Default|GetArrow2))
  (|CallParentFunction)
  (Rendering|SetVisibility (Variables|Default|GetSkeletalMesh) false false)
  (Rendering|SetVisibility _skm_worm_sliced_01 true false)
  (Utilities|FlowControl|DelayUntilNextTick)
  (Physics|SetSimulatePhysics _skm_worm_sliced_01 true)
  (Utilities|FlowControl|DelayUntilNextTick)
  (Physics|AddImpulse _skm_worm_sliced_01 "500.000000,500.000000,9000.000000" "None" false)
  (Utilities|FlowControl|Sequence
    (:then_0
      (Niagara|SpawnSystematLocation "/Game/Particles/Magic/NS_Worm_Hit_Death.NS_Worm_Hit_Death" (Transformation|GetWorldLocation (Variables|Default|GetArrow4))))
    (:then_1
      (Game|SpawnActorfromClass "/Game/Bluprints/Items/BP_Food_WormRound.BP_Food_WormRound_C" (Math|Transform|MakeTransform (Transformation|GetWorldLocation _arrow1) (Transformation|GetWorldRotation _arrow1) "1.000000,1.000000,1.000000") "AlwaysSpawn" "MultiplyWithRoot" self 1 (Utilities|Struct|MakeDataTableRowHandle "/Game/DCT/Data/DT_Items.DT_Items" "Food_WormRound") true 0)
      (Game|SpawnActorfromClass "/Game/Bluprints/Items/BP_Food_WormRound.BP_Food_WormRound_C" (Math|Transform|MakeTransform (Transformation|GetWorldLocation _arrow2) (Transformation|GetWorldRotation _arrow2) "1.000000,1.000000,1.000000") "AlwaysSpawn" "MultiplyWithRoot" self 1 (Utilities|Struct|MakeDataTableRowHandle "/Game/DCT/Data/DT_Items.DT_Items" "Food_WormRound") true 0)
      (Game|SpawnActorfromClass "/Game/Bluprints/Items/BP_Food_WormRound.BP_Food_WormRound_C" (Math|Transform|MakeTransform (Transformation|GetWorldLocation _arrow3) (Transformation|GetWorldRotation _arrow3) "1.000000,1.000000,1.000000") "AlwaysSpawn" "MultiplyWithRoot" self 1 (Utilities|Struct|MakeDataTableRowHandle "/Game/DCT/Data/DT_Items.DT_Items" "Food_WormRound") true 0))))

(fn ConstructionScript
  (|CallParentFunction))