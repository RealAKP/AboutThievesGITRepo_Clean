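; Slime monster (Szlamek) Blueprint that extends a parent monster class and adds its own death effects and loot drop.
; BeginPlay and construction only call the parent.
; KillMonster runs the parent logic, then spawns a slime burst Niagara effect and a slime decal at the actor's location.
; It then spawns three randomly rotated valuables loot actors at a fixed offset, staggered by short delays, before destroying itself.
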(event EventBeginPlay
  (|CallParentFunction))

(event EventKillMonster
  (bind _returnvalue (Math|Random|RandomRotator false))
  (bind _returnvalue_2 (Transformation|GetActorLocation))
  (bind _returnvalue_3 (+ _returnvalue_2 "60.000000,0.000000,140.000000"))
  (bind _returnvalue_4 (Math|Transform|MakeTransform _returnvalue_3 _returnvalue))
  (|CallParentFunction)
  (Niagara|SpawnSystematLocation "/Game/Particles/Magic/NS_SlimeBurst_Die.NS_SlimeBurst_Die" _returnvalue_2)
  (Rendering|Decal|SpawnDecalatLocation "/Game/Materials/Decals/MI_Slime_Decal.MI_Slime_Decal" "16.000000,128.000000,128.000000" _returnvalue_2 "-90.000000,0.000000,0.000000" 0.0)
  (Game|SpawnActorfromClass "/Game/Bluprints/Items/BP_Random_Loot_Valuables_Szlamek.BP_Random_Loot_Valuables_Szlamek_C" _returnvalue_4 "AdjustIfPossibleButAlwaysSpawn" "OverrideRootScale" 0 0)
  (Utilities|FlowControl|Delay 0.2)
  (Game|SpawnActorfromClass "/Game/Bluprints/Items/BP_Random_Loot_Valuables_Szlamek.BP_Random_Loot_Valuables_Szlamek_C" _returnvalue_4 "AdjustIfPossibleButAlwaysSpawn" "OverrideRootScale" 0 0)
  (Utilities|FlowControl|Delay 0.2)
  (Game|SpawnActorfromClass "/Game/Bluprints/Items/BP_Random_Loot_Valuables_Szlamek.BP_Random_Loot_Valuables_Szlamek_C" _returnvalue_4 "AdjustIfPossibleButAlwaysSpawn" "OverrideRootScale" 0 0)
  (Actor|DestroyActor))

(fn ConstructionScript
  (|CallParentFunction))