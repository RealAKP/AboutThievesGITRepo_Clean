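; Pressure plate interactable that switches state and powers other actors based on the weight resting on it.
; Overlap events sum the weights reported by overlapping actors and call Power when the total crosses WeightThreshold, unless the plate is exhausted.
; Activate runs a timeline that moves the plate vertically, plays a switch sound and passes the new InteractState to powered actors.
; Deactivation reverses the timeline only when no BP_Effect overlaps.
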(event EventUpdateStateInstantly
  (params (DesiredState :type EInteractState%20Enum :default "NewEnumerator0"))
  (bind _trigger (Timeline|TL_Open SetNewTime)
    (:Update
      (Transformation|SetRelativeLocation (Variables|Default|GetPlate) (Math|Vector|MakeVector 0.0 0.0 (* _trigger -5.0)) false false))
    (:Finished
      (Audio|PlaySoundatLocation "/Game/DCT/Sound/A_Switch_Cue.A_Switch_Cue" (Transformation|GetActorLocation) "0, 0, 0" 1.0 1.0 0.0 "/Game/DCT/Sound/ATT_Dungeon.ATT_Dungeon" 0 0 0))
    (:Pressed
      (bind _output_get (Variables|Default|SetInteractState (Variables|Default|GetDesiredState)))
      (CallFunction|PowerActors _output_get))))

(event EventActivate
  (params (bTurnOn :type Boolean) (TriggeringActor :type Actor%20Object%20Reference))
  (if bTurnOn
    (bind _trigger (Timeline|TL_Open Play)
      (:Update
        (Transformation|SetRelativeLocation (Variables|Default|GetPlate) (Math|Vector|MakeVector 0.0 0.0 (* _trigger -5.0)) false false))
      (:Finished
        (Audio|PlaySoundatLocation "/Game/DCT/Sound/A_Switch_Cue.A_Switch_Cue" (Transformation|GetActorLocation) "0, 0, 0" 1.0 1.0 0.0 "/Game/DCT/Sound/ATT_Dungeon.ATT_Dungeon" 0 0 0))
      (:Pressed
        (bind _output_get (Variables|Default|SetInteractState (Variables|Default|GetDesiredState)))
        (CallFunction|PowerActors _output_get)))
    (elif (== (Utilities|Array|Length (Collision|GetOverlappingActors "/Game/Bluprints/Effects/BP_Effect.BP_Effect_C" :!class /Script/Engine.Actor)) 0)
      (Timeline|TL_Open Reverse))))

(event Collision|EventActorBeginOverlap
  (params (OtherActor :type Actor%20Object%20Reference))
  (if (not (CallFunction|CheckifExhausted))
    (if (Utilities|Enum|Equal(Enum) (Variables|Default|GetInteractState) "NewEnumerator0")
      (bind _weight (Class|BPIWeight|GetWeight(Message) OtherActor))
      (if (> _weight 0.0)
        (if (>= (CallFunction|GetTotalWeightOfOverlappingObjects) (Variables|Default|GetWeightThreshold))
          (CallFunction|Power OtherActor "NewEnumerator2"))))))

(event Collision|EventActorEndOverlap
  (params (OtherActor :type Actor%20Object%20Reference))
  (if (not (CallFunction|CheckifExhausted))
    (if (Utilities|Enum|Equal(Enum) (Variables|Default|GetInteractState) "NewEnumerator2")
      (if (< (CallFunction|GetTotalWeightOfOverlappingObjects) (Variables|Default|GetWeightThreshold))
        (CallFunction|Power 0 "NewEnumerator0")))))

(fn ConstructionScript)

(fn GetTotalWeightOfOverlappingObjects
  (for _array_element (Collision|GetOverlappingActors 0 :!class /Script/Engine.Actor)
    (bind _weight (Class|BPIWeight|GetWeight(Message) _array_element))
    (if (> _weight 0.0)
      (LocalVariables|SetLocalWeight (+ (LocalVariables|GetLocalWeight) _weight))))
  (return (LocalVariables|GetLocalWeight)))