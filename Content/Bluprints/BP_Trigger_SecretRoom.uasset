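; BP_Trigger_SecretRoom is a one-shot trigger that announces the discovery of a secret room.
; On the first overlap by any actor, a DoOnce plays a secret sound at its location and shows the WBP_SecretRoom widget.
; After a five-second delay it removes the widget and destroys itself.
; AttemptInteract and GetAttachSlot are stubs, with interaction always returning false.
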(event Collision|EventActorBeginOverlap
  (params (OtherActor :type Actor%20Object%20Reference))
  (|CallParentFunction OtherActor)
  (Utilities|FlowControl|DoOnce false
    (:Completed
      (Audio|PlaySoundatLocation "/Game/Audio/Interface/A_Secret_Cue.A_Secret_Cue" (Transformation|GetActorLocation) "0, 0, 0" 1.0 1.0 0.0 0 0 0 0)
      (bind _returnvalue (UserInterface|CreateWidget "/Game/DCT/UserInterface/WBP_SecretRoom.WBP_SecretRoom_C"))
      (UserInterface|Viewport|AddtoViewport _returnvalue 0)
      (Utilities|FlowControl|Delay 5.0)
      (Widget|RemovefromParent _returnvalue)
      (Actor|DestroyActor))))

(fn ConstructionScript
  (|CallParentFunction))

(fn AttemptInteract
  (params (TriggeringActor :type Actor%20Object%20Reference))
  (return false))

(fn GetAttachSlot
  (return 0))