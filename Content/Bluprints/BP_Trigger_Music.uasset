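; Music trigger actor that switches the background track when the player pawn overlaps it.
; It compares its Audio variable to the sound on the MusicController's AudioComponent and only prints a debug message if they match.
; Otherwise it fades the current track out, waits for the fade, swaps the sound and fades the new one in more slowly.
; CheckForWizardsAndRogues is a stub that always returns false.
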(event Collision|EventActorBeginOverlap
  (params (OtherActor :type Actor%20Object%20Reference))
  (bind _musiccontroller (Variables|Default|GetMusicController))
  (bind _audio (Variables|Default|GetAudio))
  (bind _audiocomponent (Variables|/Game/Bluprints/BP_MusicController.BP_MusicController_C|GetAudioComponent _musiccontroller))
  (if (== OtherActor (Game|Player|GetPlayerPawn 0))
    (if (== (Variables|/Script/Engine.AudioComponent|GetSound _audiocomponent) _audio)
      (Development|PrintString "Juz gra")
      (else
        (Audio|Components|Audio|FadeOut _audiocomponent 1.0 0.0 "Linear" :!class /Script/Engine.AudioComponent)
        (Utilities|FlowControl|Delay 1.0)
        (Audio|Components|Audio|SetSound _audiocomponent _audio)
        (Audio|Components|Audio|FadeIn _audiocomponent 4.0 1.0 0.0 "Linear" :!class /Script/Engine.AudioComponent)))))

(fn ConstructionScript)

(fn CheckforWizardsandRogues
  (return false))