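; Weapon item effect that, on use, fires the item's projectile or, if none is set, performs a grid-based melee strike.
; Strike spawns particles and queries BP_DungeonManager for BPI_AttackTarget actors on an adjacent tile.
; Each target gets an accuracy-minus-dodge roll, leading to random bonus-adjusted damage with a hit sound, or floating "MISS" text.
; It also builds the item description with two-handed label, damage range and armor icons.
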(event Custom|Strike
  (bind _returnvalue (Game|Player|GetPlayerPawn 0))
  (bind _value (CallFunction|GetItemStatValue "(TagName=\"Stat.DamageBonus\")" "NewEnumerator0"))
  (bind _activatingplayercharacter (Variables|Default|GetActivatingPlayerCharacter))
  (bind _statvalue (Default|GetStatValue _activatingplayercharacter "(TagName=\"Stat.DamageBonus\")" false))
  (bind _returnvalue_2 (Transformation|GetActorTransform _returnvalue))
  (bind _returnvalue_3 (+ _value _statvalue))
  (Niagara|SpawnSystematLocation (.Particle (Utilities|Struct|BreakFItem (CallFunction|GetItemData))) (Math|Vector|MakeVector (.x (.location _returnvalue_2)) (.y (.location _returnvalue_2)) (+ (.z (.location _returnvalue_2)) 6e+01)) (.rotation _returnvalue_2))
  (bind (_bsuccess _targets) (CallFunction|FindValidTarget))
  (if _bsuccess
    (for _array_element _targets
      (bind _dodgechance (Class|BPIAttackTarget|GetDodgeChance(Message) _array_element))
      (if (< (Math|Random|RandomFloat) (- (Default|GetStatValue (Variables|Default|GetActivatingPlayerCharacter) "(TagName=\"Stat.Accuracy\")" false) _dodgechance))
        (CallFunction|Hit _array_element (Math|Conversions|ToFloat(Integer) (Math|Random|RandomIntegerinRange (Math|Float|Floor (+ (CallFunction|GetItemStatValue "(TagName=\"Stat.MinDamage\")" "NewEnumerator0") _returnvalue_3)) (Math|Float|Floor (+ (CallFunction|GetItemStatValue "(TagName=\"Stat.MaxDamage\")" "NewEnumerator0") _returnvalue_3)))))
        (else
          (CallFunction|Miss))))
    (else
      (CallFunction|Miss))))

(event Custom|Miss
  (bind _returnvalue (Game|Player|GetPlayerPawn 0))
  (bind _returnvalue_2 (Transformation|GetActorForwardVector _returnvalue))
  (bind _returnvalue_3 (Transformation|GetActorLocation _returnvalue))
  (bind _returnvalue_4 (* _returnvalue_2 1.5e+02))
  (bind _returnvalue_5 (+ _returnvalue_3 _returnvalue_4))
  (Game|SpawnActorfromClass "/Game/DCT/Blueprints/Core/BP_FloatingText.BP_FloatingText_C" (Math|Transform|MakeTransform (+ _returnvalue_5 "0, 0,100.000000") (Math|Rotator|FindLookatRotation _returnvalue_5 _returnvalue_3) "0.800000,0.800000,0.800000") "AlwaysSpawn" "OverrideRootScale" 0 "MISS" 0))

(event Custom|Hit
  (params (Target :type Actor%20Object%20Reference) (Damage :type Float%20%28double-precision%29))
  (bind _returnvalue (Game|Player|GetPlayerPawn 0))
  (Class|BPIAttackTarget|TakeDamage(Message) Target Damage)
  (Audio|PlaySoundatLocation (Utilities|Struct|BreakFItem (CallFunction|GetItemData)) (+ (+ (Transformation|GetActorLocation _returnvalue) (* (Transformation|GetActorForwardVector _returnvalue) 1.5e+02)) "0, 0,100.000000") "0, 0, 0" 2.0 1.0 0.0 "/Game/Audio/SA_Breaking_Things.SA_Breaking_Things" 0 0 0))

(event EventUseEffect
  (params (ActivatingPlayerCharacter :type BP%20Player%20Character%20Object%20Reference) (ResidingSlot :type WBP%20Slot%20Object%20Reference) (ItemType :type Data%20Table%20Row%20Handle%20Structure))
  (bind _returnvalue (Game|Player|GetPlayerPawn 0))
  (bind _returnvalue_2 (Transformation|GetActorTransform _returnvalue))
  (|CallParentFunction ActivatingPlayerCharacter ResidingSlot ItemType)
  (if (Utilities|IsValidClass (Utilities|Struct|BreakFItem (CallFunction|GetItemData)))
    (Game|SpawnActorfromClass (Utilities|Struct|BreakFItem (CallFunction|GetItemData)) (Math|Transform|MakeTransform (+ (.location _returnvalue_2) (Math|Vector|MakeVector 0.0 0.0 (Variables|Default|GetProjectileSpawnHeight))) (.rotation _returnvalue_2) (.scale _returnvalue_2)) "Undefined" "SelectDefaultAtRuntime" 0 7e+02 0.0 (Variables|Default|GetItemType) _returnvalue 0)
    (else
      (CallFunction|Strike))))

(fn ConstructionScript
  (|CallParentFunction))

(fn FindValidTarget
  (bind _localtargets (LocalVariables|GetLocalTargets))
  (bind _returnvalue (Actor|GetActorOfClass "/Game/DCT/Blueprints/Core/BP_DungeonManager.BP_DungeonManager_C"))
  (bind _adjacentgridindex (Default|GetAdjacentTilefromLocation _returnvalue (Game|Player|GetPlayerPawn 0) "NewEnumerator0"))
  (bind (_bobjectfound _objectrefs) (Default|GetAllObjectsonTile _returnvalue _adjacentgridindex))
  (if _bobjectfound
    (for _array_element _objectrefs
      (bind _asactor (Utilities|Casting|CastToActor _array_element))
      (if (Utilities|DoesObjectImplementInterface _array_element "/Game/DCT/Blueprints/Core/BPI_AttackTarget.BPI_AttackTarget_C")
        (Utilities|Array|Add (LocalVariables|GetLocalTargets) _asactor)))
    (return (> (Utilities|Array|Length _localtargets) 0) _localtargets)
    (else
      (return false 0))))

(fn GetEffectDescription
  (params (ItemType :type Data%20Table%20Row%20Handle%20Structure))
  (bind _itemdata (CallFunction|GetItemData))
  (bind (_type _effectstats) (Utilities|Struct|BreakFItem _itemdata))
  (bind _armorvalue (CallFunction|GetArmorValue _effectstats))
  (bind (_mindamage _maxdamage) (CallFunction|GetDamageRange _effectstats))
  (bind _returnvalue (Utilities|String|ToString(Integer) _maxdamage))
  (bind _statdescription (|CallParentFunction ItemType))
  (return (Utilities|String|Append (Utilities|String|SelectString "Two-handed 
" "" (Utilities|Enum|Equal(Enum) _type "NewEnumerator4")) (select (== _mindamage _maxdamage) (Utilities|String|Append "<img id=\"StatWeapon\"/> " _returnvalue) (Utilities|String|Append "<img id=\"StatWeapon\"/> " (Utilities|String|ToString(Integer) _mindamage) " - " _returnvalue)) _statdescription (Utilities|String|SelectString "" (Utilities|String|Append "<img id=\"StatArmor\"/>" (Utilities|String|ToString(Integer) _armorvalue)) (== _armorvalue 0)))))