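; Passive Toughness power effect Blueprint whose main job is supplying its tooltip text.
; GetEffectDescription prefixes the parent description with a "(Passive)" tag, then appends an inline armor stat icon and the floored Armor value from the item's equip stats.
; The construction script only calls its parent, and the file shows no logic that applies the armor itself.
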(fn ConstructionScript
  (|CallParentFunction))

(fn GetEffectDescription
  (params (ItemType :type Data%20Table%20Row%20Handle%20Structure))
  (bind _statdescription (|CallParentFunction ItemType))
  (return (Utilities|String|Append (Utilities|String|Append "(Passive)" _statdescription) " 
<img id=\"StatArmor\"/>" (Utilities|String|ToString(Integer) (Math|Float|Floor (.Value (Utilities|Map|Find (Utilities|Struct|BreakFItem (CallFunction|GetItemData)) "(TagName=\"Stat.Armor\")")))))))