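; BP_Effect implements item effects for a dungeon game, driven by the item's data table row.
; UseEffect plays the item's sound and particle at the player, and RunSlotEffect equips or unequips items in stat-conferring slots.
; ProjectileHit triggers monster strikes or rolls item damage, adding an Intelligence bonus for one item type.
; Helpers supply stats, rich-text tooltips and adjacency-checked interaction, while drop and attach-slot hooks are empty.
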(event Custom|RunDropEffect)

(event EventRunSlotEffect
  (params (bRemoved :type Boolean) (Slot :type WBP%20Slot%20Object%20Reference) (SlotOwningPlayerCharacter :type BP%20Player%20Character%20Object%20Reference) (ItemWidget :type WBP%20Item%20Object%20Reference))
  (Utilities|IsValid SlotOwningPlayerCharacter
    (:Is%20Valid
      (if (Variables|/Game/DCT/UserInterface/WBP_Slot.WBP_Slot_C|GetbConfersStats Slot)
        (Default|Equip SlotOwningPlayerCharacter (Default|GetItemName ItemWidget) bRemoved)))))

(event EventUseEffect
  (params (ActivatingPlayerCharacter :type BP%20Player%20Character%20Object%20Reference) (ResidingSlot :type WBP%20Slot%20Object%20Reference) (ItemType :type Data%20Table%20Row%20Handle%20Structure))
  (bind _itemdata (CallFunction|GetItemData))
  (bind _returnvalue (Game|Player|GetPlayerPawn 0))
  (bind _itemdata_2 (CallFunction|GetItemData))
  (bind _usesound (Utilities|Struct|BreakFItem _itemdata))
  (bind (_particle _particlespawnoffset) (Utilities|Struct|BreakFItem _itemdata_2))
  (Variables|Default|SetActivatingPlayerCharacter ActivatingPlayerCharacter)
  (Variables|Default|SetResidingSlot ResidingSlot)
  (Variables|Default|SetItemType ItemType)
  (Utilities|FlowControl|Sequence
    (:then_0
      (Utilities|IsValid _usesound
        (:Is%20Valid
          (Audio|PlaySoundatLocation _usesound (Transformation|GetActorLocation (Game|Player|GetPlayerPawn 0)) "0, 0, 0" 2.0 1.0 0.0 "/Game/Audio/SA_Magic_Missile.SA_Magic_Missile" 0 0 0))))
    (:then_1
      (Utilities|IsValid _particle
        (:Is%20Valid
          (Niagara|SpawnSystemAttached _particle (Variables|/Script/Engine.Actor|GetRootComponent _returnvalue) "None" (+ (Transformation|GetActorLocation _returnvalue) (Math|Transform|TransformDirection (Transformation|GetActorTransform _returnvalue) _particlespawnoffset)) "0, 0, 0" "KeepRelativeOffset" true))))))

(event EventProjectileHit
  (params (SourceActor :type Actor%20Object%20Reference) (HitActor :type Actor%20Object%20Reference) (HeldItem :type Data%20Table%20Row%20Handle%20Structure))
  (bind _itemdata (CallFunction|GetItemData))
  (bind _effectstats (Utilities|Struct|BreakFItem _itemdata))
  (bind (_mindamage _maxdamage) (CallFunction|GetDamageRange _effectstats))
  (bind _returnvalue (Math|Random|RandomIntegerinRange _mindamage _maxdamage))
  (bind _returnvalue_2 (Math|Conversions|ToFloat(Integer) _returnvalue))
  (bind _asbp_monster (Utilities|Casting|CastToBP_Monster SourceActor)
    (:then
      (Utilities|Casting|CastToBP_DungeonPawn HitActor)
      (Default|StrikePlayer _asbp_monster))
    (:CastFailed
      (bind _output_get (Variables|Default|SetItemType HeldItem))
      (bind _returnvalue_3 (Utilities|GetDataTableRow (.datatable _output_get) (.rowname _output_get))
        (:then
          (if (Utilities|Enum|Equal(Enum) (Utilities|Struct|BreakFItem _returnvalue_3) "NewEnumerator13")
            (Class|BPIAttackTarget|TakeDamage(Message) HitActor (+ _returnvalue_2 (Math|Float|Floor (/ (Default|GetStatValue (stale EventRunSlotEffect SlotOwningPlayerCharacter) "(TagName=\"Stat.Intelligence\")" false) 4.0))))
            (else
              (Class|BPIAttackTarget|TakeDamage(Message) HitActor _returnvalue_2))))))))

(fn ConstructionScript)

(fn GetItemData
  (bind _itemtype (Variables|Default|GetItemType))
  (bind _returnvalue (Utilities|GetDataTableRow (.datatable _itemtype) (.rowname _itemtype))
    (:then
      (return _returnvalue))
    (:RowNotFound
      (return ""))))

(fn GetItemStatValue
  (params (Stat :type Gameplay%20Tag%20Structure) (StatType :type EItemStatType%20Enum :default "NewEnumerator0"))
  (bind _itemdata (CallFunction|GetItemData))
  (return (Utilities|Select :Index StatType :NewEnumerator0 (.Value (Utilities|Map|Find (.effectstats _itemdata) Stat)) :NewEnumerator1 (.Value (Utilities|Map|Find (.equipstats _itemdata) Stat)) :NewEnumerator2 (.Value (Utilities|Map|Find (.coststats _itemdata) Stat)))))

(fn GetEffectDescription
  (params (ItemType :type Data%20Table%20Row%20Handle%20Structure))
  (bind _itemdata (CallFunction|GetItemData))
  (bind (_maxstacksize _cooldown _weight) (Utilities|Struct|BreakFItem _itemdata))
  (bind _returnvalue (> _maxstacksize 1))
  (Variables|Default|SetItemType ItemType)
  (return (Utilities|String|Append (Utilities|String|SelectString (Utilities|String|Append " 
<img id=\"StatTime\"/>" (Utilities|String|ToString(Integer) (Math|Float|Floor _cooldown)) " s") "" (> _cooldown 0.0)) (Utilities|String|SelectString (Utilities|String|Append " 
<img id=\"StatLoad\"/>" (Utilities|String|ToString(Float) _weight) " kg" (Utilities|String|SelectString " each" "" _returnvalue)) "" (> _weight 0.0)) (Utilities|String|SelectString " 
 
(Hold <img id=\"TSHIFT\"/>  for single item)" "" _returnvalue))))

(fn GetItemName
  (return (.RowName (Utilities|Struct|BreakDataTableRowHandle (Variables|Default|GetItemType)))))

(fn AttemptInteract
  (params (TriggeringActor :type Actor%20Object%20Reference))
  (bind _returnvalue (Actor|GetActorOfClass "/Game/DCT/Blueprints/Core/BP_DungeonManager.BP_DungeonManager_C"))
  (if (Default|IsAdjacent _returnvalue (Transformation|GetActorLocation TriggeringActor) (Transformation|GetActorLocation))
    (bind _asbp_pc_dungeon (Utilities|Casting|CastToBP_PC_Dungeon (Game|GetPlayerController 0))
      (:then
        (Utilities|IsValid (Variables|/Game/DCT/Blueprints/Core/BP_PC_Dungeon.BP_PC_Dungeon_C|GetMouseFollowWidget _asbp_pc_dungeon)
          (:Is%20Valid
            (return true))
          (:Is%20Not%20Valid
            (CallFunction|Interact TriggeringActor)
            (return true))))
      (:CastFailed
        _)))
  (return false))

(fn GetAttachSlot
  (return 0))

(fn GetWeight
  (return 1.0))