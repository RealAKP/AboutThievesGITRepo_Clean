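; Power effect that revives the party's player characters in the dungeon when used.
; UseEffect runs the parent logic, then calls RevivePlayerCharacter on every player character in the game state's DungeonState, with no filtering in this Blueprint.
; GetEffectDescription builds comma-separated text from the item data's EffectStats, pairing formatted values with friendly tag names, and prepends it to the parent's description.
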(event EventUseEffect
  (params (ActivatingPlayerCharacter :type BP%20Player%20Character%20Object%20Reference) (ResidingSlot :type WBP%20Slot%20Object%20Reference) (ItemType :type Data%20Table%20Row%20Handle%20Structure))
  (|CallParentFunction ActivatingPlayerCharacter ResidingSlot ItemType)
  (for _array_element (Variables|/Game/DCT/Blueprints/Core/BP_Dungeon_State.BP_Dungeon_State_C|GetPlayerCharacters (.DungeonState (CallFunction|GetDungeonGameState)))
    (Default|RevivePlayerCharacter _array_element)))

(fn ConstructionScript
  (|CallParentFunction))

(fn GetEffectDescription
  (params (ItemType :type Data%20Table%20Row%20Handle%20Structure))
  (bind _itemdata (CallFunction|GetItemData))
  (bind _effectstats (Utilities|Struct|BreakFItem _itemdata))
  (bind _statdescription (|CallParentFunction ItemType))
  (bind _keys (Utilities|Map|Keys _effectstats))
  (for (_array_element _array_index) _keys
    (bind _formattedtext (CallFunction|GetFormattedStatValueText _array_element (.Value (Utilities|Map|Find _effectstats _array_element))))
    (bind _friendlyname (CallFunction|GetTagFriendlyName _array_element))
    (LocalVariables|SetLocalDescription (Utilities|String|Append (Utilities|String|SelectString (Utilities|String|Append (LocalVariables|GetLocalDescription) ", ") (LocalVariables|GetLocalDescription) (> _array_index 0)) (Utilities|String|ToString(Text) _formattedtext) " " _friendlyname)))
  (return (Utilities|String|Append (LocalVariables|GetLocalDescription) _statdescription)))