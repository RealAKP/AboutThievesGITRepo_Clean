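; Effect Blueprint for magic scroll items that supplies their description text; its UseEffect event is empty.
; GetEffectDescription overrides the parent and looks up Mana in the item data's cost stats.
; When a mana cost exists, it wraps the parent text with the floored cost and the item weight, using rich-text image tags for stat icons.
; Otherwise it returns the parent description unchanged.
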(event EventUseEffect
  (params (ActivatingPlayerCharacter :type BP%20Player%20Character%20Object%20Reference) (ResidingSlot :type WBP%20Slot%20Object%20Reference) (ItemType :type Data%20Table%20Row%20Handle%20Structure)))

(fn ConstructionScript
  (|CallParentFunction))

(fn GetEffectDescription
  (params (ItemType :type Data%20Table%20Row%20Handle%20Structure))
  (bind _itemdata (CallFunction|GetItemData))
  (bind (_coststats _weight) (Utilities|Struct|BreakFItem _itemdata))
  (bind (_value _returnvalue) (Utilities|Map|Find _coststats "(TagName=\"Stat.Mana\")"))
  (bind _statdescription (|CallParentFunction ItemType))
  (if _returnvalue
    (return (Utilities|String|Append " 
<img id=\"StatMana\"/>" (Utilities|String|ToString(Integer) (Math|Float|Floor _value)) " mana" _statdescription "" (Utilities|String|Append " 
<img id=\"StatLoad\"/> " (Utilities|String|ToString(Float) _weight) " kg")))
    (else
      (return _statdescription))))