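; Shield of Faith power effect that temporarily applies the item's stat modifiers to every party character, described in its tooltip as armor.
; On use, a DoOnce prevents stacking while a retriggerable delay, using the item's Cooldown as duration, restarts.
; Activation attaches looping Niagara and audio to the player pawn.
; Expiry reverses the stats, destroys both components and plays end effects at the pawn once per party character.
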(event Custom|ActivateShield
  (bind _returnvalue (Game|Player|GetPlayerPawn 0))
  (bind _rootcomponent (Variables|/Script/Engine.Actor|GetRootComponent _returnvalue))
  (for _array_element (Variables|/Game/DCT/Blueprints/Core/BP_Dungeon_State.BP_Dungeon_State_C|GetPlayerCharacters (.DungeonState (CallFunction|GetDungeonGameState)))
    (Default|ModifyFullStats _array_element (Utilities|Struct|BreakFItem (CallFunction|GetItemData)) "NewEnumerator0" false true))
  (bind _returnvalue_2 (Niagara|SpawnSystemAttached "/Game/Particles/Magic/NS_PH_ShieldofFaith.NS_PH_ShieldofFaith" _rootcomponent "None" "0, 0, 0" "0, 0, 0" "KeepRelativeOffset" false))
  (Variables|Default|SetShieldEmitter _returnvalue_2)
  (bind _returnvalue_3 (Audio|SpawnSoundAttached "/Game/Audio/Magic___Spell_Sounds_PRO/Casting___Loops/cue/General_Cast_Loop_8_Cue.General_Cast_Loop_8_Cue" _rootcomponent "None" "0, 0, 0" "0, 0, 0" "KeepRelativeOffset" true 1.0 1.0 0.0 "/Game/Audio/SA_Magic_Missile.SA_Magic_Missile" 0))
  (bind _output_get (Variables|Default|SetShieldAmbient _returnvalue_3))
  (Audio|Components|Audio|FadeIn _output_get 1.0 1.0 0.0 "Linear" :!class /Script/Engine.AudioComponent))

(event Custom|DeactivateShield
  (bind _returnvalue (Game|Player|GetPlayerPawn 0))
  (bind _returnvalue_2 (Transformation|GetActorLocation _returnvalue))
  (bind (_x _y _z) (Math|Vector|BreakVector _returnvalue_2))
  (for _array_element (Variables|/Game/DCT/Blueprints/Core/BP_Dungeon_State.BP_Dungeon_State_C|GetPlayerCharacters (.DungeonState (CallFunction|GetDungeonGameState)))
    (Default|ModifyFullStats _array_element (Utilities|Struct|BreakFItem (CallFunction|GetItemData)) "NewEnumerator1" false true)
    (Niagara|SpawnSystematLocation "/Game/Particles/Magic/NS_PH_ShieldofFaith_End.NS_PH_ShieldofFaith_End" (Math|Vector|MakeVector _x _y (+ _z 5e+01)) "0, 0, 0" "1.000000,1.000000,1.000000" false)
    (Audio|PlaySoundatLocation "/Game/Audio/Magic___Spell_Sounds_PRO/Elements___School/Shadow/cue/Shadow_Spell_9_Cue.Shadow_Spell_9_Cue" _returnvalue_2 "0, 0, 0" 1.0 1.0 0.0 0 0 0 0))
  (Components|DestroyComponent (Variables|Default|GetShieldEmitter)))

(event EventUseEffect
  (params (ActivatingPlayerCharacter :type BP%20Player%20Character%20Object%20Reference) (ResidingSlot :type WBP%20Slot%20Object%20Reference) (ItemType :type Data%20Table%20Row%20Handle%20Structure))
  (|CallParentFunction ActivatingPlayerCharacter ResidingSlot ItemType)
  (Utilities|FlowControl|Sequence
    (:then_0
      (Utilities|FlowControl|DoOnce false :!label _label
        (:Completed
          (CallFunction|ActivateShield))))
    (:then_1
      (Utilities|FlowControl|RetriggerableDelay (Utilities|Struct|BreakFItem (CallFunction|GetItemData)))
      (Utilities|FlowControl|Sequence
        (:then_0
          (goto _label Reset))
        (:then_1
          (CallFunction|DeactivateShield))))))

(fn ConstructionScript
  (|CallParentFunction))

(fn GetEffectDescription
  (params (ItemType :type Data%20Table%20Row%20Handle%20Structure))
  (bind _itemdata (CallFunction|GetItemData))
  (bind _effectstats (Utilities|Struct|BreakFItem _itemdata))
  (bind _statdescription (|CallParentFunction ItemType))
  (bind _keys (Utilities|Map|Keys _effectstats))
  (for _array_element _keys
    (bind _formattedtext (CallFunction|GetFormattedStatValueText _array_element (.Value (Utilities|Map|Find _effectstats _array_element)))))
  (return (Utilities|String|Append (Utilities|String|Append (Utilities|String|ToString(Text) _formattedtext) " " "<img id=\"StatArmor\"/> " "to all characters.") _statdescription)))