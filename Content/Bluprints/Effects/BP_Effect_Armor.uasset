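; BP_Effect_Armor is an item effect Blueprint that builds the stat description text for armor items.
; GetEffectDescription reads the item data and joins armor value, dodge and weight in kg into one string, each with an inline rich-text icon tag.
; Dodge is scaled by 100 and rounded, and appears only when the result is non-zero.
; The construction script only calls its parent.
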(fn ConstructionScript
  (|CallParentFunction))

(fn GetEffectDescription
  (params (ItemType :type Data%20Table%20Row%20Handle%20Structure))
  (bind _itemdata (CallFunction|GetItemData))
  (bind (_equipstats _weight) (Utilities|Struct|BreakFItem _itemdata))
  (bind _dodgevalue (CallFunction|GetDodgeValue _equipstats))
  (bind _returnvalue (* _dodgevalue 1e+02))
  (bind _returnvalue_2 (Class|KismetMathLibrary|Round64 _returnvalue))
  (Variables|Default|SetItemType ItemType)
  (return (Utilities|String|Append (Utilities|String|Append "<img id=\"StatArmor\"/> " (Utilities|String|ToString(Integer) (CallFunction|GetArmorValue _equipstats))) "" (Utilities|String|SelectString (Utilities|String|Append " 
<img id=\"StatDodge\"/> " (Utilities|String|ToString(Integer) _returnvalue_2)) "" (!= _returnvalue_2 0)) "" (Utilities|String|Append " 
<img id=\"StatLoad\"/> " (Utilities|String|ToString(Float) _weight) " kg"))))