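; Interactable wall lever that powers other actors when switched.
; Activate plays or reverses a timeline that rolls the lever mesh; when it finishes, a handle sound plays, InteractState updates and PowerActors receives the new state.
; UpdateStateInstantly sets the timeline time directly.
; Cursor hover toggles a Highlight material parameter on the lever.
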(event MouseInput|EventActorBeginCursorOver
  (Rendering|Material|SetScalarParameterValueonMaterials (Variables|Default|GetLever) "Highlight" 1.0))

(event MouseInput|EventActorEndCursorOver
  (Rendering|Material|SetScalarParameterValueonMaterials (Variables|Default|GetLever) "Highlight" 0.0))

(event EventUpdateStateInstantly
  (params (DesiredState :type EInteractState%20Enum :default "NewEnumerator0"))
  (bind _rotate (Timeline|TL_Press SetNewTime)
    (:Update
      (Transformation|SetRelativeRotation (Variables|Default|GetLever) (Math|Rotator|MakeRotator _rotate 0.0 0.0) false false))
    (:Finished
      (Audio|PlaySoundatLocation "/Game/Audio/Items/A_lever_klamka_Cue.A_lever_klamka_Cue" (Transformation|GetActorLocation) "0, 0, 0" 1.0 1.0 0.0 "/Game/DCT/Sound/ATT_Dungeon.ATT_Dungeon" 0 0 0)
      (bind _output_get (Variables|Default|SetInteractState (Variables|Default|GetDesiredState)))
      (CallFunction|PowerActors _output_get))))

(event EventActivate
  (params (bTurnOn :type Boolean) (TriggeringActor :type Actor%20Object%20Reference))
  (if bTurnOn
    (bind _rotate (Timeline|TL_Press Play)
      (:Update
        (Transformation|SetRelativeRotation (Variables|Default|GetLever) (Math|Rotator|MakeRotator _rotate 0.0 0.0) false false))
      (:Finished
        (Audio|PlaySoundatLocation "/Game/Audio/Items/A_lever_klamka_Cue.A_lever_klamka_Cue" (Transformation|GetActorLocation) "0, 0, 0" 1.0 1.0 0.0 "/Game/DCT/Sound/ATT_Dungeon.ATT_Dungeon" 0 0 0)
        (bind _output_get (Variables|Default|SetInteractState (Variables|Default|GetDesiredState)))
        (CallFunction|PowerActors _output_get)))
    (else
      (Timeline|TL_Press Reverse))))

(fn ConstructionScript)