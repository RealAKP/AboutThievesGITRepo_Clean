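; Kill trigger that removes Szlamek monsters (regular, Red and Small) when they overlap it, with a shrink-and-fade death effect.
; On overlap it casts to each of the three classes, calls GoIdle on the match and starts that type's own timeline.
; The timeline drives actor scale and the skeletal mesh Opacity material parameter, then calls KillMonster when finished.
; Each type shares a single timeline, so a new overlap of the same type restarts it.
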(event Collision|EventActorBeginOverlap
  (params (OtherActor :type Actor%20Object%20Reference))
  (Utilities|FlowControl|Sequence
    (:then_0
      (bind _asbp_monster_szlamek (Utilities|Casting|CastToBP_Monster_Szlamek OtherActor))
      (Default|GoIdle _asbp_monster_szlamek)
      (bind (_direction _shrinkingz _shrinkingxy _matopacity) (Timeline|Szlamek PlayFromStart)
        (:Update
          (Utilities|FlowControl|Sequence
            (:then_0
              (Transformation|SetActorRelativeTransform _asbp_monster_szlamek (Math|Transform|MakeTransform (Transformation|GetActorLocation _asbp_monster_szlamek) (Transformation|GetActorRotation _asbp_monster_szlamek) (Math|Vector|MakeVector _shrinkingxy _shrinkingxy _shrinkingz)) false false))
            (:then_1
              (Rendering|Material|SetScalarParameterValueonMaterials (Variables|/Game/DCT/Blueprints/Monsters/BP_Monster.BP_Monster_C|GetSkeletalMesh _asbp_monster_szlamek) "Opacity" _matopacity))))
        (:Finished
          (Default|KillMonster _asbp_monster_szlamek))))
    (:then_1
      (bind _asbp_monster_szlamek_red (Utilities|Casting|CastToBP_Monster_Szlamek_Red OtherActor))
      (Default|GoIdle _asbp_monster_szlamek_red)
      (bind (_direction_2 _shrinkingz_2 _shrinkingxy_2 _matopacity_2) (Timeline|Timeline PlayFromStart)
        (:Update
          (Utilities|FlowControl|Sequence
            (:then_0
              (Transformation|SetActorRelativeTransform _asbp_monster_szlamek_red (Math|Transform|MakeTransform (Transformation|GetActorLocation _asbp_monster_szlamek_red) (Transformation|GetActorRotation _asbp_monster_szlamek_red) (Math|Vector|MakeVector _shrinkingxy_2 _shrinkingxy_2 _shrinkingz_2)) false false))
            (:then_1
              (Rendering|Material|SetScalarParameterValueonMaterials (Variables|/Game/DCT/Blueprints/Monsters/BP_Monster.BP_Monster_C|GetSkeletalMesh _asbp_monster_szlamek_red) "Opacity" _matopacity_2))))
        (:Finished
          (Default|KillMonster _asbp_monster_szlamek_red))))
    (:then_2
      (bind _asbp_monster_szlamek_small (Utilities|Casting|CastToBP_Monster_Szlamek_Small OtherActor))
      (Default|GoIdle _asbp_monster_szlamek_small)
      (bind (_direction_3 _shrinkingz_3 _shrinkingxy_3 _matopacity_3) (Timeline|Timeline_0 PlayFromStart)
        (:Update
          (Utilities|FlowControl|Sequence
            (:then_0
              (Transformation|SetActorRelativeTransform _asbp_monster_szlamek_small (Math|Transform|MakeTransform (Transformation|GetActorLocation _asbp_monster_szlamek_small) (Transformation|GetActorRotation _asbp_monster_szlamek_small) (Math|Vector|MakeVector _shrinkingxy_3 _shrinkingxy_3 _shrinkingz_3)) false false))
            (:then_1
              (Rendering|Material|SetScalarParameterValueonMaterials (Variables|/Game/DCT/Blueprints/Monsters/BP_Monster.BP_Monster_C|GetSkeletalMesh _asbp_monster_szlamek_small) "Opacity" _matopacity_3))))
        (:Finished
          (Default|KillMonster _asbp_monster_szlamek_small))))))

(fn ConstructionScript)