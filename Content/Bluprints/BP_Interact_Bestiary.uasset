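; BP_Interact_Bestiary is an interactable note actor that shows a bestiary entry for a monster.
; Its Power event sets DesiredState, then creates a WBP_Note_Bestiary widget, passes in the monster's name, Latin name, description and sketch, and adds it to the viewport.
; Cursor hover events toggle a Highlight scalar parameter on the SMNote materials.
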(event MouseInput|EventActorBeginCursorOver
  (Rendering|Material|SetScalarParameterValueonMaterials (Variables|Default|GetSM_Note) "Highlight" 1.0))

(event EventPower
  (params (TriggeringActor :type Actor%20Object%20Reference) (DesiredState :type EInteractState%20Enum :default "NewEnumerator0"))
  (Variables|Default|SetDesiredState "NewEnumerator2")
  (bind _returnvalue (UserInterface|CreateWidget "/Game/DCT/UserInterface/WBP_Note_Bestiary.WBP_Note_Bestiary_C" (Game|GetPlayerController 0)))
  (Variables|/Game/DCT/UserInterface/WBP_Note_Bestiary.WBP_Note_Bestiary_C|SetDescription _returnvalue (Variables|Default|GetDescription))
  (Variables|/Game/DCT/UserInterface/WBP_Note_Bestiary.WBP_Note_Bestiary_C|SetMonsterSketch _returnvalue (Variables|Default|GetMonster%20Sketch))
  (Variables|/Game/DCT/UserInterface/WBP_Note_Bestiary.WBP_Note_Bestiary_C|SetMonsterName _returnvalue (Variables|Default|GetMonster%20Name))
  (Variables|/Game/DCT/UserInterface/WBP_Note_Bestiary.WBP_Note_Bestiary_C|SetLatin%20Name _returnvalue (Variables|Default|GetLatin%20Name))
  (UserInterface|Viewport|AddtoViewport _returnvalue 0))

(event MouseInput|EventActorEndCursorOver
  (Rendering|Material|SetScalarParameterValueonMaterials (Variables|Default|GetSM_Note) "Highlight" 0.0))

(fn ConstructionScript)