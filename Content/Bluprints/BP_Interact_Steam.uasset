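; Interactable steam hazard that blocks a path with a particle effect, collision box and continuous damage trigger until its post-interact state.
; BeginPlay applies the desired state; instant state updates toggle the wall box's collision and call Activate.
; Activate's TurnOn is inverted relative to the steam: true stops it.
; The damage trigger is toggled by teleporting it vertically with relative offsets, which accumulate on repeated calls.
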(event EventActivate
  (params (bTurnOn :type Boolean) (TriggeringActor :type Actor%20Object%20Reference))
  (bind _bp_trigger_damage_continuos (Variables|Default|GetBP_Trigger_Damage_Continuos))
  (bind _p_steam_a_converted (Variables|Default|GetP_Steam_A_Converted))
  (if bTurnOn
    (Components|Activation|Deactivate _p_steam_a_converted)
    (Transformation|AddLocalOffset _bp_trigger_damage_continuos "0.000000,0.000000,-500.000000" false true)
    (else
      (Components|Activation|Activate _p_steam_a_converted false)
      (Transformation|AddLocalOffset _bp_trigger_damage_continuos "0.000000,0.000000,500.000000" false true))))

(event EventUpdateStateInstantly
  (params (DesiredState :type EInteractState%20Enum :default "NewEnumerator0"))
  (bind _wallblockingbox (Variables|Default|GetWallBlockingBox))
  (switch Utilities|FlowControl|Switch|SwitchonEInteractState DesiredState
    (:NewEnumerator0
      (Collision|SetCollisionEnabled _wallblockingbox "QueryOnly")
      (CallFunction|Activate false))
    (:NewEnumerator2
      (Collision|SetCollisionEnabled _wallblockingbox "NoCollision")
      (CallFunction|Activate true))))

(event EventBeginPlay
  (|CallParentFunction)
  (CallFunction|UpdateDesiredState (Variables|Default|GetDesiredState)))

(fn ConstructionScript
  (|CallParentFunction))

(fn GetAttachSlot
  (return 0))