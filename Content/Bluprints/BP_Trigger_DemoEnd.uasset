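; BP_Trigger_DemoEnd is a trigger actor that ends the demo when an actor overlaps it.
; After calling the parent overlap handler, a DoOnce disables player input, adds the WBP_Loading_lvl3 widget to the viewport and plays the demo-end music as 2D sound.
; The Blueprint itself does not check which actor overlaps, and its AttemptInteract always returns false.
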(event Collision|EventActorBeginOverlap
  (params (OtherActor :type Actor%20Object%20Reference))
  (|CallParentFunction OtherActor)
  (Utilities|FlowControl|DoOnce false
    (:Completed
      (Input|DisableInput (Game|Player|GetPlayerPawn 0) (Game|GetPlayerController 0))
      (bind _returnvalue (UserInterface|CreateWidget "/Game/DCT/UserInterface/WBP_Loading_lvl3.WBP_Loading_lvl3_C"))
      (UserInterface|Viewport|AddtoViewport _returnvalue 10)
      (Audio|PlaySound2D "/Game/Audio/Music/Music_DemoEnd_Cue.Music_DemoEnd_Cue" 1.0 1.0 0.0 0 0))))

(fn ConstructionScript
  (|CallParentFunction))

(fn AttemptInteract
  (params (TriggeringActor :type Actor%20Object%20Reference))
  (return false))

(fn GetAttachSlot
  (return 0))