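; Slot rule Blueprint that decides whether an item may be placed in a given slot, returning an allowed flag and a failure message.
; It rejects items without valid data or whose type is not among the slot's allowed types.
; For slots linked to another hand, it also blocks placement when that hand holds a two-handed item.
; The two-handed check examines only the item already in the other hand, not the incoming one.
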(fn CheckifCanPutinSlot
  (params (Item :type WBP%20Item%20Object%20Reference) (Slot :type WBP%20Slot%20Object%20Reference))
  (bind _otherhand (Variables|/Game/DCT/UserInterface/WBP_Slot.WBP_Slot_C|GetOtherHand Slot))
  (bind _slotteditem (Variables|/Game/DCT/UserInterface/WBP_Slot.WBP_Slot_C|GetSlottedItem _otherhand))
  (bind (_itemdata _bvalid) (CallFunction|GetItemData Item))
  (if _bvalid
    (if (Utilities|Set|Contains (Variables|/Game/DCT/UserInterface/WBP_Slot.WBP_Slot_C|GetAllowedItemTypes Slot) (.Type (Utilities|Struct|BreakFItem _itemdata)))
      (Utilities|IsValid _otherhand
        (:Is%20Valid
          (Utilities|IsValid _slotteditem
            (:Is%20Valid
              (bind _itemdata_2 (CallFunction|GetItemData _slotteditem))
              (return (Utilities|Enum|NotEqual(Enum) (.Type (Utilities|Struct|BreakFItem _itemdata_2)) "NewEnumerator4") "Two handed item equipped in other hand"))
            (:Is%20Not%20Valid
              _)))
        (:Is%20Not%20Valid
          _))
      (return true "")
      (else
        (return false "Wrong item type for slot")))
    (else
      (return false "Invalid item"))))