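; Slot rule for power items that decides whether a power can be placed in a given slot.
; It runs the parent rule first and passes on its failure message.
; For a previously slotted item, it rejects slots belonging to a different character, then blocks equipping the same power type as the one in the slot's paired OtherPower1 slot.
; Items with no last slot skip both checks.
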(fn CheckifCanPutinSlot
  (params (Item :type WBP%20Item%20Object%20Reference) (Slot :type WBP%20Slot%20Object%20Reference))
  (bind _otherpower1 (Variables|/Game/DCT/UserInterface/WBP_Slot.WBP_Slot_C|GetOtherPower1 Slot))
  (bind _slotteditem (Variables|/Game/DCT/UserInterface/WBP_Slot.WBP_Slot_C|GetSlottedItem _otherpower1))
  (bind (_ballowed _failmessage) (|CallParentFunction Item Slot))
  (if _ballowed
    (bind _lastslot (Variables|/Game/DCT/UserInterface/WBP_Item.WBP_Item_C|GetLastSlot Item)
      (:then
        (if (== (Variables|/Game/DCT/UserInterface/WBP_Slot.WBP_Slot_C|GetPlayerCharacterRef Slot) (Variables|/Game/DCT/UserInterface/WBP_Slot.WBP_Slot_C|GetPlayerCharacterRef _lastslot))
          (Utilities|FlowControl|Sequence
            (:then_0
              (Utilities|IsValid _otherpower1
                (:Is%20Valid
                  (Utilities|IsValid _slotteditem
                    (:Is%20Valid
                      (return (Utilities|Name|NotEqual(Name) (.rowname (Variables|/Game/DCT/UserInterface/WBP_Item.WBP_Item_C|GetItemType _slotteditem)) (.rowname (Variables|/Game/DCT/UserInterface/WBP_Item.WBP_Item_C|GetItemType Item))) "Cannot equip two of the same power"))
                    (:Is%20Not%20Valid
                      _)))
                (:Is%20Not%20Valid
                  _))
              (return true "")))
          (else
            (return false (Utilities|String|Append "Power belongs to " (Utilities|String|ToString(Name) (Variables|/Game/DCT/Blueprints/Core/BP_PlayerCharacter.BP_PlayerCharacter_C|GetName (Variables|/Game/DCT/UserInterface/WBP_Slot.WBP_Slot_C|GetPlayerCharacterRef _lastslot))))))))
      (:else
        (return true "")))
    (else
      (return false _failmessage))))