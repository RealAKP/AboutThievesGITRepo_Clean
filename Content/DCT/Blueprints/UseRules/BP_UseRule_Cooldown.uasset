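; BP_UseRule_Cooldown is an item use rule that gates slotted item use behind a cooldown.
; Use is allowed only while the slot's reload bar is full, otherwise it fails with a "Not yet ready" message.
; On use, it looks up the item's data table row and starts the slot cooldown when that row's value is positive, returning false only if the row is missing.
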(fn CheckifUseAllowed
  (params (Slot :type WBP%20Slot%20Object%20Reference))
  (return (>= (Variables|/Script/UMG.ProgressBar|GetPercent (Variables|/Game/DCT/UserInterface/WBP_Slot.WBP_Slot_C|GetReloadBar Slot)) 1.0) "Not yet ready"))

(fn ResolveUseConsequence
  (params (Slot :type WBP%20Slot%20Object%20Reference))
  (bind _slotteditem (Variables|/Game/DCT/UserInterface/WBP_Slot.WBP_Slot_C|GetSlottedItem Slot))
  (bind _itemtype (Variables|/Game/DCT/UserInterface/WBP_Item.WBP_Item_C|GetItemType _slotteditem))
  (bind _returnvalue (Utilities|GetDataTableRow (.datatable _itemtype) (.rowname _itemtype))
    (:then
      (if (> (Utilities|Struct|BreakFItem _returnvalue) 0.0)
        (Default|StartCooldown Slot (Utilities|Struct|BreakFItem _returnvalue))
        (return true)
        (else
          (return true))))
    (:RowNotFound
      (return false))))