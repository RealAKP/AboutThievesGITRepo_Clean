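; BP_UseRule_Ammo is an item use rule that requires and consumes ammo, such as arrows, held in the other hand.
; The check looks up the other hand's item in its data table and allows use only if its EffectBlueprint matches AmmoType, otherwise failing with "No arrows equipped".
; The consequence step reduces that item's amount by one, without repeating the validity checks.
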(fn CheckifUseAllowed
  (params (Slot :type WBP%20Slot%20Object%20Reference))
  (bind _otherhand (Variables|/Game/DCT/UserInterface/WBP_Slot.WBP_Slot_C|GetOtherHand Slot))
  (bind _slotteditem (Variables|/Game/DCT/UserInterface/WBP_Slot.WBP_Slot_C|GetSlottedItem _otherhand))
  (bind _itemtype (Variables|/Game/DCT/UserInterface/WBP_Item.WBP_Item_C|GetItemType _slotteditem))
  (Utilities|IsValid _otherhand
    (:Is%20Valid
      (Utilities|IsValid _slotteditem
        (:Is%20Valid
          (bind _returnvalue (Utilities|GetDataTableRow (.datatable _itemtype) (.rowname _itemtype))
            (:then
              (if (== (Utilities|Struct|BreakFItem _returnvalue) (Variables|Default|GetAmmoType))
                (return true "")
                (else
                  (return false "No arrows equipped"))))
            (:RowNotFound
              _)))
        (:Is%20Not%20Valid
          _)))
    (:Is%20Not%20Valid
      _))
  (return false "No arrows equipped"))

(fn ResolveUseConsequence
  (params (Slot :type WBP%20Slot%20Object%20Reference))
  (bind _otherhand (Variables|/Game/DCT/UserInterface/WBP_Slot.WBP_Slot_C|GetOtherHand Slot))
  (bind _slotteditem (Variables|/Game/DCT/UserInterface/WBP_Slot.WBP_Slot_C|GetSlottedItem _otherhand))
  (Default|UpdateAmount _slotteditem (- (Variables|/Game/DCT/UserInterface/WBP_Item.WBP_Item_C|GetAmount _slotteditem) 1))
  (return true))