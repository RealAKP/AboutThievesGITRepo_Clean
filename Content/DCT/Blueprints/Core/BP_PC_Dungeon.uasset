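; Player controller for the dungeon crawler that builds the HUD and routes party, menu and world-click input.
; SetupUi creates layout, warning, minimap and menu widgets, then, once game state is valid, per-character sheets and mini portraits with saved items.
; Tick moves the held-item widget with the mouse and rotates the compass toward a north marker.
; ScreenInteract traces under the cursor to interact or drop held items as physics actors, relocating blocked drops.
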(event Custom|SimulateClickSlot
  (params (CharacterIndex :type Integer) (SlotIndex :type Integer))
  (bind _aswbp_mini_character (Utilities|Casting|CastToWBP_MiniCharacter (Class|PanelWidget|GetChildat (Variables|/Game/DCT/UserInterface/WBP_Layout.WBP_Layout_C|GetMiniCharacterPanel (Variables|Default|GetLayoutRef)) (- CharacterIndex 1))))
  (Default|ClickSlot _aswbp_mini_character SlotIndex))

(event Custom|SetupUi
  (bind (_bvalid _dungeonstate) (CallFunction|GetDungeonGameState))
  (bind _dungeonstate_2 (CallFunction|GetDungeonGameState))
  (bind _playercharacters (Variables|/Game/DCT/Blueprints/Core/BP_Dungeon_State.BP_Dungeon_State_C|GetPlayerCharacters _dungeonstate_2))
  (bind _output (Utilities|Array|Get(acopy) _playercharacters))
  ;[0 0 0] Setup UI
  (Utilities|FlowControl|Sequence
    (:then_0
      (bind _returnvalue (UserInterface|CreateWidget "/Game/DCT/UserInterface/WBP_Layout.WBP_Layout_C" self))
      (bind _output_get (Variables|Default|SetLayoutRef _returnvalue))
      (UserInterface|Viewport|AddtoViewport _output_get 0)
      (bind _returnvalue_2 (UserInterface|CreateWidget "/Game/DCT/UserInterface/WBP_WarningDisplay.WBP_WarningDisplay_C" self))
      (bind _output_get_2 (Variables|Default|SetWarningDisplayRef _returnvalue_2))
      (UserInterface|Viewport|AddtoViewport _output_get_2 0)
      (Utilities|DelayWhile (not _bvalid)
        (:Continue
          (for (_array_element _array_index) (Variables|/Game/DCT/Blueprints/Core/BP_Dungeon_State.BP_Dungeon_State_C|GetPlayerCharacters _dungeonstate)
            (CallFunction|SetupPlayerCharacterUi _array_element _array_index))
          (Class|BPIDungeonSingletons|SetActiveWidgetCharacter(Message) _dungeonstate_2 _output "NewEnumerator0")
          (Default|ToggleSubsheets (Variables|/Game/DCT/Blueprints/Core/BP_PlayerCharacter.BP_PlayerCharacter_C|GetCharacterSheetRef _output))
          (CallFunction|LoadCharacterItems))))
    (:then_1
      ;[0.06848 0.04971 0.4793] Compas
      (bind _returnvalue_3 (UserInterface|CreateWidget "/Game/DCT/UserInterface/WBP_Minimap.WBP_Minimap_C"))
      (bind _output_get_3 (Variables|Default|SetWBP%20Minimap _returnvalue_3))
      (UserInterface|Viewport|AddtoViewport _output_get_3 -1)
      (bind _returnvalue_4 (Actor|GetActorOfClass "/Game/Bluprints/BP_NorthMarker.BP_NorthMarker_C"))
      (Variables|Default|SetNorth%20Location (Transformation|GetActorLocation _returnvalue_4)))
    (:then_2
      (bind _returnvalue_5 (UserInterface|CreateWidget "/Game/DCT/UserInterface/WBP_Menu.WBP_Menu_C"))
      (bind _output_get_4 (Variables|Default|SetWBP%20Menu _returnvalue_5))
      (UserInterface|Viewport|AddtoViewport _output_get_4 200)
      (Widget|SetVisibility _output_get_4 "Hidden"))))

(event Custom|ScreenInteract
  (bind _returnvalue (Game|Player|GetPlayerPawn 0))
  (bind _returnvalue_2 (Game|Player|GetPlayerPawn 0))
  (bind _mousefollowwidget (Variables|Default|GetMouseFollowWidget))
  (bind _returnvalue_3 (Transformation|GetActorTransform _returnvalue_2))
  (bind _returnvalue_4 (Transformation|GetActorTransform _returnvalue))
  (bind (_location _rotation) (Math|Transform|BreakTransform _returnvalue_4))
  (bind (_location_2 _rotation_2) (Math|Transform|BreakTransform _returnvalue_3))
  ;[0 0 0] Screen Interact
  (bind _output_get (Variables|Default|SetScreenInteractResult (.HitResult (Game|Player|GetHitResultUnderCursorbyChannel "TraceTypeQuery1" false))))
  ;;[0.15 0.15 0.15 0.5] Wall Click
  (if (.ReturnValue (Game|Player|GetHitResultUnderCursorbyChannel "TraceTypeQuery3" false))
    (Audio|PlaySoundatLocation "/Game/Audio/Real_Footsteps/A_Wall_Hit.A_Wall_Hit" (.Location (Collision|BreakHitResult _output_get)) "0, 0, 0" 1.0 1.0 0.0 0 0 0 0))
  (Development|PrintString (Utilities|GetDisplayName (.HitActor (Collision|BreakHitResult _output_get))) true true "(R=0.000304,G=0.658375,B=0.141263,A=1.000000)")
  (Utilities|IsValid (.HitActor (Collision|BreakHitResult _output_get))
    (:Is%20Valid
      (if (Utilities|DoesObjectImplementInterface (.HitActor (Collision|BreakHitResult _output_get)) "/Game/DCT/Blueprints/Core/BPI_Interact.BPI_Interact_C")
        (bind _bsuccess (Class|BPIInteract|AttemptInteract(Message) (.HitActor (Collision|BreakHitResult _output_get)) (Game|Player|GetPlayerPawn 0)))
        (if _bsuccess
          ;;[0 0 0.3 1 12] v.1.1
          (Utilities|IsValid (Variables|Default|GetMouseFollowWidget)
            (:Is%20Valid
              (bind _btrue (Default|IsPower (Variables|Default|GetMouseFollowWidget)))
              (if _btrue
                (CallFunction|ClearMouseFollowWidget :!label _label))))
          (else
            (Utilities|IsValid (Variables|Default|GetMouseFollowWidget) :!label _label_2
              (:Is%20Valid
                (bind _btrue_2 (Default|IsPower (Variables|Default|GetMouseFollowWidget)))
                (if _btrue_2
                  (goto _label)
                  (elif (and (Utilities|IsValid (.HitComponent (Collision|BreakHitResult _output_get))) (Class|GameplayStatics|ObjectIsA (.HitComponent (Collision|BreakHitResult _output_get)) "/Script/Engine.StaticMeshComponent"))
                    (switch Utilities|FlowControl|Switch|SwitchonECollisionResponse (Collision|GetCollisionResponsetoChannel (.HitComponent (Collision|BreakHitResult _output_get)) "ECC_GameTraceChannel2")
                      (:ECR_Block
                        (if (.bBlockingHit (Collision|BreakHitResult (Variables|Default|GetScreenInteractResult)))
                          (if (< (Math|Float|Absolute(Float) (Math|Vector|VectorLength (- (.Location (Collision|BreakHitResult (Variables|Default|GetScreenInteractResult))) _location_2))) 2.8e+02)
                            (bind _returnvalue_5 (Game|SpawnActorfromClass "/Game/DCT/Blueprints/Core/BP_Item.BP_Item_C" (Math|Transform|MakeTransform (+ (.Location (Collision|BreakHitResult (Variables|Default|GetScreenInteractResult))) "0.000000,0.000000,30.000000") _rotation_2) "AdjustIfPossibleButAlwaysSpawn" "OverrideRootScale" 0 (Variables|/Game/DCT/UserInterface/WBP_Item.WBP_Item_C|GetAmount _mousefollowwidget) (Utilities|Struct|MakeDataTableRowHandle "/Game/DCT/Data/DT_Items.DT_Items" (Default|GetItemName _mousefollowwidget)) true 0))
                            (Audio|PlaySoundatLocation (.UseSound (Utilities|Struct|BreakFItem (Default|GetItemData _returnvalue_5))) (+ (.Location (Collision|BreakHitResult (Variables|Default|GetScreenInteractResult))) "0.000000,0.000000,30.000000") "0, 0, 0" 1.0 1.0 0.0 0 0 0 0)
                            (bind _returnvalue_6 (Collision|BoxTraceByChannel (+ (.Location (Collision|BreakHitResult (Variables|Default|GetScreenInteractResult))) "0.000000,0.000000,30.000000") (+ (.Location (Collision|BreakHitResult (Variables|Default|GetScreenInteractResult))) "0.000000,0.000000,30.000000") (.Max (Components|StaticMesh|GetLocalBounds (Variables|/Game/DCT/Blueprints/Core/BP_Item.BP_Item_C|GetItemMesh _returnvalue_5))) (Transformation|GetWorldRotation (Variables|/Game/DCT/Blueprints/Core/BP_Item.BP_Item_C|GetItemMesh _returnvalue_5)) "TraceTypeQuery3" false 0 "ForOneFrame" true "(R=0.000000,G=1.000000,B=0.278894,A=1.000000)" "(R=1.000000,G=0.004847,B=0.000000,A=1.000000)"))
                            (bind _returnvalue_7 (Collision|BoxTraceByChannel (+ (.Location (Collision|BreakHitResult (Variables|Default|GetScreenInteractResult))) "0.000000,0.000000,30.000000") (+ (.Location (Collision|BreakHitResult (Variables|Default|GetScreenInteractResult))) "0.000000,0.000000,30.000000") (.Max (Components|StaticMesh|GetLocalBounds (Variables|/Game/DCT/Blueprints/Core/BP_Item.BP_Item_C|GetItemMesh _returnvalue_5))) (Transformation|GetWorldRotation (Variables|/Game/DCT/Blueprints/Core/BP_Item.BP_Item_C|GetItemMesh _returnvalue_5)) "TraceTypeQuery5" false 0 "ForOneFrame" true "(R=0.000000,G=1.000000,B=0.278894,A=1.000000)" "(R=1.000000,G=0.004847,B=0.000000,A=1.000000)"))
                            (if (or _returnvalue_7 _returnvalue_6)
                              (Transformation|SetActorLocationAndRotation _returnvalue_5 (+ (+ _location "0.000000,0.000000,30.000000") (* (Math|Vector|GetForwardVector _rotation) "80.000000,80.000000,80.000000")) _rotation)
                              (CallFunction|ClearMouseFollowWidget)
                              (else
                                (CallFunction|ClearMouseFollowWidget)))
                            (else
                              (Default|PlaceBackinLastSlotifValid (Variables|Default|GetMouseFollowWidget))))
                          (else
                            (Default|PlaceBackinLastSlotifValid (Variables|Default|GetMouseFollowWidget))))))))))))
        (else
          (goto _label_2))))
    (:Is%20Not%20Valid
      (goto _label_2))))

(event Input|EnhancedActionEvents|EnhancedInputActionIA_Inventory
  (params (ActionValue :type Boolean) (ElapsedSeconds :type Float%20%28double-precision%29) (TriggeredSeconds :type Float%20%28double-precision%29) (InputAction :type Input%20Action%20Object%20Reference :default "/Game/DCT/Input/IA_Inventory.IA_Inventory"))
  ;[0 0 0] UI input
  (:Started
    (bind _playercharacterref (Class|BPIDungeonSingletons|GetActiveWidgetCharacter(Message) (Game|GetGameState)))
    (Default|ToggleSubsheets (.Value (Utilities|Map|Find (Variables|Default|GetCharacterSheets) _playercharacterref)))))

(event Input|EnhancedActionEvents|EnhancedInputActionIA_Character
  (params (ActionValue :type Boolean) (ElapsedSeconds :type Float%20%28double-precision%29) (TriggeredSeconds :type Float%20%28double-precision%29) (InputAction :type Input%20Action%20Object%20Reference :default "/Game/DCT/Input/IA_Character.IA_Character"))
  ;[0 0 0] UI input
  (:Started
    (bind _playercharacterref (Class|BPIDungeonSingletons|GetActiveWidgetCharacter(Message) (Game|GetGameState)))
    (Default|ToggleSubsheets (.Value (Utilities|Map|Find (Variables|Default|GetCharacterSheets) _playercharacterref)) 1)))

(event Input|EnhancedActionEvents|EnhancedInputActionIA_Powers
  (params (ActionValue :type Boolean) (ElapsedSeconds :type Float%20%28double-precision%29) (TriggeredSeconds :type Float%20%28double-precision%29) (InputAction :type Input%20Action%20Object%20Reference :default "/Game/DCT/Input/IA_Powers.IA_Powers"))
  ;[0 0 0] UI input
  (:Started
    (bind _playercharacterref (Class|BPIDungeonSingletons|GetActiveWidgetCharacter(Message) (Game|GetGameState)))
    (Default|ToggleSubsheets (.Value (Utilities|Map|Find (Variables|Default|GetCharacterSheets) _playercharacterref)) 2)))

(event Input|EnhancedActionEvents|EnhancedInputActionIA_StackSplit
  (params (ActionValue :type Boolean) (ElapsedSeconds :type Float%20%28double-precision%29) (TriggeredSeconds :type Float%20%28double-precision%29) (InputAction :type Input%20Action%20Object%20Reference :default "/Game/DCT/Input/IA_StackSplit.IA_StackSplit"))
  ;[0 0 0] UI input
  (:Started
    (Variables|Default|SetbStackSplitPressed true))
  (:Canceled
    (Variables|Default|SetbStackSplitPressed false :!label _label))
  (:Completed
    (goto _label)))

(event EventDisplayWarning
  (params (MessageText :type Text))
  ;[0 0 0] Error Message Display
  (Default|DisplayWarning (Variables|Default|GetWarningDisplayRef) MessageText))

(event EventTick
  (params (DeltaSeconds :type Float%20%28single-precision%29))
  (Utilities|FlowControl|Sequence
    (:then_0
      ;[0 0 0] Move mouse widget on tick
      (Utilities|IsValid (Variables|Default|GetMouseFollowWidget)
        (:Is%20Valid
          (bind _returnvalue (Class|WidgetLayoutLibrary|GetMousePositiononViewport))
          (Class|Widget|SetRenderTransform (Variables|Default|GetMouseFollowWidget) (Utilities|Struct|MakeWidgetTransform (Math|Vector2D|MakeVector2D (.x _returnvalue) (.y _returnvalue)) "(X=1.000000,Y=1.000000)" "(X=0.000000,Y=0.000000)" 0.0))
          (Widget|SetVisibility (Variables|Default|GetMouseFollowWidget) (select (.ReturnValue (Game|Player|GetMousePosition)) "HitTestInvisible" "Hidden")))))
    (:then_1
      ;[0.06848 0.04971 0.4793] Compas 2
      (Class|Widget|SetRenderTransformAngle (Variables|/Game/DCT/UserInterface/WBP_Minimap.WBP_Minimap_C|GetMap_Rose (Variables|Default|GetWBP%20Minimap)) (Utilities|Operators|Subtract (.yaw (Math|Rotator|FindLookatRotation (Transformation|GetActorLocation) (Variables|Default|GetNorth%20Location))) (.yaw (Pawn|GetControlRotation :!class /Script/Engine.Controller)))))))

(event EventSetMouseWidget
  (params (Widget :type WBP%20Item%20Object%20Reference))
  (bind _layoutref (Variables|Default|GetLayoutRef))
  (bind _wbp_helditemdisplay (Variables|/Game/DCT/UserInterface/WBP_Layout.WBP_Layout_C|GetWBP_HeldItemDisplay _layoutref))
  ;[0 0 0] Set Mouse Widget
  (bind _output_get (Variables|Default|SetMouseFollowWidget Widget))
  (Utilities|IsValid _output_get
    (:Is%20Valid
      (CallFunction|UpdateMouseFollowWidgetinVieport)
      (Utilities|FlowControl|Delay 0.0)
      (Default|UpdateHeldItemDisplay _wbp_helditemdisplay (Default|GetItemName (Variables|Default|GetMouseFollowWidget))))
    (:Is%20Not%20Valid
      (Default|UpdateHeldItemDisplay _wbp_helditemdisplay "None"))))

(event EventBeginPlay
  ;[0 0 0] Setup Input
  (Input|AddMappingContext (PlayerController|LocalPlayerSubsystems|GetEnhancedInputLocalPlayerSubsystem) "/Game/DCT/Input/IMC_DCT.IMC_DCT" 0 "(bIgnoreAllPressedKeysUntilRelease=True,bForceImmediately=False,bNotifyUserSettings=False)"))

(event Input|ActionEvents|InputActionSlot1_a
  (params (Key :type Key%20Structure :default "None"))
  (:Pressed
    (CallFunction|SimulateClickSlot 1 1)))

(event Input|ActionEvents|InputActionSlot3_b
  (params (Key :type Key%20Structure :default "None"))
  (:Pressed
    (CallFunction|SimulateClickSlot 3 2)))

(event Input|ActionEvents|InputActionSlot4_a
  (params (Key :type Key%20Structure :default "None"))
  (:Pressed
    (CallFunction|SimulateClickSlot 4 1)))

(event Input|ActionEvents|InputActionSlot4_b
  (params (Key :type Key%20Structure :default "None"))
  (:Pressed
    (CallFunction|SimulateClickSlot 4 2)))

(event Input|ActionEvents|InputActionMenuButton
  (params (Key :type Key%20Structure :default "None"))
  ;[0 0 0] Open/Close Menu
)

(event Input|ActionEvents|InputActionSlot1_b
  (params (Key :type Key%20Structure :default "None"))
  (:Pressed
    (CallFunction|SimulateClickSlot 1 2)))

(event Input|ActionEvents|InputActionSlot2_a
  (params (Key :type Key%20Structure :default "None"))
  (:Pressed
    (CallFunction|SimulateClickSlot 2 1)))

(event Input|ActionEvents|InputActionSlot2_b
  (params (Key :type Key%20Structure :default "None"))
  (:Pressed
    (CallFunction|SimulateClickSlot 2 2)))

(event Input|ActionEvents|InputActionSlot3_a
  (params (Key :type Key%20Structure :default "None"))
  (:Pressed
    (CallFunction|SimulateClickSlot 3 1)))

(event Input|KeyboardEvents|F12
  (params (Key :type Key%20Structure :default "None"))
  (:Pressed
    (Development|ExecuteConsoleCommand "shot showui" 0)
    (Audio|PlaySound2D "/Game/Audio/Magic___Spell_Sounds_PRO/General/wav/Healing_32_2.Healing_32_2" 1.0 1.0 0.0 0 0)
    (CallFunction|DisplayWarning "Screenshot with UI taken")))

(event Input|KeyboardEvents|CtrlX
  (params (Key :type Key%20Structure :default "None"))
  (bind _wbp_menu (Variables|Default|GetWBP%20Menu))
  ;[0 0 0] Open/Close Menu
  (:Pressed
    (bind _bisopen (Class|BPIDungeonSingletons|IsCharacterSheetOpen(Message) (Game|GetGameState)))
    (if _bisopen
      (Class|BPIDungeonSingletons|CloseCharacterSheet(Message) (Game|GetGameState))
      (elif (Utilities|Enum|Equal(Enum) (Widget|GetVisibility (Variables|Default|GetWBP%20Menu)) "Visible")
        (Widget|SetVisibility _wbp_menu "Hidden")
        (else
          (Widget|SetVisibility _wbp_menu "Visible")
          (Game|SetGamePaused true))))))

(event Input|KeyboardEvents|Escape
  (params (Key :type Key%20Structure :default "None"))
  (bind _wbp_menu (Variables|Default|GetWBP%20Menu))
  ;[0 0 0] Open/Close Menu
  (:Pressed
    (bind _bisopen (Class|BPIDungeonSingletons|IsCharacterSheetOpen(Message) (Game|GetGameState)))
    (if _bisopen
      (Class|BPIDungeonSingletons|CloseCharacterSheet(Message) (Game|GetGameState))
      (elif (Utilities|Enum|Equal(Enum) (Widget|GetVisibility (Variables|Default|GetWBP%20Menu)) "Visible")
        (Widget|SetVisibility _wbp_menu "Hidden")
        (else
          (Widget|SetVisibility _wbp_menu "Visible")
          (Game|SetGamePaused true))))))

(event Input|KeyboardEvents|ShiftF12
  (params (Key :type Key%20Structure :default "None"))
  (:Pressed
    (Development|ExecuteConsoleCommand "shot" 0)
    (Audio|PlaySound2D "/Game/Audio/Magic___Spell_Sounds_PRO/General/wav/Healing_32_2.Healing_32_2" 1.0 1.0 0.0 0 0)
    (CallFunction|DisplayWarning "Screenshot taken")))

(fn ConstructionScript)

(fn SetupPlayerCharacterUi
  (params (PlayerCharacter :type BP%20Player%20Character%20Object%20Reference) (CharacterIndex :type Integer))
  (bind _returnvalue (UserInterface|CreateWidget "/Game/DCT/UserInterface/WBP_CharacterSheet.WBP_CharacterSheet_C" self PlayerCharacter))
  (bind _output_get (Variables|/Game/DCT/Blueprints/Core/BP_PlayerCharacter.BP_PlayerCharacter_C|SetCharacterSheetRef PlayerCharacter _returnvalue))
  (Utilities|Map|Add (Variables|Default|GetCharacterSheets) PlayerCharacter _output_get)
  (Widget|Panel|AddChild (Variables|/Game/DCT/UserInterface/WBP_Layout.WBP_Layout_C|GetSheetSwitcher (Variables|Default|GetLayoutRef)) _output_get)
  (bind _returnvalue_2 (UserInterface|CreateWidget "/Game/DCT/UserInterface/WBP_MiniCharacter.WBP_MiniCharacter_C" self _output_get PlayerCharacter 0))
  (Class|UniformGridPanel|AddChildtoUniformGrid (Variables|/Game/DCT/UserInterface/WBP_Layout.WBP_Layout_C|GetMiniCharacterPanel (Variables|Default|GetLayoutRef)) _returnvalue_2 (/ CharacterIndex 1) (Math|Integer|%(Integer) CharacterIndex 1))
  (Default|UpdateMiniCharacter _returnvalue_2)
  (Variables|/Game/DCT/Blueprints/Core/BP_PlayerCharacter.BP_PlayerCharacter_C|SetMiniCharacterRef PlayerCharacter _returnvalue_2)
  (return))

(fn LoadCharacterItems
  (bind (_bvalid _playercharacterdata) (Default|GetSavedCharacters (.DungeonInstance (CallFunction|GetDungeonGameInstance))))
  (if _bvalid
    (bind _values (Utilities|Map|Values (Variables|Default|GetCharacterSheets)))
    (for (_array_element _array_index) _values
      (Default|LoadItems (Variables|/Game/DCT/UserInterface/WBP_CharacterSheet.WBP_CharacterSheet_C|GetWBP_Inventory _array_element) (.inventory (Utilities|Array|Get(acopy) _playercharacterdata _array_index)) (.equipment (Utilities|Array|Get(acopy) _playercharacterdata _array_index)) false))
    (return)))

(fn ClearMouseFollowWidget
  (bind _mousefollowwidget (Variables|Default|GetMouseFollowWidget)
    (:then
      (Widget|RemovefromParent _mousefollowwidget)
      (CallFunction|SetMouseWidget)
      (return))
    (:else
      (return))))

(fn UpdateMouseFollowWidgetinVieport
  (Widget|RemovefromParent (Variables|Default|GetMouseFollowWidget))
  (Class|CanvasPanel|AddChildtoCanvas (Variables|/Game/DCT/UserInterface/WBP_Layout.WBP_Layout_C|GetHeldItemCanvas (Variables|Default|GetLayoutRef)) (Variables|Default|GetMouseFollowWidget))
  (Class|CanvasPanelSlot|SetSize (Class|WidgetLayoutLibrary|SlotasCanvasSlot (Variables|Default|GetMouseFollowWidget)) (LocalVariables|GetLocalWidgetSize))
  (Widget|SetVisibility (Variables|Default|GetMouseFollowWidget) "SelfHitTestInvisible")
  (return))

(fn GetMouseWidget
  (return (Variables|Default|GetMouseFollowWidget)))

(fn IsStackSplitPressed
  (return (Variables|Default|GetbStackSplitPressed)))