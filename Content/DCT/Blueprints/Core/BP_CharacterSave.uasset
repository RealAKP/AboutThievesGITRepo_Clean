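; BP_CharacterSave stores player character data (identity, stats, inventory and equipment) for saving.
; StoreCharacters rebuilds the data array from the given characters, optionally overwriting each one's base stats with its current stats.
; When item storing is enabled, it reads items directly from each character sheet's inventory grid and paper doll widgets, recording type and amount by slot index.
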(fn StoreCharacters
  (params (PlayerCharacters :type Array%20of%20BP%20Player%20Character%20Object%20References) (bRebaseCharacters :type Boolean) (bStoreItems :type Boolean))
  (Utilities|Array|Clear (Variables|Default|GetPlayerCharacterData))
  (for _array_element PlayerCharacters
    (if bRebaseCharacters
      (Variables|/Game/DCT/Blueprints/Core/BP_PlayerCharacter.BP_PlayerCharacter_C|SetBaseStats _array_element (Variables|/Game/DCT/Blueprints/Core/BP_PlayerCharacter.BP_PlayerCharacter_C|GetCurrentStats _array_element)))
    (if bStoreItems
      (Utilities|Map|Clear (LocalVariables|GetLocalEquipment))
      (Utilities|Map|Clear (LocalVariables|GetLocalInventory))
      (for (_array_element_2 _array_index) (Class|PanelWidget|GetAllChildren (Variables|/Game/DCT/UserInterface/WBP_Inventory.WBP_Inventory_C|GetSlotGrid (Variables|/Game/DCT/UserInterface/WBP_CharacterSheet.WBP_CharacterSheet_C|GetWBP_Inventory (Variables|/Game/DCT/Blueprints/Core/BP_PlayerCharacter.BP_PlayerCharacter_C|GetCharacterSheetRef _array_element))))
        (bind _aswbp_slot (Utilities|Casting|CastToWBP_Slot _array_element_2))
        (Utilities|IsValid (Variables|/Game/DCT/UserInterface/WBP_Slot.WBP_Slot_C|GetSlottedItem _aswbp_slot)
          (:Is%20Valid
            (Utilities|Map|Add (LocalVariables|GetLocalInventory) _array_index (Utilities|Struct|MakeFItemSave (Variables|/Game/DCT/UserInterface/WBP_Item.WBP_Item_C|GetItemType (Variables|/Game/DCT/UserInterface/WBP_Slot.WBP_Slot_C|GetSlottedItem _aswbp_slot)) (Variables|/Game/DCT/UserInterface/WBP_Item.WBP_Item_C|GetAmount (Variables|/Game/DCT/UserInterface/WBP_Slot.WBP_Slot_C|GetSlottedItem _aswbp_slot)) "0.000000,0.000000,0.000000|0.000000,0.000000,-0.000000|1.000000,1.000000,1.000000" true)))))
      (for (_array_element_3 _array_index_2) (Variables|/Game/DCT/UserInterface/WBP_PaperDoll.WBP_PaperDoll_C|GetSlots (Variables|/Game/DCT/UserInterface/WBP_Inventory.WBP_Inventory_C|GetWBP_PaperDoll (Variables|/Game/DCT/UserInterface/WBP_CharacterSheet.WBP_CharacterSheet_C|GetWBP_Inventory (Variables|/Game/DCT/Blueprints/Core/BP_PlayerCharacter.BP_PlayerCharacter_C|GetCharacterSheetRef _array_element))))
        (Utilities|IsValid (Variables|/Game/DCT/UserInterface/WBP_Slot.WBP_Slot_C|GetSlottedItem _array_element_3)
          (:Is%20Valid
            (Utilities|Map|Add (LocalVariables|GetLocalEquipment) _array_index_2 (Utilities|Struct|MakeFItemSave (Variables|/Game/DCT/UserInterface/WBP_Item.WBP_Item_C|GetItemType (Variables|/Game/DCT/UserInterface/WBP_Slot.WBP_Slot_C|GetSlottedItem _array_element_3)) (Variables|/Game/DCT/UserInterface/WBP_Item.WBP_Item_C|GetAmount (Variables|/Game/DCT/UserInterface/WBP_Slot.WBP_Slot_C|GetSlottedItem _array_element_3)) "0.000000,0.000000,0.000000|0.000000,0.000000,-0.000000|1.000000,1.000000,1.000000" true))))))
    (Utilities|Array|Add (Variables|Default|GetPlayerCharacterData) (Utilities|Struct|MakeFCharacterData (Variables|/Game/DCT/Blueprints/Core/BP_PlayerCharacter.BP_PlayerCharacter_C|GetName _array_element) (Variables|/Game/DCT/Blueprints/Core/BP_PlayerCharacter.BP_PlayerCharacter_C|GetPortrait _array_element) (LocalVariables|GetLocalInventory) (LocalVariables|GetLocalEquipment) (Variables|/Game/DCT/Blueprints/Core/BP_PlayerCharacter.BP_PlayerCharacter_C|GetRaces _array_element) (Variables|/Game/DCT/Blueprints/Core/BP_PlayerCharacter.BP_PlayerCharacter_C|GetCharacterClass _array_element) (Variables|/Game/DCT/Blueprints/Core/BP_PlayerCharacter.BP_PlayerCharacter_C|GetBaseStats _array_element) (Variables|/Game/DCT/Blueprints/Core/BP_PlayerCharacter.BP_PlayerCharacter_C|GetCurrentStats _array_element) (Variables|/Game/DCT/Blueprints/Core/BP_PlayerCharacter.BP_PlayerCharacter_C|GetVoices _array_element))))
  (return))