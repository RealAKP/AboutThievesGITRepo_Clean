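; BP_Item is a world item pickup for the dungeon game, taking its mesh, weight and other data from an ItemType data table row, with optional physics.
; Interaction requires the pawn's grid location within range and a free cursor, then replaces the actor with a mouse-held WBP_Item widget.
; Cursor hover toggles a material highlight.
; SaveActor records type, amount, transform and physics in the DungeonInstance, while UpdatePreplaced destroys the actor.
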(event MouseInput|EventActorBeginCursorOver
  (Rendering|Material|SetScalarParameterValueonMaterials (Variables|Default|GetItemMesh) "Highlight" 1.0))

(event MouseInput|EventActorEndCursorOver
  (Rendering|Material|SetScalarParameterValueonMaterials (Variables|Default|GetItemMesh) "Highlight" 0.0))

(event EventSaveActor
  (params (DungeonInstance :type BP%20GI%20Dungeon%20Object%20Reference))
  (Utilities|Array|Add (Variables|/Game/DCT/Blueprints/Core/BP_GI_Dungeon.BP_GI_Dungeon_C|GetSavedItems DungeonInstance) (Utilities|Struct|MakeFItemSave (Variables|Default|GetItemType) (Variables|Default|GetAmount) (Transformation|GetActorTransform) (Variables|Default|GetbEnablePhysics))))

(event EventUpdatePreplaced
  (Actor|DestroyActor))

(event EventInteract
  (params (TriggeringActor :type Actor%20Object%20Reference))
  (bind _asbp_pc_dungeon (Utilities|Casting|CastToBP_PC_Dungeon (Game|GetPlayerController 0)))
  (bind _returnvalue (UserInterface|CreateWidget "/Game/DCT/UserInterface/WBP_Item.WBP_Item_C" _asbp_pc_dungeon (Variables|Default|GetAmount) (Variables|Default|GetItemType)))
  (Class|BPIPlayerController|SetMouseWidget(Message) (Game|GetPlayerController 0) _returnvalue)
  (Actor|DestroyActor))

(fn ConstructionScript
  (bind _itemtype (Variables|Default|GetItemType))
  (bind _returnvalue (Utilities|GetDataTableRow (.datatable _itemtype) (.rowname _itemtype))
    (:then
      (Components|StaticMesh|SetStaticMesh (Variables|Default|GetItemMesh) (Utilities|Struct|BreakFItem _returnvalue))
      (Physics|SetSimulatePhysics (Variables|Default|GetItemMesh) (Variables|Default|GetbEnablePhysics)))))

(fn GetItemData
  (bind _itemtype (Variables|Default|GetItemType))
  (bind _returnvalue (Utilities|GetDataTableRow (.datatable _itemtype) (.rowname _itemtype))
    (:then
      (return _returnvalue))
    (:RowNotFound
      (return ""))))

(fn GetItemName
  (return (.RowName (Utilities|Struct|BreakDataTableRowHandle (Variables|Default|GetItemType)))))

(fn CheckifAllowedInteract
  (params (TriggeringActor :type Actor%20Object%20Reference))
  (bind _asbp_dungeon_pawn (Utilities|Casting|CastToBP_DungeonPawn TriggeringActor))
  (if (.ReturnValue (Utilities|Map|Find (Variables|/Game/DCT/Blueprints/Core/BP_DungeonManager.BP_DungeonManager_C|GetGridLocations (.DungeonManager (CallFunction|GetDungeonManager))) (Variables|/Game/DCT/Blueprints/Core/BP_DungeonPawn.BP_DungeonPawn_C|GetGridIndex _asbp_dungeon_pawn)))
    (Variables|Default|SetLocalTriggeringLocation (.Value (Utilities|Map|Find (Variables|/Game/DCT/Blueprints/Core/BP_DungeonManager.BP_DungeonManager_C|GetGridLocations (.DungeonManager (CallFunction|GetDungeonManager))) (Variables|/Game/DCT/Blueprints/Core/BP_DungeonPawn.BP_DungeonPawn_C|GetGridIndex _asbp_dungeon_pawn))))
    (else
      (Variables|Default|SetLocalTriggeringLocation (Transformation|GetActorLocation TriggeringActor))))
  (if (<= (Math|Float|Absolute(Float) (Math|Vector|Distance(Vector) (Variables|Default|GetLocalTriggeringLocation) (Transformation|GetActorLocation))) (Variables|/Game/DCT/Blueprints/Core/BP_DungeonManager.BP_DungeonManager_C|GetMaxInteractionRange (.DungeonManager (CallFunction|GetDungeonManager))))
    (bind _asbp_pc_dungeon (Utilities|Casting|CastToBP_PC_Dungeon (Game|GetPlayerController 0))
      (:then
        (Utilities|IsValid (Variables|/Game/DCT/Blueprints/Core/BP_PC_Dungeon.BP_PC_Dungeon_C|GetMouseFollowWidget _asbp_pc_dungeon)
          (:Is%20Valid
            (return false))
          (:Is%20Not%20Valid
            (return true))))
      (:CastFailed
        _)))
  (return false))

(fn AttemptInteract
  (params (TriggeringActor :type Actor%20Object%20Reference))
  (bind _allowed (CallFunction|CheckifAllowedInteract TriggeringActor))
  (if _allowed
    (CallFunction|Interact TriggeringActor)
    (return true)
    (else
      (return false))))

(fn GetAttachSlot
  (return 0))

(fn GetWeight
  (return (Utilities|Struct|BreakFItem (CallFunction|GetItemData))))