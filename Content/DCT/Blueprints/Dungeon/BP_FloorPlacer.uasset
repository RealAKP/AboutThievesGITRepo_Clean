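; BP_FloorPlacer is a dungeon construction actor that tiles a chosen floor mesh over a rectangular area set by SizeWidget.
; The construction script divides that area by the mesh's bounding-box size, rounding up, and SpawnFloor adds the grid as instances on FloorHism.
; DoubleSided adds a second grid, rolled over and lowered by a fixed offset.
; The Ceiling flag turns collision off on the instanced mesh component.
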(event EventBeginPlay)

(event Collision|EventActorBeginOverlap
  (params (OtherActor :type Actor%20Object%20Reference)))

(event EventTick
  (params (DeltaSeconds :type Float%20%28single-precision%29)))

(fn ConstructionScript
  (bind _floorhism (Variables|Default|GetFloorHism))
  (bind _sizewidget (Variables|Default|GetSizeWidget))
  (bind _staticmesh (Variables|/Script/Engine.StaticMeshComponent|GetStaticMesh _floorhism))
  (bind _returnvalue (StaticMesh|GetBoundingBox _staticmesh))
  (bind _returnvalue_2 (- (.y (.min _returnvalue)) (.y (.max _returnvalue))))
  (bind _returnvalue_3 (- (.x (.min _returnvalue)) (.x (.max _returnvalue))))
  (bind _returnvalue_4 (Math|Float|Absolute(Float) _returnvalue_2))
  (bind _returnvalue_5 (Math|Float|Absolute(Float) _returnvalue_3))
  (bind _returnvalue_6 (/ (.y _sizewidget) _returnvalue_4))
  (bind _returnvalue_7 (/ (.x _sizewidget) _returnvalue_5))
  (bind _returnvalue_8 (Math|Float|Ceil _returnvalue_7))
  (bind _returnvalue_9 (Math|Float|Ceil _returnvalue_6))
  (Collision|SetCollisionEnabled (Variables|Default|GetFloorHism) (select (Variables|Default|GetbCeiling) "NoCollision" "QueryAndPhysics"))
  (Components|StaticMesh|SetStaticMesh (Variables|Default|GetFloorHism) (Variables|Default|GetFloorMesh))
  (Utilities|IsValid _staticmesh
    (:Is%20Valid
      (CallFunction|SpawnFloor _returnvalue_8 _returnvalue_9 _returnvalue_5 _returnvalue_4 false)
      (if (Variables|Default|GetbDoubleSided)
        (CallFunction|SpawnFloor _returnvalue_8 _returnvalue_9 _returnvalue_5 _returnvalue_4 true)))))

(fn SpawnFloor
  (params (FloorSizeX :type Integer) (FloorSizeY :type Integer) (FloorMeshSizeX :type Float%20%28single-precision%29) (FloorMeshSizeY :type Float%20%28single-precision%29) (bFlipped :type Boolean))
  (for _index (range 0 (- (* FloorSizeX FloorSizeY) 1))
    (Components|InstancedStaticMesh|AddInstance (Variables|Default|GetFloorHism) (Math|Transform|MakeTransform (Math|Vector|MakeVector (* (Math|Integer|%(Integer) _index FloorSizeX) FloorMeshSizeX) (* (/ _index FloorSizeX) FloorMeshSizeY) (Math|Float|SelectFloat -45.0 0.0 bFlipped)) (Math|Rotator|MakeRotator (Math|Float|SelectFloat 1.8e+02 0.0 bFlipped) 0.0 0.0) "1,1,1")))
  (return))