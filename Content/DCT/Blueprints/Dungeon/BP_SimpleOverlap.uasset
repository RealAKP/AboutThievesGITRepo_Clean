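; A grid dungeon interactable that fires when a dungeon pawn steps into or out of its overlap areas.
; Construction builds box components from the configured areas; BeginPlay attaches to an optional slot and records the nearest valid tile's grid index.
; Overlap binds to the pawn's step end, which interacts on standing in a "Step" box, then again on leaving before unbinding.
; Direct attempts respect single-use, transition and "Click" box checks, and its state saves to the dungeon instance.
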(event Custom|CallOnPlayerStepEnd
  (params (DungeonPawn :type BP%20Dungeon%20Pawn%20Object%20Reference))
  (bind _desiredstate (Variables|Default|GetDesiredState))
  (bind _boverlaps (CallFunction|DoesActorOverlapCollisionBoxwithTag DungeonPawn "Step"))
  (if _boverlaps
    (switch Utilities|FlowControl|Switch|SwitchonEInteractState _desiredstate
      (:NewEnumerator0
        (CallFunction|Interact DungeonPawn :!label _label)))
    (else
      (switch Utilities|FlowControl|Switch|SwitchonEInteractState _desiredstate
        (:NewEnumerator2
          (Utilities|FlowControl|Sequence
            (:then_0
              (goto _label))
            (:then_1
              (EventDispatchers|UnbindEventfromOnStepEnd DungeonPawn (delegate Custom|CallOnPlayerStepEnd)))))))))

(event EventSaveActor
  (params (DungeonInstance :type BP%20GI%20Dungeon%20Object%20Reference))
  (Utilities|Array|Add (Variables|/Game/DCT/Blueprints/Core/BP_GI_Dungeon.BP_GI_Dungeon_C|GetSavedInteractables DungeonInstance) (Utilities|Struct|MakeFInteractableSave (Utilities|GetDisplayName self) (Transformation|GetActorTransform) (Variables|Default|GetDesiredState) 0)))

(event Collision|EventActorBeginOverlap
  (params (OtherActor :type Actor%20Object%20Reference))
  (if (> (Utilities|Array|Length (Variables|Default|GetInteractionOverlapAreas)) 0)
    (bind _asbp_dungeon_pawn (Utilities|Casting|CastToBP_DungeonPawn OtherActor))
    (EventDispatchers|BindEventtoOnStepEnd _asbp_dungeon_pawn (delegate Custom|CallOnPlayerStepEnd))))

(event EventBeginPlay
  (CallFunction|AttachtoSelectedSlotifValid)
  (Utilities|FlowControl|Delay 0.0)
  (bind _gridindex (Default|FindNearbyValidTile (.DungeonManager (CallFunction|GetDungeonManager)) (Transformation|GetActorLocation)))
  (Variables|Default|SetGridIndex _gridindex))

(fn ConstructionScript
  (for _array_element (Variables|Default|GetInteractionOverlapAreas)
    (AddComponent|AddBoxComponent false _array_element))
  (CallFunction|UpdateDesiredState (Variables|Default|GetDesiredState)))

(fn CheckifAllowedInteract
  (params (TriggeringActor :type Object%20Object%20Reference))
  (if (or (Variables|Default|GetbAllowInteractDuringTransition) (== (Variables|Default|GetInteractState) (Variables|Default|GetDesiredState)))
    (Utilities|IsValid TriggeringActor
      (:Is%20Valid
        (bind _aspawn (Utilities|Casting|CastToPawn TriggeringActor)
          (:then
            (bind _boverlaps (CallFunction|DoesActorOverlapCollisionBoxwithTag _aspawn "Click"))
            (return _boverlaps))
          (:CastFailed
            (return true))))
      (:Is%20Not%20Valid
        (return true)))
    (else
      (return false))))

(fn GetOppositeInteractState
  (params (Index :type EInteractState%20Enum :default "NewEnumerator0"))
  (return (Utilities|Select :Index Index :NewEnumerator0 "NewEnumerator2" :NewEnumerator2 "NewEnumerator0")))

(fn DoesActorOverlapCollisionBoxwithTag
  (params (Actor :type Actor%20Object%20Reference) (CollisionBoxTag :type Name :default "Click"))
  (for _array_element (Class|Actor|GetOverlappingComponents Actor)
    (bind _asbox_collision (Utilities|Casting|CastToBoxComponent _array_element))
    (if (Utilities|Array|ContainsItem (Actor|GetComponentsbyTag "/Script/Engine.BoxComponent" CollisionBoxTag) _asbox_collision)
      (return true)))
  (return false))

(fn AttachtoSelectedSlotifValid
  (bind _attachslot (Class|BPIInteract|GetAttachSlot(Message) (Variables|Default|GetActorToAttach)))
  (Utilities|IsValid _attachslot
    (:Is%20Valid
      (Transformation|AttachComponentToComponent _attachslot "None" "KeepWorld" "KeepWorld" "KeepWorld" true)
      (return true))
    (:Is%20Not%20Valid
      (return true))))

(fn CheckifExhausted
  (return (and (Variables|Default|GetbSingleUse) (Utilities|Enum|Equal(Enum) (Variables|Default|GetInteractState) "NewEnumerator2"))))

(fn AttemptInteract
  (params (TriggeringActor :type Actor%20Object%20Reference))
  (if (not (CallFunction|CheckifExhausted))
    (bind _ballowed (CallFunction|CheckifAllowedInteract TriggeringActor))
    (if _ballowed
      (Variables|Default|SetTriggeringActor TriggeringActor)
      (CallFunction|Interact TriggeringActor)
      (return true)
      (else
        (return false)))))

(fn GetAttachSlot
  (return 0))