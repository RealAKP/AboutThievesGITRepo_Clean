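; Destructible dungeon prop that occupies a grid tile until damage depletes its health.
; On BeginPlay it finds the nearest valid tile through the DungeonManager, blocks it and registers itself on the grid.
; Each hit spawns red floating damage text, and breaking plays a particle, unregisters the prop and reopens the tile.
; It rejects interaction, reports fixed weight and negative dodge chance, and takes its mesh from Appearance.
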(event EventBeginPlay
  (Utilities|FlowControl|Delay 0.0)
  (bind _gridindex (Default|FindNearbyValidTile (.DungeonManager (CallFunction|GetDungeonManager)) (Transformation|GetActorLocation)))
  (Variables|Default|SetGridIndex _gridindex)
  (Default|BlockTile (.DungeonManager (CallFunction|GetDungeonManager)) (Variables|Default|GetGridIndex))
  (Default|AddObjecttoGrid (.DungeonManager (CallFunction|GetDungeonManager)) self (Variables|Default|GetGridIndex)))

(event EventTakeDamage
  (params (Damage :type Float%20%28single-precision%29))
  (Variables|Default|SetHealth (- (Variables|Default|GetHealth) Damage))
  (bind _returnvalue (Game|SpawnActorfromClass "/Game/DCT/Blueprints/Core/BP_FloatingText.BP_FloatingText_C" (Math|Transform|MakeTransform (+ (Transformation|GetActorLocation) "0,0.000000,100.000000") "0, 0, 0" "1,1,1") "AlwaysSpawn" 0 (Utilities|Text|ToText(Float) Damage "HalfToEven") 0))
  (Default|SetColor _returnvalue "(R=1.000000,G=0.000000,B=0.000000,A=1.000000)")
  (if (< (Variables|Default|GetHealth) 1.0)
    (Default|RemoveObjectfromGrid (.DungeonManager (CallFunction|GetDungeonManager)) self (Variables|Default|GetGridIndex))
    (Effects|SpawnEmitteratLocation (Variables|Default|GetBreakParticle) (Transformation|GetActorLocation) "0, 0, 0" "2.000000,2.000000,2.000000")
    (Actor|DestroyActor)
    (Default|ReopenTile (.DungeonManager (CallFunction|GetDungeonManager)) (Variables|Default|GetGridIndex))))

(fn ConstructionScript
  (Components|StaticMesh|SetStaticMesh (Variables|Default|GetStaticMesh) (Variables|Default|GetAppearance)))

(fn GetWeight
  (return 1.0))

(fn AttemptInteract
  (params (TriggeringActor :type Actor%20Object%20Reference))
  (return false))

(fn GetDodgeChance
  (return -0.5))