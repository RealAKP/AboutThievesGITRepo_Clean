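; Dungeon spike trap interactable that stabs the party when triggered on its grid cell.
; Interact plays a stab sound and runs a timeline that moves the spikes vertically and fires a damage event.
; That event checks whether the dungeon pawn occupies the trap's cell, then damages each living player character.
; Inside that same loop, a triggering monster also takes damage, so only when the party is on the cell.
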(event EventUpdateDesiredState
  (params (NewState :type EInteractState%20Enum :default "NewEnumerator0"))
  (|CallParentFunction NewState))

(event EventInteract
  (params (TriggeringActor :type Actor%20Object%20Reference))
  (bind _damage (Variables|Default|GetDamage))
  (Audio|PlaySoundatLocation "/Game/DCT/Sound/A_Hit_Stab.A_Hit_Stab" (Transformation|GetActorLocation) "0, 0, 0" 1.0 1.0 0.0 "/Game/DCT/Sound/ATT_Dungeon.ATT_Dungeon" 0 0 0)
  (bind _trigger (Timeline|TL_Open PlayFromStart)
    (:Update
      (Transformation|SetRelativeLocation (Variables|Default|GetSpikes) (Math|Vector|MakeVector 0.0 0.0 (- (* _trigger 1e+02) 1e+02)) false false))
    (:Damage
      (if (== (Default|ConvertLocationtoIndex (.DungeonManager (CallFunction|GetDungeonManager)) (Transformation|GetActorLocation (.DungeonPawn (CallFunction|GetDungeonPawn)))) (Variables|Default|GetGridIndex))
        (bind _livingplayercharacters (Default|GetLivingPlayerCharacters (.DungeonState (CallFunction|GetDungeonGameState))))
        (for _array_element _livingplayercharacters
          (Class|BPIAttackTarget|TakeDamage(Message) _array_element _damage)
          (bind _asbp_monster (Utilities|Casting|CastToBP_Monster TriggeringActor))
          (Class|BPIAttackTarget|TakeDamage(Message) _asbp_monster _damage))))))

(fn ConstructionScript)