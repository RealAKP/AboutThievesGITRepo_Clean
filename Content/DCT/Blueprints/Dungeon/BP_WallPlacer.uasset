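; Dungeon wall placer that procedurally tiles WallMesh into two perpendicular walls along local X and Y, sized by SizeWidget.
; The construction script measures the mesh bounds and calls SpawnWall, which adds rotated HISM instances in rows and stacked layers.
; IncludeBase triggers a Y-only pass on WallBaseHism without a MeshHeight, which SpawnWall's height check requires; the X base call is unreachable.
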(event EventBeginPlay)

(event Collision|EventActorBeginOverlap
  (params (OtherActor :type Actor%20Object%20Reference)))

(event EventTick
  (params (DeltaSeconds :type Float%20%28single-precision%29)))

(fn ConstructionScript
  (bind _sizewidget (Variables|Default|GetSizeWidget))
  (bind _wallhism (Variables|Default|GetWallHism))
  (bind _sizewidget_2 (Variables|Default|GetSizeWidget))
  (bind _sizewidget_3 (Variables|Default|GetSizeWidget))
  (bind _staticmesh (Variables|/Script/Engine.StaticMeshComponent|GetStaticMesh _wallhism))
  (bind _returnvalue (StaticMesh|GetBoundingBox _staticmesh))
  (bind _returnvalue_2 (- (.z (.min _returnvalue)) (.z (.max _returnvalue))))
  (bind _returnvalue_3 (- (.y (.min _returnvalue)) (.y (.max _returnvalue))))
  (bind _returnvalue_4 (Math|Float|Absolute(Float) _returnvalue_2))
  (bind _returnvalue_5 (Math|Float|Absolute(Float) _returnvalue_3))
  (Components|StaticMesh|SetStaticMesh (Variables|Default|GetWallHism) (Variables|Default|GetWallMesh))
  (Utilities|IsValid _staticmesh
    (:Is%20Valid
      (CallFunction|SpawnWall (.y _sizewidget_2) (.z _sizewidget_2) _returnvalue_5 _returnvalue_4 "0,1.000000, 0" (Variables|Default|GetWallHism))
      (CallFunction|SpawnWall (.x _sizewidget_3) (.z _sizewidget_3) _returnvalue_5 _returnvalue_4 "1.000000, 0, 0" (Variables|Default|GetWallHism))
      (if (Variables|Default|GetbIncludeBase)
        (CallFunction|SpawnWall (.y _sizewidget) (.z _sizewidget) _returnvalue_5 0.0 "0,1.000000, 0" (Variables|Default|GetWallBaseHism))))))

(fn SpawnWall
  (params (TotalLength :type Float%20%28single-precision%29) (TotalHeight :type Float%20%28single-precision%29) (MeshLength :type Float%20%28single-precision%29) (MeshHeight :type Float%20%28single-precision%29) (Direction :type Vector) (MeshInstance :type Instanced%20Static%20Mesh%20Component%20Object%20Reference))
  (if (and (> MeshHeight 0.0) (> MeshHeight 0.0))
    (for _index (range 0 (Math|Float|Floor (/ TotalHeight MeshHeight)))
      (for _index_2 (range 0 (Math|Float|Floor (/ (- TotalLength 1.0) MeshLength)))
        (Components|InstancedStaticMesh|AddInstance MeshInstance (Math|Transform|MakeTransform (+ (* Direction (+ (* _index_2 MeshLength) (/ MeshLength 2.0))) (Math|Vector|MakeVector 0.0 0.0 (* _index MeshHeight))) (Math|Rotator|CombineRotators (Math|Rotator|MakeRotationfromAxes Direction "0, 0, 0" "0, 0, 0") "0,90.000000, 0") "1,1,1"))))
    (return)))